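; Arena actor that colors the battle floor for each side and visually reflects which player has the upper hand.
; InitSide passes an arena skin to InitFloor, which writes its floor color into that side's material color parameter.
; BeginPlay retries each tick until the GameInstance's BattleManager is valid, then binds to its upper-hand change.
; Each change runs a timeline that lerps a Material Parameter Collection's Progression toward P1, P2 or the neutral middle.
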(event EventBeginPlay
  (bind _asbp_gi (Utilities|Casting|CastToBP_GI (Game|GetGameInstance)))
  (bind _battlemanager (Variables|/Game/BP/BP_GI.BP_GI_C|GetBattleManager _asbp_gi :!label _label)
    (:then
      (EventDispatchers|BindEventtoOnUpperHandStateChanged _battlemanager (|OnUpperHandState_Changed)))
    (:else
      (Utilities|FlowControl|DelayUntilNextTick)
      (goto _label))))

(fn ConstructionScript)

(fn InitSide
  (params (Index :type Integer) (ArenaSkin :type S%20Arena%20Skin%20Structure))
  (Utilities|InitFloor Index ArenaSkin))

(event Custom|OnUpperHandStateChanged
  (params (New%20State :type E_UpperHand%20Enum :default "NewEnumerator0"))
  (bind _returnvalue (Rendering|Material|GetScalarParameterValue (Variables|MPC|GetMPC) (Variables|MPC|GetProgression) :!class /Script/Engine.KismetMaterialLibrary))
  (Variables|Default|SetOldUpperHandProg _returnvalue)
  (Variables|Default|SetNewUpperHandProg (Utilities|Select :Index New%20State :NewEnumerator0 0.5 :NewEnumerator1 1.0 :NewEnumerator2 0.0))
  (bind _value (Timeline|Timeline PlayFromStart)
    (:Update
      (Rendering|Material|SetScalarParameterValue (Variables|MPC|GetMPC) (Variables|MPC|GetProgression) (Math|Float|Lerp (Variables|Default|GetOldUpperHandProg) (Variables|Default|GetNewUpperHandProg) _value) :!class /Script/Engine.KismetMaterialLibrary))))