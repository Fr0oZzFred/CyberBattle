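; BP_BattleManager is a manager Blueprint that runs a battle countdown timer tied to the game state.
; On BeginPlay it registers itself with BP_GI, the game instance, and binds to its game state change event.
; The state change enables Tick in In Game and disables it in Pause or Game Over.
; Tick decrements Time and formats it into Timer as decimal minutes rather than minutes and seconds.
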(event Custom|OnGameStateChanged
  (switch Utilities|FlowControl|Switch|SwitchonE_GameState (Variables|/Game/BP/BP_GI.BP_GI_C|GetCurrentState (stale EventBeginPlay _asbp_gi))
    (:NewEnumerator3
      (Actor|Tick|SetActorTickEnabled true))
    (:NewEnumerator5
      (Actor|Tick|SetActorTickEnabled false :!label _label))
    (:NewEnumerator4
      (goto _label))))

(event EventBeginPlay
  (bind _asbp_gi (Utilities|Casting|CastToBP_GI (Game|GetGameInstance)))
  (Variables|/Game/BP/BP_GI.BP_GI_C|SetBattleManager _asbp_gi self)
  (EventDispatchers|BindEventtoOnGameStateChanged _asbp_gi (delegate Custom|OnGameStateChanged)))

(event EventTick
  (params (DeltaSeconds :type Float%20%28single-precision%29))
  (bind _output_get (Variables|Default|SetTime (- (stale _output_get) DeltaSeconds)))
  (Variables|Default|SetTimer (Utilities|Text|ToText(Float) (/ (Variables|Default|GetTime) 6e+01) "HalfToEven" false true 1 324 0 2)))

(fn ConstructionScript)