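; AI-controlled fighter pawn, adapted from the player Fighter, that battles P1 in station-versus-station matches.
; BeginPlay loads stats from data tables, spawns skill and ultimate actors, and binds to game-state changes.
; Tick faces P1, or its station when P1 is dead, and outside auto-aim, dash and spin fires off-cooldown actions through input-gated events.
; Projectile overlaps drive shield, damage and death, which toggles station vulnerability and starts respawning.
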(event Custom|AI_Shot
  ;[1 1 1 1 100] Inputs
  ;;[1 1 1 1 50] Shot
  (bind _recieveinput (CallFunction|RecieveInput))
  (if _recieveinput
    ;;;[1 0.6128 0.3355] Check Reload Cooldown
    (if (<= (Variables|Default|GetReloadTimer) 0.0)
      (if (Variables|Default|GetUseOverHeat)
        (if (not (Variables|Default|GetHasOverheat))
          (bind _output_get (Variables|Default|SetOverheatBar (+ (Variables|Default|GetOverheatBar) 1.0)))
          (if (> _output_get (Variables|Default|GetOverheatMax))
            (Variables|Default|SetHasOverheat true))
          ;;;[1 0.4986 0.1305] Attack
          (CallFunction|Shot :!label _label)
          ;;;[1 0.6335 0.3727] Set Reload Cooldown
          (Variables|Default|SetReloadTimer (Variables|Default|GetReloadCooldownTimeUse)))
        (else
          (goto _label))))))

(event Custom|AI_Skill1
  ;[1 1 1 1 100] Inputs
  ;;[1 1 1 1 50] Skills, Bonus, Ultime
  (bind _recieveinput (CallFunction|RecieveInput))
  (if _recieveinput
    ;;;[1 0.6128 0.3355] Check Skill 1 Reload Cooldown
    (if (<= (Variables|/Game/BP/Skills/BP_SkillParent.BP_SkillParent_C|GetSkillCooldownTimer (Variables|Default|GetSkill1Object)) 0.0)
      (Default|UseSkill (Variables|Default|GetSkill1Object)))))

(event Custom|CustomEvent
  (params (New%20State :type E_GameState%20Enum :default "NewEnumerator0"))
  ;[1 1 1] Copy of Fighter
  (switch Utilities|FlowControl|Switch|SwitchonE_GameState New%20State
    (:NewEnumerator7
      (CallFunction|SetEnable false true :!label _label))
    (:NewEnumerator3
      (CallFunction|SetEnable true false))
    (:NewEnumerator5
      (CallFunction|SetEnable false false))
    (:NewEnumerator4
      (goto _label))))

(event Custom|AI_Skill2
  ;[1 1 1 1 100] Inputs
  ;;[1 1 1 1 50] Skills, Bonus, Ultime
  (bind _recieveinput (CallFunction|RecieveInput))
  (if _recieveinput
    ;;;[1 0.6128 0.3355] Check Skill 1 Reload Cooldown
    (if (<= (Variables|/Game/BP/Skills/BP_SkillParent.BP_SkillParent_C|GetSkillCooldownTimer (Variables|Default|GetSkill2Object)) 0.0)
      (Default|UseSkill (Variables|Default|GetSkill2Object)))))

(event Custom|AI_Ultime
  ;[1 1 1 1 100] Inputs
  ;;[1 1 1 1 50] Skills, Bonus, Ultime
  (bind _recieveinput (CallFunction|RecieveInput))
  (if _recieveinput
    ;;;[1 1 1] Check Ultime Cooldown
    (if (<= (Variables|/Game/BP/Ultime/BP_UltimeParent.BP_UltimeParent_C|GetUltimeCooldownTimer (Variables|Default|GetUltimeObject)) 0.0)
      (Default|UseUltime (Variables|Default|GetUltimeObject)))))

(event Custom|AI_Bonus
  ;[1 1 1 1 100] Inputs
  ;;[1 1 1 1 50] Skills, Bonus, Ultime
  (switch Utilities|FlowControl|Switch|SwitchonE_GameState (Variables|/Game/BP/BP_GI.BP_GI_C|GetCurrentState (Variables|Default|GetGI))
    (:NewEnumerator7
      (Default|TrytoSkipBattleBeginCutscene (Variables|/Game/BP/BP_GI.BP_GI_C|GetBattleManager (Variables|Default|GetGI)) (Variables|Default|GetIndex)))
    (:NewEnumerator3
      (bind _recieveinput (CallFunction|RecieveInput))
      (if _recieveinput
        (Utilities|IsValid (Variables|Default|GetCurrentBonus)
          (:Is%20Valid
            (CallFunction|UseBonus)))))
    (:NewEnumerator4
      (Default|TrytoSkipGOCutscene (Variables|/Game/BP/BP_GI.BP_GI_C|GetBattleManager (Variables|Default|GetGI)) (Variables|Default|GetIndex)))))

(event Custom|AI_Dash
  (params (DashX :type Float%20%28double-precision%29) (DashY :type Float%20%28double-precision%29))
  ;[1 1 1 1 100] Inputs
  ;;[1 1 1 1 50] Dash
  (bind _recieveinput (CallFunction|RecieveInput))
  (if _recieveinput
    (|Dash DashX DashY)))

(event EventBeginPlay
  ;[1 1 1] Copy of Fighter
  (bind _asbp_gi (Utilities|Casting|CastToBP_GI (Game|GetGameInstance)))
  (Variables|Default|SetGI _asbp_gi)
  (Utilities|FlowControl|Sequence
    (:then_0
      (CallFunction|InitSkinMacro)
      ;;[1 1 1] Set & Store Initialize Pos & Rot
      (bind _output_get (Variables|Default|SetStartPos (Transformation|GetActorTransform)))
      (Variables|Default|SetStickRotation (.rotation _output_get))
      (Variables|Default|SetSpawnPos (Utilities|Array|MakeArray (.location (Variables|Default|GetStartPos)) (+ (.location (Variables|Default|GetStartPos)) "0.000000,300.000000,0.000000") (+ (.location (Variables|Default|GetStartPos)) "0.000000,-300.000000,0.000000")))
      (|SetUpOverHeat_2
        (:execute
          (|SetVarwithDataTable_2 ; Tapis Poussiére
            (:return
              ;;[1 1 1] Check Mappable Input
              (if (Math|Conversions|ToBoolean(Integer) (Utilities|Array|Length (Class|EnhancedInputSubsystemInterface|GetAllPlayerMappableActionKeyMappings (PlayerController|LocalPlayerSubsystems|GetEnhancedInputLocalPlayerSubsystem (Game|GetPlayerController (Variables|Default|GetIndex)))))) :!label _label
                (Variables|Default|SetMapping (Class|EnhancedInputSubsystemInterface|GetAllPlayerMappableActionKeyMappings (PlayerController|LocalPlayerSubsystems|GetEnhancedInputLocalPlayerSubsystem (Game|GetPlayerController (Variables|Default|GetIndex)))))
                (bind _mappingselectionwb (Variables|Default|GetMappingSelectionWB)
                  (:then
                    (Default|RefreshMappings _mappingselectionwb (Variables|Default|GetMapping)))
                  (:else))
                (else
                  (Utilities|FlowControl|DelayUntilNextTick)
                  (goto _label))))))))
    (:then_1
      (EventDispatchers|BindEventtoOnGameStateChanged (Variables|Default|GetGI) (delegate Custom|CustomEvent))
      (Variables|Default|SetPoolManager (Variables|/Game/BP/BP_GI.BP_GI_C|GetPoolManager (Variables|Default|GetGI)))
      (|SkillFeedback_2))))

(event Collision|EventActorBeginOverlap
  (params (OtherActor :type Actor%20Object%20Reference))
  (bind _station (Variables|Default|GetStation))
  (Utilities|FlowControl|Sequence
    (:then_0
      ;[1 0.3318 0.2701] Hit Check
      (bind _asbp_projectile_pawn (Utilities|Casting|CastToBP_ProjectilePawn OtherActor))
      (if (and (!= (Variables|Default|GetIndex) (Variables|/Game/BP/Players/Projectile/BP_ProjectilePawn.BP_ProjectilePawn_C|GetIndex _asbp_projectile_pawn)) (Utilities|Enum|NotEqual(Enum) (Variables|/Game/BP/Players/Projectile/BP_ProjectilePawn.BP_ProjectilePawn_C|GetProjectileType _asbp_projectile_pawn) "NewEnumerator5"))
        (Utilities|FlowControl|Sequence
          (:then_0
            (if (not (Variables|Default|GetIsInvulnerable))
              (if (== (Utilities|GetClass (Variables|Default|GetCurrentBonus)) "/Game/BP/Bonus/Shield/BP_Shield.BP_Shield_C")
                (Default|ChangeState (Variables|Default|GetCurrentBonus) "NewEnumerator2")
                (Variables|Default|SetCurrentBonus 0)
                (elif (Variables|Default|GetUseLife)
                  (bind _output_get (Variables|Default|SetLifeFighter (- (Variables|Default|GetLifeFighter) (Variables|/Game/BP/Players/Projectile/BP_ProjectilePawn.BP_ProjectilePawn_C|GetDamageToFighter _asbp_projectile_pawn))))
                  (CallFunction|UpdateLifeMaterialMacro)
                  (if (<= _output_get 0.0)
                    (CallFunction|Destruct true :!label _label))
                  (else
                    (goto _label))))))
          (:then_1
            (Default|Destroy _asbp_projectile_pawn)))))
    (:then_1
      (Utilities|IsValid _station
        (:Is%20Valid
          (if (Variables|/Game/BP/Players/Station/BP_Station.BP_Station_C|GetIsVulnerable _station)
            (bind _asbp_fighter_pawn (Utilities|Casting|CastToBP_FighterPawn OtherActor))
            (Utilities|FlowControl|DelayUntilNextTick)
            (Utilities|IsValid _asbp_fighter_pawn
              (:Is%20Valid
                (Variables|/Script/Engine.MovementComponent|SetVelocity (Variables|/Game/BP/Players/Fighter/BP_FighterPawn.BP_FighterPawn_C|GetFloatingPawnMovement _asbp_fighter_pawn) (Math|Vector|MakeVector (.x (* (Math|Vector|Normalize (Math|Vector|GetUnitDirection(Vector) (Transformation|GetActorLocation _station) (Transformation|GetActorLocation _asbp_fighter_pawn))) 5e+03)) (.y (* (Math|Vector|Normalize (Math|Vector|GetUnitDirection(Vector) (Transformation|GetActorLocation _station) (Transformation|GetActorLocation _asbp_fighter_pawn))) 5e+03)) 0.0))
                (Default|SetStun _asbp_fighter_pawn 1.5 3e+01)))))))))

(event EventTick
  (params (DeltaSeconds :type Float%20%28single-precision%29))
  (bind _returnvalue (Transformation|GetActorTransform))
  (bind _floatingpawnmovement (Variables|Default|GetFloatingPawnMovement))
  (bind _dashdir (Variables|Default|GetDashDir))
  (bind _frame (Variables|Default|GetFrame))
  (bind _returnvalue_2 (Transformation|GetRelativeTransform _frame))
  (bind _returnvalue_3 (* _dashdir DeltaSeconds))
  (bind _returnvalue_4 (+ _returnvalue_3 (.location _returnvalue_2)))
  ;[1 1 1] Actualiser Vision
  (Utilities|IsValid (Variables|Default|GetEnemyFighter)
    (:Is%20Valid
      (Variables|Default|SetEnemyPos (Transformation|GetActorLocation (Variables|Default|GetEnemyFighter)))
      (Variables|Default|SetDistanceToEnemy (Math|Vector|Distance(Vector) (Transformation|GetActorLocation) (Transformation|GetActorLocation (Variables|Default|GetEnemyFighter))))
      (Variables|Default|SetEnemyDirection (Math|Rotator|FindLookatRotation (Transformation|GetActorLocation) (Math|Vector|SelectVector (Transformation|GetActorLocation (Variables|/Game/BP/Players/Fighter/BP_FighterPawn.BP_FighterPawn_C|GetStation (Variables|Default|GetEnemyFighter))) (Transformation|GetActorLocation (Variables|Default|GetEnemyFighter)) (Variables|/Game/BP/Players/Fighter/BP_FighterPawn.BP_FighterPawn_C|GetIsDead (Variables|Default|GetEnemyFighter)))))
      ;[1 1 1] Copy of Fighter
      (CallFunction|SwitchControllerMacro)
      ;;[1 1 1] Tmer Check
      (CallFunction|TimerManagerMacro DeltaSeconds)
      (if (Variables|Default|GetUseDash)
        (CallFunction|DashTimerManagerMacro DeltaSeconds)
        ;;[1 1 1] State Dash Check
        (if (Variables|Default|GetIsDashing)
          ;;[1 1 1] Dash Movement
          (Transformation|SetRelativeTransform (Variables|Default|GetFrame) (Math|Transform|MakeTransform (Math|Vector|MakeVector (Math|Float|Clamp(Float) (.x _returnvalue_4) 0.0 2.1e+03) (Math|Float|Clamp(Float) (.y _returnvalue_4) 0.0 1e+03) (.z _returnvalue_4)) (.rotation _returnvalue_2) (.scale _returnvalue_2)) true false)
          (else
            (if (<= (Variables|Default|GetTimerSpin) 0.0) :!label _label
              (if (Variables|Default|GetUseAutoAim)
                ;;[1 1 1] Movement V3
                (CallFunction|MovingAutoAim)
                (else
                  (CallFunction|Moving DeltaSeconds)
                  ;;[1 1 1] Decrease Speed
                  (Variables|Default|SetSpeedX 0.0)
                  (Variables|Default|SetSpeedY 0.0)
                  (Transformation|SetActorTransform (Math|Transform|MakeTransform (Math|Vector|MakeVector (.x (.location _returnvalue)) (.y (.location _returnvalue)) 7e+01) (.rotation _returnvalue) (.scale _returnvalue)))
                  (Transformation|SetRelativeTransform (Variables|Default|GetFrame) (Math|Transform|MakeTransform (.location (Transformation|GetActorTransform)) (Variables|Default|GetEnemyDirection) "1.000000,1.000000,1.000000") true false)
                  (if (<= (Variables|Default|GetReloadTimer) 0.0)
                    (CallFunction|AIShot))
                  (if (<= (Variables|Default|GetDashTimer) 0.0)
                    (CallFunction|AIDash (.x (Math|Vector|GetForwardVector (Variables|Default|GetEnemyDirection))) (.y (Math|Vector|GetForwardVector (Variables|Default|GetEnemyDirection)))))
                  (if (<= (Variables|/Game/BP/Skills/BP_SkillParent.BP_SkillParent_C|GetSkillCooldownTimer (Variables|Default|GetSkill1Object)) 0.0)
                    (CallFunction|AISkill1))
                  (if (<= (Variables|/Game/BP/Skills/BP_SkillParent.BP_SkillParent_C|GetSkillCooldownTimer (Variables|Default|GetSkill2Object)) 0.0)
                    (CallFunction|AISkill2))
                  (if (<= (Variables|/Game/BP/Ultime/BP_UltimeParent.BP_UltimeParent_C|GetUltimeCooldownTimer (Variables|Default|GetUltimeObject)) 0.0)
                    (CallFunction|AIUltime))))
              (else
                ;;[1 1 1] Spin me round round
                (CallFunction|Spinning)))))
        (else
          (CallFunction|BoostTimerManagerMacro DeltaSeconds)
          (if (> (Variables|Default|GetBoostGauge) 0.0)
            (goto _label)
            (else
              ;;[1 0.9551 0.2425] Reset To Normal Speed
              (Variables|Default|SetIsBoosting false)
              (Variables|/Script/Engine.FloatingPawnMovement|SetAcceleration _floatingpawnmovement (Variables|Default|GetAcceleration))
              (Variables|/Script/Engine.FloatingPawnMovement|SetMaxSpeed _floatingpawnmovement (Variables|Default|GetMaxSpeed))
              (goto _label))))))
    (:Is%20Not%20Valid
      (bind _asbp_gi (Utilities|Casting|CastToBP_GI (Game|GetGameInstance)))
      (Variables|Default|SetEnemyFighter (Variables|/Game/BP/BP_BattleManager.BP_BattleManager_C|GetP1 (Variables|/Game/BP/BP_GI.BP_GI_C|GetBattleManager _asbp_gi))))))

(fn ConstructionScript
  (|CallParentFunction))

(fn Destruct
  (params (LooseUpperHand :type Boolean))
  (bind _vfx_fighterexplosion (Variables|Default|GetVFX_FighterExplosion))
  (bind _index (Variables|Default|GetIndex))
  (bind _frame (Variables|Default|GetFrame))
  (bind _gi (Variables|Default|GetGI))
  (bind _frame_2 (Variables|Default|GetFrame))
  (bind _vfx_fighterexplosion_2 (Variables|Default|GetVFX_FighterExplosion))
  (bind _battlemanager (Variables|/Game/BP/BP_GI.BP_GI_C|GetBattleManager _gi))
  (bind _p1 (Variables|/Game/BP/BP_BattleManager.BP_BattleManager_C|GetP1 _battlemanager))
  (bind _p2 (Variables|/Game/BP/BP_BattleManager.BP_BattleManager_C|GetP2 _battlemanager))
  (bind _returnvalue (Utilities|Select :Index _index :Option%200 _p2 :Option%201 _p1))
  (if (<= (Variables|Default|GetInvulnerabilityTimer) 0.0)
    (bind _currentbonus (Variables|Default|GetCurrentBonus)
      (:then
        (Default|ChangeState _currentbonus "NewEnumerator2")
        (Variables|Default|SetCurrentBonus 0))
      (:else
        _))
    (Camera|PlayWorldCameraShake "/Game/BP/BP_CameraShake2.BP_CameraShake2_C" (Transformation|GetActorLocation) 0.0 2e+03)
    (Variables|Default|SetIsDead true)
    (Default|ChangeVulnerability (Variables|/Game/BP/Players/Fighter/BP_FighterPawn.BP_FighterPawn_C|GetStation _returnvalue) (Variables|Default|GetIsOverTime))
    (bind _return (Default|IsRespawning _returnvalue))
    (if _return
      _
      (elif LooseUpperHand
        (Default|ChangeVulnerability (Variables|Default|GetStation) LooseUpperHand)
        (Audio|PlaySound2D "/Game/Sounds/SoundEffect/ShieldDown.ShieldDown" 1.0 1.0 0.0 0 0)
        (Variables|Default|SetRespawnTimer (Variables|Default|GetRespawnCooldown))
        (Rendering|SetVisibility _frame false true)
        (Collision|SetActorEnableCollision false)
        (LocalVariables|SetKillPosition (Transformation|GetWorldLocation _frame))
        (Transformation|SetWorldLocation _vfx_fighterexplosion_2 (LocalVariables|GetKillPosition) false false)
        (Rendering|SetVisibility _vfx_fighterexplosion_2 true false)
        (Components|Activation|Activate _vfx_fighterexplosion_2 false)
        (Default|CallOnKilled (Variables|Default|GetIndex))
        (Audio|PlaySound2D "/Game/Sounds/SoundEffect/Explosion.Explosion" 1.0 1.0 0.0 0 0)
        (Variables|Default|SetRespawnPosIndex (Math|Random|RandomInteger 3))
        (return false)
        (else
          _)))
    (Variables|Default|SetRespawnTimer (Variables|Default|GetRespawnCooldown))
    (Rendering|SetVisibility _frame_2 false true)
    (Collision|SetActorEnableCollision false)
    (LocalVariables|SetKillPosition (Transformation|GetWorldLocation _frame_2))
    (Transformation|SetWorldLocation _vfx_fighterexplosion (LocalVariables|GetKillPosition) false false)
    (Rendering|SetVisibility _vfx_fighterexplosion true false)
    (Components|Activation|Activate _vfx_fighterexplosion false)
    (Default|CallOnKilled (Variables|Default|GetIndex))
    (Audio|PlaySound2D "/Game/Sounds/SoundEffect/Explosion.Explosion" 1.0 1.0 0.0 0 0)
    (Variables|Default|SetRespawnPosIndex (Math|Random|RandomInteger 3))
    (return false)))

(event Custom|BonusPickup
  (params (Fighter :type BP%20Fighter%20Pawn%20Object%20Reference))
  (bind _recieveinput (CallFunction|RecieveInput))
  (if _recieveinput
    (CallFunction|CreateFeedbackText (Utilities|Text|ToText(Name) (Variables|/Game/BP/Bonus/BP_BonusParent.BP_BonusParent_C|GetName (Variables|Default|GetCurrentBonus))))))

(event Custom|RecoverSkill1
  (params (NewState :type Enum_SkillState%20Enum :default "NewEnumerator0") (Index :type Integer))
  (switch Utilities|FlowControl|Switch|SwitchonEnum_SkillState NewState
    (:NewEnumerator0
      (CallFunction|CreateFeedbackText (Utilities|Text|ToText(Name) (Variables|/Game/BP/Skills/BP_SkillParent.BP_SkillParent_C|GetName (Variables|Default|GetSkill1Object)))))))

(event Custom|RecoverSkill2
  (params (NewState :type Enum_SkillState%20Enum :default "NewEnumerator0") (Index :type Integer))
  (switch Utilities|FlowControl|Switch|SwitchonEnum_SkillState NewState
    (:NewEnumerator0
      (CallFunction|CreateFeedbackText (Utilities|Text|ToText(Name) (Variables|/Game/BP/Skills/BP_SkillParent.BP_SkillParent_C|GetName (Variables|Default|GetSkill2Object)))))))