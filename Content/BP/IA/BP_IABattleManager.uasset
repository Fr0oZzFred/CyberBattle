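; Battle manager actor for a two-player station fight, running the match from intro cutscene to game over and registering itself on BP_GI.
; Game state changes toggle its Tick, which counts down the timer, then starts overtime by making both stations vulnerable.
; Station vulnerability sets the upper-hand state, and station life picks the winner's ending sequence.
; Events drive UI, skippable cutscenes and the fight countdown with timed bloc and wave spawns.
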(event Custom|RemoveBB_CutsceneBorders
  ;[1 1 1 1 50] BattleBegin
  (Default|RemoveCutsceneBorders (Variables|/Game/UI/HUD_Manager.HUD_Manager_C|GetBattleBegin (Variables|/Game/BP/BP_GI.BP_GI_C|GetUIManager (Variables|Default|GetGI)))))

(event Custom|StartFight
  (bind _gi (Variables|Default|GetGI))
  ;[1 1 1 1 50] BattleBegin
  (Default|SetGameState (Variables|Default|GetGI) "NewEnumerator3")
  (Default|SetEnable (Variables|BlocManagement|GetGrid) false false)
  (CallFunction|SetEnable false false)
  (Variables|/Game/BP/BP_GI.BP_GI_C|SetInCinematic _gi true)
  (Default|StartFight (Variables|/Game/UI/HUD_Manager.HUD_Manager_C|GetInBattle (Variables|/Game/BP/BP_GI.BP_GI_C|GetUIManager _gi)))
  (|SpawnBlocs
    (:Completed
      (Utilities|FlowControl|Delay (Variables|Intro|GetTelegraph%20Time))
      (Default|SetEnable (Variables|Default|GetP1) true false)
      (Utilities|FlowControl|Delay (- (Variables|Intro|GetCountdownDuration) (Variables|Intro|GetWaveAppearTime)))
      (Default|SpawnWavePattern (Variables|BlocManagement|GetGrid))
      (Utilities|FlowControl|Delay (Variables|Intro|GetWaveAppearTime))
      (Default|SetEnable (Variables|BlocManagement|GetGrid) true false)
      (Variables|/Game/BP/BP_GI.BP_GI_C|SetInCinematic (Variables|Default|GetGI) false)
      (CallFunction|SetEnable true false))))

(event Custom|PlayBattleBeginAnim_UI
  ;[1 1 1 1 50] BattleBegin
  (Default|PlayBattleBeginAnim (Variables|/Game/UI/HUD_Manager.HUD_Manager_C|GetBattleBegin (Variables|/Game/BP/BP_GI.BP_GI_C|GetUIManager (Variables|Default|GetGI)))))

(event Custom|PlayP1_BattleBeginAnim_UI
  ;[1 1 1 1 50] BattleBegin
  (Default|PlayPlayerAnim (Variables|/Game/UI/HUD_Manager.HUD_Manager_C|GetBattleBegin (Variables|/Game/BP/BP_GI.BP_GI_C|GetUIManager (Variables|Default|GetGI)))))

(event Custom|AddBB_CutsceneBorders
  ;[1 1 1 1 50] BattleBegin
  (Default|AddCutsceneBorders (Variables|/Game/UI/HUD_Manager.HUD_Manager_C|GetBattleBegin (Variables|/Game/BP/BP_GI.BP_GI_C|GetUIManager (Variables|Default|GetGI)))))

(event Custom|RemoveGO_CutsceneBorders
  ;[1 1 1 1 50] GameOver
  (Default|RemoveCutsceneBorders (Variables|/Game/UI/HUD_Manager.HUD_Manager_C|GetGame%20Over (Variables|/Game/BP/BP_GI.BP_GI_C|GetUIManager (Variables|Default|GetGI)))))

(event Custom|SetStateToGO
  (bind _gi (Variables|Default|GetGI))
  ;[1 1 1 1 50] GameOver
  (Variables|/Game/BP/BP_GI.BP_GI_C|SetInCinematic _gi false)
  (Default|SetGameState _gi "NewEnumerator4")
  (Default|DisplayWinnerSkipButton (Variables|/Game/UI/HUD_Manager.HUD_Manager_C|GetGame%20Over (Variables|/Game/BP/BP_GI.BP_GI_C|GetUIManager (Variables|Default|GetGI))) (Variables|Default|GetP2_Won)))

(event Custom|StartGameOverAnim
  (bind _gi (Variables|Default|GetGI))
  (bind _battleendsequence (Variables|Sequences|GetBattleEndSequence))
  ;[1 1 1 1 50] GameOver
  (if (not (Variables|/Game/BP/BP_GI.BP_GI_C|GetInCinematic _gi))
    (Variables|/Game/BP/BP_GI.BP_GI_C|SetInCinematic _gi true)
    (Variables|Default|SetP2_Won (< (Variables|/Game/BP/Players/Station/BP_Station.BP_Station_C|GetLifeStation (Variables|/Game/BP/Players/Fighter/BP_FighterPawn.BP_FighterPawn_C|GetStation (Variables|Default|GetP1))) (Variables|/Game/BP/Players/Station/BP_Station.BP_Station_C|GetLifeStation (Variables|/Game/BP/Players/Fighter/BP_FighterPawn.BP_FighterPawn_C|GetStation (Variables|Default|GetP2)))))
    (Class|LevelSequenceActor|SetSequence _battleendsequence (select (Variables|Default|GetP2_Won) "/Game/Sequences/BattleOver_Win_P2.BattleOver_Win_P2" "/Game/Sequences/BattleOver_Win_P1.BattleOver_Win_P1"))
    (Sequencer|Player|Play (Variables|/Script/LevelSequence.LevelSequenceActor|GetSequencePlayer _battleendsequence) :!class /Script/MovieScene.MovieSceneSequencePlayer)))

(event Custom|StartGO_AnimUI
  ;[1 1 1 1 50] GameOver
  (Default|StartGameOverAnim (Variables|/Game/UI/HUD_Manager.HUD_Manager_C|GetGame%20Over (Variables|/Game/BP/BP_GI.BP_GI_C|GetUIManager (Variables|Default|GetGI)))))

(event Custom|TryToSkipBattleBeginCutscene
  (params (Index :type Integer))
  ;[1 1 1 1 50] BattleBegin
  (Default|OnSkip (Variables|/Game/UI/HUD_Manager.HUD_Manager_C|GetBattleBegin (Variables|/Game/BP/BP_GI.BP_GI_C|GetUIManager (Variables|Default|GetGI))) Index)
  (Utilities|Array|SetArrayElem (Variables|Default|GetWantsToSkipBattleBegin) Index true)
  (if (Utilities|PlayersWanttoSkip)
    (Utilities|SkipCutscenetoFrame (Variables|/Script/LevelSequence.LevelSequenceActor|GetSequencePlayer (Variables|Sequences|GetBattleBeginSequence)) (Variables|Sequences|GetBattleBegin_SkipFramePoint)
      (:Skipped
        (Default|StopPlayersAnim (Variables|/Game/UI/HUD_Manager.HUD_Manager_C|GetBattleBegin (Variables|/Game/BP/BP_GI.BP_GI_C|GetUIManager (Variables|Default|GetGI))))))))

(event Custom|TryToSkipGO_Cutscene
  (params (Index :type Integer))
  ;[1 1 1 1 50] GameOver
  (if (== Index (Variables|Default|GetP2_Won))
    (Utilities|SkipCutscenetoFrame (Variables|/Script/LevelSequence.LevelSequenceActor|GetSequencePlayer (Variables|Sequences|GetBattleEndSequence)) (Variables|Sequences|GetGO_SkipFramePoint))))

(event Custom|PlayP2_BattleBeginAnim_UI
  ;[1 1 1 1 50] BattleBegin
  (Default|PlayPlayerAnim (Variables|/Game/UI/HUD_Manager.HUD_Manager_C|GetBattleBegin (Variables|/Game/BP/BP_GI.BP_GI_C|GetUIManager (Variables|Default|GetGI))) 1))

(event Custom|PlayBattleBeginSequence
  ;[1 1 1 1 50] BattleBegin
  (Sequencer|Player|Play (Variables|/Script/LevelSequence.LevelSequenceActor|GetSequencePlayer (Variables|Sequences|GetBattleBeginSequence)) :!class /Script/MovieScene.MovieSceneSequencePlayer))

(event EventBeginPlay
  ;[1 1 1 1 50] BeginPlay
  (bind _asbp_gi (Utilities|Casting|CastToBP_GI (Game|GetGameInstance)))
  (bind _output_get (Variables|Default|SetGI _asbp_gi))
  (Variables|/Game/BP/BP_GI.BP_GI_C|SetBattleManager _output_get self)
  (EventDispatchers|BindEventtoOnGameStateChanged (Variables|Default|GetGI) (|OnGameState_Changed))
  (Utilities|FlowControl|Sequence
    (:then_0
      (bind _fighter (Utilities|GetFighter))
      (bind _output_get_2 (Variables|Default|SetP1 _fighter))
      (Utilities|InitforBattle _output_get_2)
      (Utilities|SetPlayerValid :!label _label
        (:Both%20Valid
          (EventDispatchers|BindEventtoOnVulnerableChanged (Variables|/Game/BP/Players/Fighter/BP_FighterPawn.BP_FighterPawn_C|GetStation (Variables|Default|GetP1)) (|OnVulnChanged)))))
    (:then_1
      (bind _fighter_2 (Utilities|GetFighter 1))
      (bind _output_get_3 (Variables|Default|SetP2 _fighter_2))
      (Utilities|InitforBattle _output_get_3)
      (goto _label))
    (:then_2
      (Utilities|SetTimetoBattleTimer)
      (Variables|Bonus|SetBonusListActive (Variables|/Game/BP/BP_GI.BP_GI_C|GetBonusListActive (Variables|Default|GetGI))))))

(event EventTick
  (params (DeltaSeconds :type Float%20%28single-precision%29))
  (bind _p1 (Variables|Default|GetP1))
  (bind _p2 (Variables|Default|GetP2))
  (bind _station (Variables|/Game/BP/Players/Fighter/BP_FighterPawn.BP_FighterPawn_C|GetStation _p1))
  (bind _station_2 (Variables|/Game/BP/Players/Fighter/BP_FighterPawn.BP_FighterPawn_C|GetStation _p2))
  ;[1 1 1 1 50] Tick
  (bind _output_get (Variables|Default|SetTime (- (stale _output_get) DeltaSeconds)))
  (Utilities|SetTimetoBattleTimer)
  (if (<= _output_get 0.0)
    (bind _output_get_2 (Variables|Default|SetBattleTimer (Utilities|Text|ToText(String) (Utilities|String|Append "+" (Utilities|String|ToString(Text) (stale _output_get_2))))))
    (Utilities|FlowControl|Sequence
      (:then_0
        (Default|ChangeVulnerability _station true)
        (Variables|/Game/BP/Players/Fighter/BP_FighterPawn.BP_FighterPawn_C|SetIsOverTime _p1 true))
      (:then_1
        (Default|ChangeVulnerability _station_2 true)
        (Variables|/Game/BP/Players/Fighter/BP_FighterPawn.BP_FighterPawn_C|SetIsOverTime _p2 true)
        ;;[1 1 1] Tie check
        (if (or (<= (Variables|/Game/BP/Players/Station/BP_Station.BP_Station_C|GetLifeStation _station) 0.0) (<= (Variables|/Game/BP/Players/Station/BP_Station.BP_Station_C|GetLifeStation _station_2) 0.0))
          (CallFunction|StartGameOverAnim))))))

(event Input|KeyboardEvents|<
  (params (Key :type Key%20Structure))
  ;[1 1 1 1 50] CheatCodes
  (:Pressed
    (Variables|Default|SetTime 0.0)
    (Default|DamageStation (Variables|/Game/BP/Players/Fighter/BP_FighterPawn.BP_FighterPawn_C|GetStation (Variables|Default|GetP2)) 9e+01)))

(fn ConstructionScript)

(fn SetUpperHandState
  (params (New%20State :type E_UpperHand%20Enum :default "NewEnumerator0"))
  (if (Utilities|Enum|NotEqual(Enum) New%20State (stale _output_get))
    (bind _output_get (Variables|UpperHand|SetUpperHandState New%20State))
    (Default|CallOnUpperHandStateChanged _output_get)))

(event Custom|OnVulnerableChanged
  (bind _p1 (Variables|Default|GetP1))
  (bind _station (Variables|/Game/BP/Players/Fighter/BP_FighterPawn.BP_FighterPawn_C|GetStation _p1))
  (bind _isvulnerable (Variables|/Game/BP/Players/Station/BP_Station.BP_Station_C|GetIsVulnerable _station))
  (if (and (not _isvulnerable) (not (Variables|/Game/BP/Players/Station/BP_Station.BP_Station_C|GetIsVulnerable (Variables|/Game/BP/Players/Fighter/BP_FighterPawn.BP_FighterPawn_C|GetStation (Variables|Default|GetP2)))))
    (CallFunction|SetUpperHandState "NewEnumerator0")
    (else
      (CallFunction|SetUpperHandState (select _isvulnerable "NewEnumerator2" "NewEnumerator1")))))

(event Custom|OnGameStateChanged
  (params (New%20State :type E_GameState%20Enum :default "NewEnumerator0"))
  (switch Utilities|FlowControl|Switch|SwitchonE_GameState New%20State
    (:NewEnumerator7
      (if (Variables|Intro|GetSkipIntro)
        (Utilities|FlowControl|DelayUntilNextTick)
        (Default|SetGameState (Variables|Default|GetGI) "NewEnumerator3")
        (else
          (CallFunction|PlayBattleBeginSequence)
          (CallFunction|SetEnable false false :!label _label))))
    (:NewEnumerator3
      (CallFunction|SetEnable (Variables|Default|GetPlayersValid) false))
    (:NewEnumerator5
      (goto _label))
    (:NewEnumerator4
      (goto _label))))

(fn SetEnable
  (params (Enable :type Boolean) (Hide :type Boolean))
  (Actor|Tick|SetActorTickEnabled Enable)
  (return false))