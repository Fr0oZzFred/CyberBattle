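; Sound manager actor that plays random 2D music for the main menu and in-game states, driven by BP_GI's game-state event.
; The first in-game track picked also sets a matching pre-analyzed loudness (LoudnessNRT) asset.
; Tick, enabled two frames after BeginPlay, samples that loudness at looped actor lifetime to pulse the post-process volume's bloom size with the music.
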(event Custom|OnGameStateChanged
  (params (New%20State :type E_GameState%20Enum :default "NewEnumerator0"))
  (switch Utilities|FlowControl|Switch|SwitchonE_GameState New%20State
    (:NewEnumerator1
      (Audio|PlaySound2D (Utilities|Select :Index (Math|Random|RandomIntegerinRange 0 1) :Option%200 "/Game/Sounds/Placeholder/Stellaris_Apocalypse_Soundtrack_-_Hostile_Fleet_Detected.Stellaris_Apocalypse_Soundtrack_-_Hostile_Fleet_Detected" :Option%201 "/Game/Sounds/Placeholder/New_Danganronpa_V3_O_S_T__White_-_46__Climax_Reasoning_V3.New_Danganronpa_V3_O_S_T__White_-_46__Climax_Reasoning_V3") 1.0 1.0 0.0 0 0))
    (:NewEnumerator3
      (Utilities|IsValid (Variables|Default|GetCurrent%20Sound%20LNRT)
        (:Is%20Not%20Valid
          (bind _output_get (Variables|Default|SetRandom (Math|Random|RandomIntegerinRange 0 2)))
          (Audio|PlaySound2D (Utilities|Select :Index _output_get :Option%200 "/Game/Sounds/Placeholder/Cyber-Space-1-5-Dropaholic-Sonic-Frontiers-_OST_.Cyber-Space-1-5-Dropaholic-Sonic-Frontiers-_OST_" :Option%201 "/Game/Sounds/Placeholder/Nightcore-Time-Lapse.Nightcore-Time-Lapse" :Option%202 "/Game/Sounds/Placeholder/Pokémon-Sword-_-Shield-OST-Gym-Leader-Battle-_Full-In-Game-Version_.Pokémon-Sword-_-Shield-OST-Gym-Leader-Battle-_Full-In-Game-Version_") 1.0 1.0 0.0 0 0)
          (Variables|Default|SetCurrent%20Sound%20LNRT (Utilities|Select :Index _output_get :Option%200 "/Game/Sounds/Placeholder/Sonic.Sonic" :Option%201 "/Game/Sounds/Placeholder/Nightcore.Nightcore" :Option%202 "/Game/Sounds/Placeholder/Pokemon.Pokemon")))))))

(event EventTick
  (params (DeltaSeconds :type Float%20%28single-precision%29))
  (bind _current_sound_lnrt (Variables|Default|GetCurrent%20Sound%20LNRT))
  (Variables|/Script/Engine.PostProcessVolume|SetSettings (Variables|Default|GetPP) (Utilities|Struct|MakePostProcessSettings (* (Variables|Default|GetPP_Bloom_Size) (Class|LoudnessNRT|GetNormalizedLoudnessatTime _current_sound_lnrt (Math|Float|%(Float) (Actor|GetGameTimeSinceCreation) (Variables|/Script/Engine.SoundBase|GetDuration (Variables|/Script/AudioAnalyzer.AudioAnalyzerNRT|GetSound _current_sound_lnrt)))) (Variables|Default|GetSound%20Effect%20Scale)))))

(event EventBeginPlay
  (bind _asbp_gi (Utilities|Casting|CastToBP_GI (Game|GetGameInstance)))
  (EventDispatchers|AssignOnGameStateChanged _asbp_gi (delegate Custom|OnGameStateChanged))
  (bind _returnvalue (Actor|GetActorOfClass "/Script/Engine.PostProcessVolume"))
  (Variables|Default|SetPP _returnvalue)
  (Variables|Default|SetPP_Bloom_Size (Utilities|Struct|BreakPostProcessSettings (Variables|/Script/Engine.PostProcessVolume|GetSettings _returnvalue)))
  (Actor|Tick|SetActorTickEnabled false)
  (Utilities|FlowControl|DelayUntilNextTick)
  (Utilities|FlowControl|DelayUntilNextTick)
  (Actor|Tick|SetActorTickEnabled true))

(fn ConstructionScript)