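; BP_PoolManager is an object pool for projectiles that carry separate damage values for stations and fighters.
; On BeginPlay it registers itself on the BP_GI game instance, then pre-spawns a set amount of projectiles, disabled and hidden.
; SpawnProjectile re-initializes and enables the first unused projectile with the shot's parameters.
; When none is free, it spawns a new one and adds it to the pool.
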(event EventBeginPlay
  (bind _asbp_gi (Utilities|Casting|CastToBP_GI (Game|GetGameInstance)))
  (Variables|/Game/BP/BP_GI.BP_GI_C|SetPoolManager _asbp_gi self)
  (Utilities|Init))

(fn ConstructionScript)

(fn SpawnProjectile
  (params (SpawnTransform :type Transform) (Index :type Integer) (Direction :type Vector) (speed :type Float%20%28double-precision%29) (DamageToStation :type Float%20%28double-precision%29) (DamageToFighter :type Float%20%28double-precision%29) (Fighter :type BP%20Fighter%20Pawn%20Object%20Reference) (MaxDistance :type Float%20%28double-precision%29) (Skin :type S%20Projectile%20Skin%20Structure) (SuperShot :type Boolean))
  (bind (_array_element _array_index) (Utilities|Array|ForEachLoopwithBreak (Variables|Projectiles|GetProjectilesPool) :!label _label)
    (:LoopBody
      (if (not (Variables|/Game/BP/Players/Projectile/BP_ProjectilePawn.BP_ProjectilePawn_C|GetUsed _array_element))
        (LocalVariables|SetActorIndex _array_index)
        (goto _label Break)))
    (:Completed
      (if (>= (LocalVariables|GetActorIndex) 0)
        (Default|Init (Utilities|Array|Get(acopy) (Variables|Projectiles|GetProjectilesPool) (LocalVariables|GetActorIndex)) SpawnTransform Index Direction speed DamageToStation DamageToFighter Fighter MaxDistance Skin SuperShot)
        (Default|SetEnable (Utilities|Array|Get(acopy) (Variables|Projectiles|GetProjectilesPool) (LocalVariables|GetActorIndex)) true false)
        (else
          (bind _returnvalue (Game|SpawnActorfromClass (Variables|Projectiles|GetProjectileType) SpawnTransform "Undefined" 0 Index Direction speed DamageToStation DamageToFighter Fighter MaxDistance Skin SuperShot 0))
          (Utilities|Array|Add (Variables|Projectiles|GetProjectilesPool) _returnvalue))))))