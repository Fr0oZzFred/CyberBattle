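; Game mode for local multiplayer that creates a player and controller for each PlayerStart index that has a matching numeric tag.
; On BeginPlay it spawns a BP_InputReciever at the start in that array slot (not necessarily the tagged one), possesses it and adds that player's Enhanced Input mapping context.
; SpawnPlayer later spawns a BP_FighterPawn at a receiver's transform and hands possession to it; SetCamera is a stub.
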(event EventBeginPlay
  (CallFunction|GetPlayerStartPoints)
  (CallFunction|SpawnInputRecievers))

(fn ConstructionScript)

(fn GetPlayerStartPoints
  (bind _outactors (Actor|GetAllActorsOfClass "/Script/Engine.PlayerStart"))
  (Variables|Default|SetPlayerStartArray _outactors))

(fn SpawnInputRecievers
  (for (_ _array_index) (Variables|Default|GetPlayerStartArray)
    (LocalVariables|SetIndex _array_index)
    (for _array_element (Variables|Default|GetPlayerStartArray)
      (if (== (CallFunction|NametoInt _array_element) (LocalVariables|GetIndex))
        (Class|GameplayStatics|CreatePlayer (LocalVariables|GetIndex))
        (bind _returnvalue (Game|SpawnActorfromClass "/Game/BP/Players/Fighter/BP_InputReciever.BP_InputReciever_C" (Transformation|GetActorTransform (Utilities|Array|Get(acopy) (Variables|Default|GetPlayerStartArray) (LocalVariables|GetIndex))) "Undefined" 0 (LocalVariables|GetIndex) 0))
        (Utilities|Array|AddUnique (Variables|Default|GetPlayerInputRecieverArray) _returnvalue)
        ;[1 1 1] Posses Pawn with each controller
        (Pawn|Possess (Game|GetPlayerController (LocalVariables|GetIndex)) _returnvalue)
        (Utilities|Array|AddUnique (Variables|Default|GetPlayerControllerArray) (Game|GetPlayerController (LocalVariables|GetIndex)))
        ;[1 1 1] Add Mapping Contexts to each player controller
        (Input|AddMappingContext (PlayerController|LocalPlayerSubsystems|GetEnhancedInputLocalPlayerSubsystem (Game|GetPlayerController (LocalVariables|GetIndex))) (Utilities|Array|Get(acopy) (Variables|Default|GetInputContexts) (LocalVariables|GetIndex)) 0 "(bIgnoreAllPressedKeysUntilRelease=True,bForceImmediately=False)")))))

(fn NametoInt
  (params (PlayerStart :type Player%20Start%20Object%20Reference))
  (return (Math|Conversions|ToInteger(Byte) (Utilities|String|ToString(Name) (Variables|/Script/Engine.PlayerStart|GetPlayerStartTag PlayerStart)))))

(fn SetCamera
  (params (CamToUse :type Actor%20Object%20Reference))
  (return false))

(fn SpawnPlayer
  (params (CurrentPlayerIndex :type Integer) (InputReciever :type BP%20Input%20Reciever%20Object%20Reference))
  (bind _returnvalue (Game|SpawnActorfromClass "/Game/BP/Players/Fighter/BP_FighterPawn.BP_FighterPawn_C" (Transformation|GetActorTransform InputReciever) "Undefined" 0 CurrentPlayerIndex 0))
  (Pawn|Possess (Game|GetPlayerController CurrentPlayerIndex) _returnvalue)
  (return false))