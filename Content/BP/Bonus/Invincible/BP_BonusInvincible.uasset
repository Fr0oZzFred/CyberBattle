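; Invincibility bonus, a child of a base bonus class, that shows a shield VFX on the fighter using it.
; On use it enables tick and activates the effect, then snaps to the fighter's transform each frame rather than attaching.
; Shield color and scale come from a VFX settings data table row, with errors reported if missing.
; It hides the effect in the None state and hands it to the parent for pausing.
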(event EventTick
  (params (DeltaSeconds :type Float%20%28single-precision%29))
  (|CallParentFunction DeltaSeconds)
  (Transformation|SetActorTransform (Transformation|GetActorTransform (Variables|Default|GetFighterUser))))

(event EventBeginPlay
  (|CallParentFunction))

(fn ConstructionScript
  (|CallParentFunction))

(fn UseBonus
  (|CallParentFunction)
  (Actor|Tick|SetActorTickEnabled true)
  (Components|Activation|Activate (Variables|Default|GetVFX_BonusInvincibility) true))

(fn PauseVFX
  (params (Enable :type Boolean))
  (Variables|Default|SetVFXs (Utilities|Array|MakeArray (Variables|Default|GetVFX_BonusInvincibility)))
  (|CallParentFunction Enable))

(fn ChangeState
  (params (state :type Enum_BonusState%20Enum :default "NewEnumerator2"))
  (|CallParentFunction state)
  (switch Utilities|FlowControl|Switch|SwitchonEnum_BonusState (Variables|Default|GetBonusState)
    (:NewEnumerator2
      (Development|SetHiddeninGame (Variables|Default|GetVFX_BonusInvincibility) true false))))

(fn InitVFX
  (bind _vfx_bonusinvincibility (Variables|Default|GetVFX_BonusInvincibility))
  (bind _returnvalue (CallFunction|GetVFXSettingsRowName))
  (bind _vfxsettings (Variables|Default|GetVFXSettings)
    (:then
      (bind _returnvalue_2 (Utilities|GetDataTableRow _vfxsettings _returnvalue)
        (:then
          (Effects|Components|ParticleSystem|SetColorParameter _vfx_bonusinvincibility "Color" (.Color (Utilities|Struct|BreakS_BonusInvincibility _returnvalue_2)))
          (Effects|Components|ParticleSystem|SetVectorParameter _vfx_bonusinvincibility "ShieldScale" (.ShieldScale (Utilities|Struct|BreakS_BonusInvincibility _returnvalue_2))))
        (:RowNotFound
          (CallFunction|CallVFXSettingsException "NOTFOUND"))))
    (:else
      (CallFunction|CallVFXSettingsException "NULL"))))