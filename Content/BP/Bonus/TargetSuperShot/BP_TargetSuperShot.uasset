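; BP_TargetSuperShot is a fighter bonus that fires one oversized projectile dealing damage equal to the user's max life.
; BeginPlay caches the pool manager and opposing fighter; using the bonus activates a target VFX, styled from a settings data table.
; Once Duration runs out, Tick turns the user toward the enemy, spawns a pooled projectile ranged to their distance, plays a random laser sound, then clears and destroys itself.
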(event EventBeginPlay
  (|CallParentFunction)
  (bind _asbp_gi (Utilities|Casting|CastToBP_GI (Game|GetGameInstance)))
  (Variables|Default|SetPoolManager (Variables|/Game/BP/BP_GI.BP_GI_C|GetPoolManager _asbp_gi))
  (bind _asbp_gi_2 (Utilities|Casting|CastToBP_GI (Game|GetGameInstance)))
  (if (== (Variables|/Game/BP/Players/Fighter/BP_FighterPawn.BP_FighterPawn_C|GetIndex (Variables|Default|GetFighterUser)) 0)
    (Variables|Default|SetFighterEnemy (Variables|/Game/BP/BP_BattleManager.BP_BattleManager_C|GetP2 (Variables|/Game/BP/BP_GI.BP_GI_C|GetBattleManager _asbp_gi_2)))
    (else
      (Variables|Default|SetFighterEnemy (Variables|/Game/BP/BP_BattleManager.BP_BattleManager_C|GetP1 (Variables|/Game/BP/BP_GI.BP_GI_C|GetBattleManager _asbp_gi_2))))))

(event EventTick
  (params (DeltaSeconds :type Float%20%28single-precision%29))
  (bind _fighteruser (Variables|Default|GetFighterUser))
  (bind _returnvalue (Transformation|GetActorForwardVector _fighteruser))
  (|CallParentFunction DeltaSeconds)
  (if (<= (Variables|Default|GetDuration) 0.0)
    (Transformation|SetRelativeTransform (Variables|/Game/BP/Players/Fighter/BP_FighterPawn.BP_FighterPawn_C|GetFrame _fighteruser) (Math|Transform|MakeTransform (.location (Transformation|GetActorTransform _fighteruser)) (Variables|/Game/BP/Players/Fighter/BP_FighterPawn.BP_FighterPawn_C|GetEnemyDirection _fighteruser) "1.000000,1.000000,1.000000") true false)
    (Default|SpawnProjectile (Variables|Default|GetPoolManager) (Math|Transform|MakeTransform (Transformation|GetSocketLocation (Variables|/Game/BP/Players/Fighter/BP_FighterPawn.BP_FighterPawn_C|GetFrame _fighteruser) "ProjSpawnPoint") (.rotation (Transformation|GetActorTransform _fighteruser)) "2.000000,2.000000,2.000000") (Variables|/Game/BP/Players/Fighter/BP_FighterPawn.BP_FighterPawn_C|GetIndex _fighteruser) (Math|Vector|MakeVector (.x _returnvalue) (.y _returnvalue) (.z _returnvalue)) 3e+03 0.0 (Variables|/Game/BP/Players/Fighter/BP_FighterPawn.BP_FighterPawn_C|GetMaxLifeFighter _fighteruser) (Transformation|GetDistanceTo (Variables|Default|GetFighterEnemy) (Variables|Default|GetFighterUser)) (select (Variables|Default|GetVFXBaseSettings) (Variables|Default|GetProjectile%20Skin) (.projectile (Variables|/Game/BP/Players/Fighter/BP_FighterPawn.BP_FighterPawn_C|GetPlayerSkin _fighteruser))) "NewEnumerator1")
    (Audio|PlaySound2D (Utilities|Select :Index (Math|Random|RandomInteger 5) :Option%200 "/Game/Sounds/SoundEffect/Fighter/laserShoot1.laserShoot1" :Option%201 "/Game/Sounds/SoundEffect/Fighter/laserShoot2.laserShoot2" :Option%202 "/Game/Sounds/SoundEffect/Fighter/laserShoot3.laserShoot3" :Option%203 "/Game/Sounds/SoundEffect/Fighter/laserShoot4.laserShoot4" :Option%204 "/Game/Sounds/SoundEffect/Fighter/laserShoot5.laserShoot5" :Option%205 "/Game/Sounds/SoundEffect/Fighter/laserShoot6.laserShoot6") 1.0 1.0 0.0 0 0)
    (CallFunction|ChangeState "NewEnumerator2")
    (Variables|/Game/BP/Players/Fighter/BP_FighterPawn.BP_FighterPawn_C|SetCurrentBonus (Variables|Default|GetFighterUser) 0)
    (Actor|DestroyActor)))

(fn ConstructionScript
  (|CallParentFunction))

(fn InitVFX
  (bind _returnvalue (CallFunction|GetVFXSettingsRowName))
  (bind _vfxsettings (Variables|Default|GetVFXSettings)
    (:then
      (bind _returnvalue_2 (Utilities|GetDataTableRow _vfxsettings _returnvalue)
        (:then
          (Effects|Components|ParticleSystem|SetColorParameter (Variables|Default|GetVFX_TargetShot) "Color" (.Color (Utilities|Struct|BreakS_TargetShot _returnvalue_2)))
          (Variables|Default|SetProjectile%20Skin (.ProjectileSkin (Utilities|Struct|BreakS_TargetShot _returnvalue_2))))
        (:RowNotFound
          (CallFunction|CallVFXSettingsException "NOTFOUND"))))
    (:else
      (CallFunction|CallVFXSettingsException "NULL"))))

(fn UseBonus
  (|CallParentFunction)
  (Components|Activation|Activate (Variables|Default|GetVFX_TargetShot) true))