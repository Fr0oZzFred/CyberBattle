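; BP_Shield is a bonus Blueprint for a shield pickup that shows an invincibility VFX and changes state when its duration runs out.
; It extends a parent bonus class, activating the VFX on use, registering it for pausing, and checking Duration each tick.
; InitVFX passes Duration to the effect and pulls its color from a settings data table row, reporting missing tables or rows through an exception call.
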(event EventTick
  (params (DeltaSeconds :type Float%20%28single-precision%29))
  (|CallParentFunction DeltaSeconds)
  (if (<= (Variables|Default|GetDuration) 0.0)
    (CallFunction|ChangeState "NewEnumerator2")))

(event EventBeginPlay
  (|CallParentFunction))

(fn ConstructionScript
  (|CallParentFunction))

(fn UseBonus
  (|CallParentFunction)
  (Components|Activation|Activate (Variables|Default|GetVFX_BonusInvincibility) true))

(fn PauseVFX
  (params (Enable :type Boolean))
  (Variables|Default|SetVFXs (Utilities|Array|MakeArray (Variables|Default|GetVFX_BonusInvincibility)))
  (|CallParentFunction Enable))

(fn InitVFX
  (Effects|Components|ParticleSystem|SetFloatParameter (Variables|Default|GetVFX_BonusInvincibility) "Duration" (Variables|Default|GetDuration))
  (bind _returnvalue (CallFunction|GetVFXSettingsRowName))
  (bind _vfxsettings (Variables|Default|GetVFXSettings)
    (:then
      (bind _returnvalue_2 (Utilities|GetDataTableRow _vfxsettings _returnvalue)
        (:then
          (Effects|Components|ParticleSystem|SetColorParameter (Variables|Default|GetVFX_BonusInvincibility) "Color" (Utilities|Struct|BreakS_Shield _returnvalue_2)))
        (:RowNotFound
          (CallFunction|CallVFXSettingsException "NOTFOUND"))))
    (:else
      (CallFunction|CallVFXSettingsException "NULL"))))