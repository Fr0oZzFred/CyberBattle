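; BP_BonusBox is a pickup that grants a bonus to the BP_FighterPawn overlapping it.
; On BeginPlay it picks a random DataTable row, which sets the plane's material and the bonus class to spawn.
; A fighter without a bonus receives the spawned actor, used immediately if Auto is set, otherwise given a state change.
; The box destroys itself on any fighter or BP_Bloc overlap.
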(event EventBeginPlay
  (bind _datatable (Variables|Default|GetDataTable))
  (bind _outrownames (DataTable|GetDataTableRowNames _datatable))
  (bind _returnvalue (Utilities|GetDataTableRow _datatable (.OutItem (Utilities|Array|Random _outrownames)))
    (:then
      (Rendering|Material|SetMaterial (Variables|Default|GetPlane) 0 (.BoxTexture (Utilities|Struct|BreakStruct_Bonus _returnvalue))))))

(event Collision|EventActorBeginOverlap
  (params (OtherActor :type Actor%20Object%20Reference))
  (bind _asbp_fighter_pawn (Utilities|Casting|CastToBP_FighterPawn OtherActor)
    (:then
      (Utilities|IsValid (Variables|/Game/BP/Players/Fighter/BP_FighterPawn.BP_FighterPawn_C|GetCurrentBonus _asbp_fighter_pawn)
        (:Is%20Valid
          (Actor|DestroyActor))
        (:Is%20Not%20Valid
          (bind _returnvalue (Game|SpawnActorfromClass (.BonusTypeClass (Utilities|Struct|BreakStruct_Bonus (stale EventBeginPlay _returnvalue))) (Math|Transform|MakeTransform "0, 0, 0" "0, 0, 0" "1.000000,1.000000,1.000000") "Undefined" 0 _asbp_fighter_pawn 0))
          (Default|SetBonus _asbp_fighter_pawn _returnvalue)
          (if (Variables|Default|GetAuto)
            (Default|UseBonus _asbp_fighter_pawn)
            (else
              (Default|ChangeState _returnvalue "NewEnumerator0")))
          (Actor|DestroyActor))))
    (:CastFailed
      (Utilities|Casting|CastToBP_Bloc OtherActor)
      (Actor|DestroyActor))))

(fn ConstructionScript)