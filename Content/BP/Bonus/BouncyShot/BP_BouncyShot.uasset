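; BP_BouncyShot is the Bouncy Shot bonus held by a fighter, extending a parent bonus class and adding its visual effect.
; UseBonus activates the bouncy VFX, and InitVFX colors its lines and points from a data table row, reporting missing settings.
; Tick watches Duration and, once it runs out, changes state, clears the fighter's current bonus and destroys the actor.
; PauseVFX registers the effect for the parent's pause handling.
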(event EventBeginPlay
  (|CallParentFunction))

(event EventTick
  (params (DeltaSeconds :type Float%20%28single-precision%29))
  (|CallParentFunction DeltaSeconds)
  (if (<= (Variables|Default|GetDuration) 0.0)
    (CallFunction|ChangeState "NewEnumerator2")
    (Variables|/Game/BP/Players/Fighter/BP_FighterPawn.BP_FighterPawn_C|SetCurrentBonus (Variables|Default|GetFighterUser) 0)
    (Actor|DestroyActor)))

(fn ConstructionScript
  (|CallParentFunction))

(fn UseBonus
  (|CallParentFunction)
  (Components|Activation|Activate (Variables|Default|GetVFX_Bouncy) true))

(fn InitVFX
  (bind _vfx_bouncy (Variables|Default|GetVFX_Bouncy))
  (bind _returnvalue (CallFunction|GetVFXSettingsRowName))
  (bind _vfxsettings (Variables|Default|GetVFXSettings)
    (:then
      (bind _returnvalue_2 (Utilities|GetDataTableRow _vfxsettings _returnvalue)
        (:then
          (Effects|Components|ParticleSystem|SetColorParameter _vfx_bouncy "ColorLines" (.ColorLines (Utilities|Struct|BreakS_BouncyShotSkin _returnvalue_2)))
          (Effects|Components|ParticleSystem|SetColorParameter _vfx_bouncy "ColorPoints" (.ColorPoints (Utilities|Struct|BreakS_BouncyShotSkin _returnvalue_2))))
        (:RowNotFound
          (CallFunction|CallVFXSettingsException "NOTFOUND"))))
    (:else
      (CallFunction|CallVFXSettingsException "NULL"))))

(fn PauseVFX
  (params (Enable :type Boolean))
  (Variables|Default|SetVFXs (Utilities|Array|MakeArray (Variables|Default|GetVFX_Bouncy)))
  (|CallParentFunction Enable))