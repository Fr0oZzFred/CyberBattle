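; Ghost Shot bonus for a fighter, implemented as a timed bonus on top of a parent bonus class.
; UseBonus runs the parent logic and enables Tick, which counts Duration down by delta time.
; On expiry it changes state, clears the user fighter's CurrentBonus and destroys itself.
; The ghost shot effect itself is not implemented in these graphs.
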(event EventBeginPlay
  (|CallParentFunction) ; This node is disabled and will not be called.\nDrag off pins to build functionality.
)

(event EventTick
  (params (DeltaSeconds :type Float%20%28single-precision%29))
  (Variables|Default|SetDuration (- (Variables|Default|GetDuration) DeltaSeconds))
  (if (<= (Variables|Default|GetDuration) 0.0)
    (CallFunction|ChangeState "NewEnumerator2")
    (Variables|/Game/BP/Players/Fighter/BP_FighterPawn.BP_FighterPawn_C|SetCurrentBonus (Variables|Default|GetFighterUser) 0)
    (Actor|DestroyActor)))

(fn ConstructionScript
  (|CallParentFunction))

(fn UseBonus
  (|CallParentFunction)
  (Actor|Tick|SetActorTickEnabled true))