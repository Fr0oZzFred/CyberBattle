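; BP_MadControl is a fighter bonus that sets a spin timer on its user and drastically shortens their reload cooldown while that timer runs.
; UseBonus saves the base cooldown and loads Duration into the fighter's TimerSpin, which this Blueprint only reads afterward.
; Tick re-randomizes the tiny cooldown every frame until the timer expires, then restores it, changes state, clears CurrentBonus and destroys the actor.
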(event EventBeginPlay
  (|CallParentFunction) ; This node is disabled and will not be called.\nDrag off pins to build functionality.
)

(event EventTick
  (params (DeltaSeconds :type Float%20%28single-precision%29))
  (bind _fighteruser (Variables|Default|GetFighterUser))
  (if (<= (Variables|/Game/BP/Players/Fighter/BP_FighterPawn.BP_FighterPawn_C|GetTimerSpin _fighteruser) 0.0)
    (Variables|/Game/BP/Players/Fighter/BP_FighterPawn.BP_FighterPawn_C|SetReloadCooldownTime _fighteruser (Variables|Default|GetBaseReload))
    (CallFunction|ChangeState "NewEnumerator2")
    (Variables|/Game/BP/Players/Fighter/BP_FighterPawn.BP_FighterPawn_C|SetCurrentBonus _fighteruser 0)
    (Actor|DestroyActor)
    (else
      (Variables|/Game/BP/Players/Fighter/BP_FighterPawn.BP_FighterPawn_C|SetReloadCooldownTime _fighteruser (Math|Random|RandomFloatinRange 0.02 0.04)))))

(fn ConstructionScript
  (|CallParentFunction))

(fn UseBonus
  (bind _fighteruser (Variables|Default|GetFighterUser))
  (|CallParentFunction)
  (Variables|Default|SetBaseReload (Variables|/Game/BP/Players/Fighter/BP_FighterPawn.BP_FighterPawn_C|GetReloadCooldownTime _fighteruser))
  (Variables|/Game/BP/Players/Fighter/BP_FighterPawn.BP_FighterPawn_C|SetTimerSpin _fighteruser (Variables|Default|GetDuration)))