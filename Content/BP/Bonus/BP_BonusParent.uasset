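; BP_BonusParent is the base Blueprint for bonuses, holding shared data and state logic.
; Its construction script looks up a data table row by its Name, caches the row and its Duration, and prints a message if none is found.
; UseBonus requests a state switch through ChangeState, which fires the OnBonusStateChange dispatcher only when the state actually changes.
; BeginPlay is empty, and no duration countdown or effect is implemented here.
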(event EventBeginPlay)

(fn ConstructionScript
  (bind _returnvalue (Utilities|GetDataTableRow (Variables|Default|GetBonusDataArray) (Variables|Default|GetName))
    (:then
      (bind _output_get (Variables|Default|SetBonusData _returnvalue))
      (Variables|Default|SetDuration (.Duration (Utilities|Struct|BreakStruct_Bonus _output_get))))
    (:RowNotFound
      (Development|PrintString "Bonus not found in DT Table" true true "(R=1.000000,G=0.000000,B=0.000000,A=1.000000)" 1e+01))))

(fn UseBonus
  (CallFunction|ChangeState "NewEnumerator1"))

(fn ChangeState
  (params (state :type Enum_BonusState%20Enum :default "NewEnumerator0"))
  (if (Utilities|Enum|NotEqual(Enum) (stale _output_get) state)
    (bind _output_get (Variables|Default|SetBonusState state))
    (Default|CallOnBonusStateChange _output_get)))