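; Base Blueprint for skills, handling data setup, cooldown timing and a skill state machine.
; The construction script fills icon, description, cooldown and duration from the SkillData row matching Name.
; UseSkill resets the use timer, starts the cooldown and enters Use; Tick counts down and returns Reload to Usable.
; ChangeState broadcasts OnSkillStateChange on actual changes; nothing here enters Reload or applies the duration.
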(event EventBeginPlay)

(event EventTick
  (params (DeltaSeconds :type Float%20%28single-precision%29))
  (if (> (Variables|Default|GetSkillCooldownTimer) 0.0)
    (Variables|Default|SetSkillCooldownTimer (- (Variables|Default|GetSkillCooldownTimer) DeltaSeconds))
    (else
      (switch Utilities|FlowControl|Switch|SwitchonEnum_SkillState (Variables|Default|GetSkillState)
        (:NewEnumerator2
          (CallFunction|ChangeState "NewEnumerator0")
          (Variables|Default|SetSkillCooldownTimer 0.0))))))

(fn ConstructionScript
  (bind _returnvalue (Utilities|GetDataTableRow (Variables|Default|GetSkillData) (Variables|Default|GetName))
    (:then
      (bind _output_get (Variables|Default|SetDataArray _returnvalue))
      (Variables|Default|SetIcon (.Icon (Utilities|Struct|BreakStruct_Skill _output_get)))
      (Variables|Default|SetDescription (.Description (Utilities|Struct|BreakStruct_Skill _output_get)))
      (Variables|Default|SetSkillCooldown (.Cooldown (Utilities|Struct|BreakStruct_Skill _output_get)))
      (Variables|Default|SetSkillDuration (.Duration (Utilities|Struct|BreakStruct_Skill _output_get))))
    (:RowNotFound
      (Development|PrintString "Skill Name not found in data table" true true "(R=1.000000,G=0.000000,B=0.006452,A=1.000000)" 3e+01))))

(fn UseSkill
  (Variables|Default|SetSkillUseTimer 0.0)
  (Variables|Default|SetSkillCooldownTimer (Variables|Default|GetSkillCooldown))
  (CallFunction|ChangeState "NewEnumerator1"))

(fn ChangeState
  (params (NewState :type Enum_SkillState%20Enum :default "NewEnumerator0"))
  (if (Utilities|Enum|NotEqual(Enum) (stale _output_get) NewState)
    (bind _output_get (Variables|Default|SetSkillState NewState))
    (Default|CallOnSkillStateChange _output_get)))