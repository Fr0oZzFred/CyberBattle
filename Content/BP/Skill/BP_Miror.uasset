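; Mirror skill actor that deflects projectiles carrying a different player index than the fighter using it.
; UseSkill resets a timer and teleports the mirror to the fighter, then Tick follows the fighter's location and rotation until the duration ends.
; On expiry it parks off at a fixed location and updates that fighter's skill slot state.
; On overlap, yaw math reflects the projectile's direction and restarts it from the mirror's position.
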(event EventBeginPlay
  (Transformation|SetActorTransform (Math|Transform|MakeTransform "0.000000,0.000000,1000.000000" "0, 0, 0" "1.000000,1.000000,1.000000") false true))

(event EventTick
  (params (DeltaSeconds :type Float%20%28single-precision%29))
  (bind _fighteruser (Variables|Default|GetFighterUser))
  (bind _fighteruser_2 (Variables|Default|GetFighterUser))
  (bind _returnvalue (Transformation|GetActorTransform _fighteruser_2))
  (if (< (Variables|Default|GetSkillTimer) (Variables|Default|GetSkillDuration))
    (Variables|Default|SetSkillTimer (+ (Variables|Default|GetSkillTimer) DeltaSeconds))
    (Transformation|SetActorTransform (Math|Transform|MakeTransform (.location _returnvalue) (.rotation _returnvalue) "1.000000,1.000000,1.000000"))
    (elif (not (== (Variables|Default|GetSkillTimer) (Variables|Default|GetSkillDuration)))
      (Variables|Default|SetSkillTimer (Variables|Default|GetSkillDuration))
      (Transformation|SetActorTransform (Math|Transform|MakeTransform "-2000.000000,-2000.000000,0.000000" "0, 0, 0" "1.000000,1.000000,1.000000") false true)
      (if (== self (Variables|/Game/BP/Fighter/BP_FighterPawn.BP_FighterPawn_C|GetSkill1Object _fighteruser))
        (Default|SetSkill1State (Variables|Default|GetFighterUser) "NewEnumerator2")
        (else
          (Default|SetSkill2State _fighteruser "NewEnumerator2"))))))

(event Collision|EventActorBeginOverlap
  (params (OtherActor :type Actor%20Object%20Reference))
  (bind _returnvalue (Transformation|GetActorRotation))
  ;[1 1 1] Check if apply miror
  (bind _asbp_projectile_pawn (Utilities|Casting|CastToBP_ProjectilePawn OtherActor))
  (if (!= (Variables|/Game/BP/Fighter/BP_ProjectilePawn.BP_ProjectilePawn_C|GetIndex _asbp_projectile_pawn) (Variables|/Game/BP/Fighter/BP_FighterPawn.BP_FighterPawn_C|GetIndex (Variables|Default|GetFighterUser)))
    ;[1 1 1] Set rotation without negative
    (if (< (.yaw _returnvalue) 0.0)
      (Variables|Default|SetUseRotation (+ (.yaw _returnvalue) 3.6e+02))
      (else
        (Variables|Default|SetUseRotation (.yaw _returnvalue))))
    (if (< (.yaw (Transformation|GetActorRotation _asbp_projectile_pawn)) 0.0)
      (Variables|Default|SetUseProjRotation (+ (.yaw (Transformation|GetActorRotation _asbp_projectile_pawn)) 3.6e+02))
      (else
        (Variables|Default|SetUseProjRotation (.yaw (Transformation|GetActorRotation _asbp_projectile_pawn)))))
    ;[1 1 1] Set to the same plan
    (bind _output_get (Variables|Default|SetUseProjRotation (+ (Variables|Default|GetUseRotation) (Variables|Default|GetUseProjRotation))))
    ;[1 1 1] correct proj value if over 360
    (if (> _output_get 3.6e+02)
      (Variables|Default|SetUseProjRotation (- _output_get 3.6e+02)))
    ;[1 1 1] Set Back value with negative
    (if (> (Variables|Default|GetUseProjRotation) 1.8e+02)
      (bind _output_get_2 (Variables|Default|SetUseProjRotation (- (Variables|Default|GetUseProjRotation) 3.6e+02))))
    ;[1 1 1] Apply deflected Angle
    (bind _output_get_3 (Variables|Default|SetUseProjRotation (* _output_get_2 -1.0)))
    ;[1 1 1] Set New Rotation and Apply Change To Projectile
    (Variables|Default|SetNewProjRotation (Math|Rotator|MakeRotator 0.0 0.0 (- _output_get_3 (+ (Variables|Default|GetUseRotation) 1.8e+02))))
    (Variables|/Game/BP/Fighter/BP_ProjectilePawn.BP_ProjectilePawn_C|SetStartLocation _asbp_projectile_pawn (Transformation|GetActorLocation))
    (Variables|/Game/BP/Fighter/BP_ProjectilePawn.BP_ProjectilePawn_C|SetDirection _asbp_projectile_pawn (Math|Vector|GetForwardVector (Variables|Default|GetNewProjRotation)))))

(fn ConstructionScript
  (|CallParentFunction))

(fn UseSkill
  (bind _returnvalue (Transformation|GetActorTransform))
  (|CallParentFunction)
  (Variables|Default|SetSkillTimer 0.0)
  (Transformation|SetActorTransform (Math|Transform|MakeTransform (.location (Transformation|GetActorTransform (Variables|Default|GetFighterUser))) (.rotation _returnvalue) (.scale _returnvalue)) false true))