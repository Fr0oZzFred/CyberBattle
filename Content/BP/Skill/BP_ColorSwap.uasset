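; BP_ColorSwap is a fighter skill that triggers a block color swap on the battle grid.
; UseSkill runs the parent logic, reaches the grid through the BattleManager on BP_GI, calls BlocColorSwap and then changes the skill state.
; An older branch that set the state per FighterUser skill slot remains unconnected, and Tick only calls the parent.
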(event EventBeginPlay)

(event Collision|EventActorBeginOverlap
  (params (OtherActor :type Actor%20Object%20Reference)))

(event EventTick
  (params (DeltaSeconds :type Float%20%28single-precision%29))
  (|CallParentFunction DeltaSeconds))

(fn ConstructionScript
  (|CallParentFunction))

(fn UseSkill
  (|CallParentFunction)
  (bind _asbp_gi (Utilities|Casting|CastToBP_GI (Game|GetGameInstance)))
  (Default|BlocColorSwap (Variables|/Game/BP/BP_BattleManager.BP_BattleManager_C|GetGrid (Variables|/Game/BP/BP_GI.BP_GI_C|GetBattleManager _asbp_gi)))
  (CallFunction|ChangeState "NewEnumerator2"))