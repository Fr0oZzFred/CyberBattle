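; BP_Mirror is a fighter skill actor that acts as a mirror attached to its user.
; UseSkill teleports it to FighterUser, then Tick matches the user's location and rotation until SkillDuration expires.
; On expiry it teleports to an off position and changes state.
; The yaw-based deflection of other fighters' projectiles is disconnected, as the overlap event is empty, and leftover timer and debug nodes never run.
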(event EventBeginPlay
  (Transformation|SetActorTransform (Math|Transform|MakeTransform "0.000000,0.000000,1000.000000" "0, 0, 0" "1.000000,1.000000,1.000000") false true))

(event EventTick
  (params (DeltaSeconds :type Float%20%28single-precision%29))
  (bind _fighteruser (Variables|Default|GetFighterUser))
  (bind _returnvalue (Transformation|GetActorTransform _fighteruser))
  (|CallParentFunction DeltaSeconds)
  (if (< (Variables|Default|GetSkillUseTimer) (Variables|Default|GetSkillDuration))
    (Variables|Default|SetSkillUseTimer (+ (Variables|Default|GetSkillUseTimer) DeltaSeconds))
    (Transformation|SetActorTransform (Math|Transform|MakeTransform (.location _returnvalue) (.rotation _returnvalue) "1.000000,1.000000,1.000000"))
    (elif (not (== (Variables|Default|GetSkillUseTimer) (Variables|Default|GetSkillDuration)))
      (Variables|Default|SetSkillUseTimer (Variables|Default|GetSkillDuration))
      (Transformation|SetActorTransform (Math|Transform|MakeTransform "-2000.000000,-2000.000000,0.000000" "0, 0, 0" "1.000000,1.000000,1.000000") false true)
      (CallFunction|ChangeState "NewEnumerator2"))))

(event Collision|EventActorBeginOverlap
  (params (OtherActor :type Actor%20Object%20Reference)))

(fn ConstructionScript
  (|CallParentFunction))

(fn UseSkill
  (bind _returnvalue (Transformation|GetActorTransform))
  (|CallParentFunction)
  (Transformation|SetActorTransform (Math|Transform|MakeTransform (.location (Transformation|GetActorTransform (Variables|Default|GetFighterUser))) (.rotation _returnvalue) (.scale _returnvalue)) false true))