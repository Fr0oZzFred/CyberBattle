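; BP_Invincibility is a fighter skill that makes its user invulnerable for the skill's duration.
; UseSkill runs the parent logic, passes the duration to the fighter's invulnerability time and resets the timer.
; Tick advances the timer, clamps it on expiry and sets a new state on skill slot 1 or 2, depending on whether it is the user's Skill1Object.
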(event EventTick
  (params (DeltaSeconds :type Float%20%28single-precision%29))
  (bind _fighteruser (Variables|Default|GetFighterUser))
  (if (< (Variables|Default|GetSkillTimer) (Variables|Default|GetSkillDuration))
    (Variables|Default|SetSkillTimer (+ (Variables|Default|GetSkillTimer) DeltaSeconds))
    (elif (not (== (Variables|Default|GetSkillTimer) (Variables|Default|GetSkillDuration)))
      (Variables|Default|SetSkillTimer (Variables|Default|GetSkillDuration))
      (if (== self (Variables|/Game/BP/Fighter/BP_FighterPawn.BP_FighterPawn_C|GetSkill1Object _fighteruser))
        (Default|SetSkill1State (Variables|Default|GetFighterUser) "NewEnumerator2")
        (else
          (Default|SetSkill2State _fighteruser "NewEnumerator2"))))))

(fn ConstructionScript
  (|CallParentFunction))

(fn UseSkill
  (|CallParentFunction)
  (Default|SetInvulnerabilityTime (Variables|Default|GetFighterUser) (Variables|Default|GetSkillDuration))
  (Variables|Default|SetSkillTimer 0.0))