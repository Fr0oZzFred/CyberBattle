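; Fighter skill actor for an expanding Ionique Wave that sends a destruct message to other fighter pawns it overlaps.
; UseSkill resets the timer, and Tick then keeps the wave on its user while lerping its X/Y scale up over the skill duration.
; Instead of spawning or destroying, the actor parks at a far-off location on BeginPlay and once the timer expires.
; A RestoreShield call on the user is present but never runs.
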(event EventBeginPlay
  (|CallParentFunction)
  (Transformation|SetActorTransform (Math|Transform|MakeTransform "-2000.000000,-2000.000000,0.000000" "0, 0, 0" "1.000000,1.000000,1.000000")))

(event EventTick
  (params (DeltaSeconds :type Float%20%28single-precision%29))
  (bind _skillduration (Variables|Default|GetSkillDuration))
  (|CallParentFunction DeltaSeconds)
  (if (< (Variables|Default|GetSkillTimer) (Variables|Default|GetSkillDuration))
    (bind _output_get (Variables|Default|SetSkillTimer (+ (Variables|Default|GetSkillTimer) DeltaSeconds)))
    (Transformation|SetActorTransform (Math|Transform|MakeTransform (.location (Transformation|GetActorTransform (Variables|Default|GetFighterUser))) "0, 0, 0" (Math|Vector|MakeVector (Math|Float|Lerp 1.0 4.0 (/ _output_get _skillduration)) (Math|Float|Lerp 1.0 4.0 (/ _output_get _skillduration)) 1.0)))
    (else
      (Variables|Default|SetSkillTimer _skillduration)
      (Transformation|SetActorTransform (Math|Transform|MakeTransform "-2000.000000,-2000.000000,0.000000" "0, 0, 0" "1.000000,1.000000,1.000000")))))

(event Collision|EventActorBeginOverlap
  (params (OtherActor :type Actor%20Object%20Reference))
  (bind _asbp_fighter_pawn (Utilities|Casting|CastToBP_FighterPawn OtherActor))
  (if (!= _asbp_fighter_pawn (Variables|Default|GetFighterUser))
    (Class|BPIFighter|Destruct(Message) OtherActor true)))

(fn ConstructionScript
  (|CallParentFunction))

(fn UseSkill
  (|CallParentFunction)
  (Variables|Default|SetSkillTimer 0.0))