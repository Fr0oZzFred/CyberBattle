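; BP_Bump is a fighter skill that knocks the opposing fighter away from the user.
; UseSkill runs the parent logic, then picks P1 or P2 from the game instance's BattleManager as the enemy, based on the user's Index.
; It overwrites the enemy's FloatingPawnMovement velocity with a fixed-strength push along the user-to-enemy direction, zeroing Z, then changes state.
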(event EventBeginPlay)

(event Collision|EventActorBeginOverlap
  (params (OtherActor :type Actor%20Object%20Reference)))

(event EventTick
  (params (DeltaSeconds :type Float%20%28single-precision%29))
  (|CallParentFunction DeltaSeconds) ; This node is disabled and will not be called.\nDrag off pins to build functionality.
)

(fn ConstructionScript
  (|CallParentFunction))

(fn UseSkill
  (|CallParentFunction)
  (bind _asbp_gi (Utilities|Casting|CastToBP_GI (Game|GetGameInstance)))
  (if (== (Variables|/Game/BP/Fighter/BP_FighterPawn.BP_FighterPawn_C|GetIndex (Variables|Default|GetFighterUser)) 0)
    (bind _output_get (Variables|Default|SetFighterEnemy (Variables|/Game/BP/BP_BattleManager.BP_BattleManager_C|GetP2 (Variables|/Game/BP/BP_GI.BP_GI_C|GetBattleManager _asbp_gi))))
    (Variables|/Script/Engine.MovementComponent|SetVelocity (Variables|/Game/BP/Fighter/BP_FighterPawn.BP_FighterPawn_C|GetFloatingPawnMovement _output_get) (Math|Vector|MakeVector (.x (* (Math|Vector|Normalize (Math|Vector|GetUnitDirection(Vector) (Transformation|GetActorLocation (Variables|Default|GetFighterUser)) (Transformation|GetActorLocation (Variables|Default|GetFighterEnemy)))) 5e+02)) (.y (* (Math|Vector|Normalize (Math|Vector|GetUnitDirection(Vector) (Transformation|GetActorLocation (Variables|Default|GetFighterUser)) (Transformation|GetActorLocation (Variables|Default|GetFighterEnemy)))) 5e+02)) 0.0))
    (else
      (bind _output_get_2 (Variables|Default|SetFighterEnemy (Variables|/Game/BP/BP_BattleManager.BP_BattleManager_C|GetP1 (Variables|/Game/BP/BP_GI.BP_GI_C|GetBattleManager _asbp_gi))))
      (Variables|/Script/Engine.MovementComponent|SetVelocity (Variables|/Game/BP/Fighter/BP_FighterPawn.BP_FighterPawn_C|GetFloatingPawnMovement _output_get_2) (Math|Vector|MakeVector (.x (* (Math|Vector|Normalize (Math|Vector|GetUnitDirection(Vector) (Transformation|GetActorLocation (Variables|Default|GetFighterUser)) (Transformation|GetActorLocation (Variables|Default|GetFighterEnemy)))) 5e+02)) (.y (* (Math|Vector|Normalize (Math|Vector|GetUnitDirection(Vector) (Transformation|GetActorLocation (Variables|Default|GetFighterUser)) (Transformation|GetActorLocation (Variables|Default|GetFighterEnemy)))) 5e+02)) 0.0))))
  (CallFunction|ChangeState "NewEnumerator2"))