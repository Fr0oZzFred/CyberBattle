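; Impulse wave skill actor for a two-player fight that knocks the opposing fighter away from the user.
; UseSkill teleports it from its off-arena parking spot to the user, plays shockwave VFX and sound, and picks the opponent through the GameInstance's BattleManager.
; Tick widens it in X/Y over the skill duration, then parks it and changes state.
; Overlapping the opponent adds outward planar velocity; the sphere-hit impulse logic is disconnected.
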(event OnComponentHit(Sphere1)
  (params (HitComponent :type Primitive%20Component%20Object%20Reference) (OtherActor :type Actor%20Object%20Reference) (OtherComp :type Primitive%20Component%20Object%20Reference) (NormalImpulse :type Vector :default "0, 0, 0") (Hit :type Hit%20Result%20Structure%20%28by%20ref%29)))

(event EventBeginPlay
  (Transformation|SetActorTransform (Math|Transform|MakeTransform "-2000.000000,-2000.000000,0.000000" "0, 0, 0" "1.000000,1.000000,1.000000") false true))

(event Collision|EventActorBeginOverlap
  (params (OtherActor :type Actor%20Object%20Reference))
  (bind _fighter_enemy (Variables|Default|GetFighter%20Enemy))
  (bind _floatingpawnmovement (Variables|/Game/BP/Fighter/BP_FighterPawn.BP_FighterPawn_C|GetFloatingPawnMovement _fighter_enemy))
  (if (== OtherActor _fighter_enemy)
    (Variables|/Script/Engine.MovementComponent|SetVelocity _floatingpawnmovement (Math|Vector|MakeVector (.x (+ (Variables|/Script/Engine.MovementComponent|GetVelocity _floatingpawnmovement) (* (Math|Vector|Normalize (Math|Vector|GetUnitDirection(Vector) (Transformation|GetActorLocation (Variables|Default|GetFighterUser)) (Transformation|GetActorLocation (Variables|Default|GetFighter%20Enemy)))) 1.5e+03))) (.y (+ (Variables|/Script/Engine.MovementComponent|GetVelocity _floatingpawnmovement) (* (Math|Vector|Normalize (Math|Vector|GetUnitDirection(Vector) (Transformation|GetActorLocation (Variables|Default|GetFighterUser)) (Transformation|GetActorLocation (Variables|Default|GetFighter%20Enemy)))) 1.5e+03))) 0.0))
    (Development|PrintString "Imp Wave")))

(event EventTick
  (params (DeltaSeconds :type Float%20%28single-precision%29))
  (bind _returnvalue (Transformation|GetActorTransform))
  (bind _skillduration (Variables|Default|GetSkillDuration))
  (|CallParentFunction DeltaSeconds)
  (if (< (Variables|Default|GetSkillUseTimer) (Variables|Default|GetSkillDuration))
    (bind _output_get (Variables|Default|SetSkillUseTimer (+ (Variables|Default|GetSkillUseTimer) DeltaSeconds)))
    (Transformation|SetActorTransform (Math|Transform|MakeTransform (.location _returnvalue) (.rotation _returnvalue) (Math|Vector|MakeVector (Math|Float|Lerp 1.0 4.0 (/ _output_get _skillduration)) (Math|Float|Lerp 1.0 4.0 (/ _output_get _skillduration)) 1.0)))
    (elif (not (== (Variables|Default|GetSkillUseTimer) (Variables|Default|GetSkillDuration)))
      (Variables|Default|SetSkillUseTimer _skillduration)
      (Transformation|SetActorTransform (Math|Transform|MakeTransform "-2000.000000,-2000.000000,0.000000" "0, 0, 0" "1.000000,1.000000,1.000000") false true)
      (CallFunction|ChangeState "NewEnumerator2"))))

(fn ConstructionScript
  (|CallParentFunction))

(fn UseSkill
  (bind _returnvalue (Transformation|GetActorTransform))
  (|CallParentFunction)
  (Transformation|SetActorTransform (Math|Transform|MakeTransform (.location (Transformation|GetActorTransform (Variables|Default|GetFighterUser))) (.rotation _returnvalue) (.scale _returnvalue)) false true)
  (Components|Activation|Activate (Variables|Default|GetVFX_Shockwave) true)
  (Audio|PlaySound2D "/Game/Sounds/SoundEffect/wave.wave" 1.0 1.0 0.0 0 0)
  (bind _asbp_gi (Utilities|Casting|CastToBP_GI (Game|GetGameInstance)))
  (if (== (Variables|/Game/BP/Fighter/BP_FighterPawn.BP_FighterPawn_C|GetIndex (Variables|Default|GetFighterUser)) 0)
    (Variables|Default|SetFighter%20Enemy (Variables|/Game/BP/BP_BattleManager.BP_BattleManager_C|GetP2 (Variables|/Game/BP/BP_GI.BP_GI_C|GetBattleManager _asbp_gi)))
    (else
      (Variables|Default|SetFighter%20Enemy (Variables|/Game/BP/BP_BattleManager.BP_BattleManager_C|GetP1 (Variables|/Game/BP/BP_GI.BP_GI_C|GetBattleManager _asbp_gi))))))