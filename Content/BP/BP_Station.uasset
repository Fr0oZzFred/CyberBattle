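; BP_Station is a two-player team base with life and a shield sphere, colored per player Index.
; While vulnerable, overlapping enemy BP_ProjectilePawns damage it; any overlapping projectile pawn is destroyed regardless.
; ChangeVulnerability toggles damageability and shows the shield only when invulnerable, while ReturnUINormalized supplies the life ratio.
; When life drops below zero, DestroyStation changes the game state through BP_GI.
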(event OnComponentBeginOverlap(Cube)
  (params (OverlappedComponent :type Primitive%20Component%20Object%20Reference) (OtherActor :type Actor%20Object%20Reference) (OtherComp :type Primitive%20Component%20Object%20Reference) (OtherBodyIndex :type Integer) (bFromSweep :type Boolean) (SweepResult :type Hit%20Result%20Structure%20%28by%20ref%29))
  (bind _asbp_projectile_pawn (Utilities|Casting|CastToBP_ProjectilePawn OtherActor))
  (if (Variables|Default|GetIsVulnerable)
    (if (!= (Variables|Default|GetIndex) (Variables|/Game/BP/BP_ProjectilePawn.BP_ProjectilePawn_C|GetIndex _asbp_projectile_pawn))
      (CallFunction|DamageStation (Variables|/Game/BP/BP_ProjectilePawn.BP_ProjectilePawn_C|GetDamage _asbp_projectile_pawn))
      (Actor|DestroyActor OtherActor)
      (else
        (Actor|DestroyActor OtherActor)))
    (else
      (Actor|DestroyActor OtherActor))))

(event Custom|Damage%20Station
  (params (Dmg :type Float%20%28double-precision%29))
  (bind _output_get (Variables|Default|SetLife (- (Variables|Default|GetLife) Dmg)))
  (if (< _output_get 0.0)
    (CallFunction|DestroyStation)
    ;[1 1 1] Debbug Show life of base
    (Development|PrintString (Utilities|String|Append "Hit Base : " (Utilities|String|ToString(Integer) (Variables|Default|GetIndex)) " Life : " (Utilities|String|ToString(Float) (Variables|Default|GetLife))) true true (Utilities|Select :Index (Variables|Default|GetIndex) :Option%200 "(R=0.008474,G=0.069453,B=1.000000,A=1.000000)" :Option%201 "(R=1.000000,G=0.000000,B=0.000000,A=1.000000)") 2.5)))

(event EventBeginPlay
  ;[1 1 1] Set Material
  (Rendering|Material|SetMaterial (Variables|Default|GetCube) 0 (Utilities|Select :Index (Variables|Default|GetIndex) :Option%200 "/Game/Materials/MI_P1.MI_P1" :Option%201 "/Game/Materials/MI_P2.MI_P2"))
  ;[1 1 1] Set Material
  (Rendering|Material|SetMaterial (Variables|Default|GetSphere) 0 (Utilities|Select :Index (Variables|Default|GetIndex) :Option%200 "/Game/Materials/MI_P1_Shield.MI_P1_Shield" :Option%201 "/Game/Materials/MI_P2_Shield.MI_P2_Shield"))
  (Variables|Default|SetLife (Variables|Default|GetMax%20Life)))

(fn ConstructionScript)

(fn ChangeVulnerability
  (params (New%20State :type Boolean))
  (bind _sphere (Variables|Default|GetSphere))
  (bind _output_get (Variables|Default|SetIsVulnerable New%20State))
  (if _output_get
    (Rendering|SetVisibility _sphere false false)
    (else
      (Rendering|SetVisibility _sphere true false))))

(fn ReturnUINormalized
  (return (/ (Variables|Default|GetLife) (Variables|Default|GetMax%20Life))))

(fn DestroyStation
  (bind _asbp_gi (Utilities|Casting|CastToBP_GI (Game|GetGameInstance)))
  (Default|SetGameState _asbp_gi "NewEnumerator4"))