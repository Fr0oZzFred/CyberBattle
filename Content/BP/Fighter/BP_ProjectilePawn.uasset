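; BP_ProjectilePawn is a projectile that moves along Direction every tick, destroying itself beyond MaxDistance and spawning an impact effect whenever destroyed.
; A short forward line trace detects BP_Mirror, reflecting Direction about the hit normal and resetting the travelled distance, without rotating the actor.
; Overlapping projectiles destroy each other.
; BP_GI game-state changes toggle ticking, freezing movement on pause or game over.
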(event Custom|OnGameStateChanged
  (params (New%20State :type E_GameState%20Enum :default "NewEnumerator0"))
  (switch Utilities|FlowControl|Switch|SwitchonE_GameState New%20State
    (:NewEnumerator3
      (CallFunction|SetEnable true))
    (:NewEnumerator5
      (CallFunction|SetEnable false :!label _label))
    (:NewEnumerator4
      (goto _label))))

(event Custom|OnDestroyed_Event
  (params (DestroyedActor :type Actor%20Object%20Reference))
  (Niagara|SpawnSystematLocation "/Game/VFX/VFX_ShotImpact.VFX_ShotImpact" (Transformation|GetWorldLocation (Variables|Default|GetDefaultSceneRoot)) (Math|Rotator|MakeRotfromZ (* (Variables|Default|GetDirection) -1.0))))

(event EventBeginPlay
  (Variables|Default|SetStartLocation (.location (Transformation|GetActorTransform)))
  ;[1 1 1] Set Material
  (Rendering|Material|SetMaterial (Variables|Default|GetCube) 0 (Utilities|Select :Index (Variables|Default|GetIndex) :Option%200 "/Game/Placeholder/Fred/OldRendering/MI_Projectile.MI_Projectile" :Option%201 "/Game/Placeholder/Fred/OldRendering/MI_Projectile.MI_Projectile"))
  (Utilities|FlowControl|Sequence
    (:then_0
      (EventDispatchers|BindEventtoOnDestroyed (delegate Custom|OnDestroyed_Event)))
    (:then_1
      (bind _asbp_gi (Utilities|Casting|CastToBP_GI (Game|GetGameInstance)))
      (EventDispatchers|BindEventtoOnGameStateChanged _asbp_gi (delegate Custom|OnGameStateChanged)))))

(event EventTick
  (params (DeltaSeconds :type Float%20%28single-precision%29))
  (bind _returnvalue (Transformation|GetActorTransform))
  (bind _returnvalue_2 (Transformation|GetActorTransform))
  (bind _speed (Variables|Default|Getspeed))
  ;[1 1 1] Move Forward in direction
  (if (< (Variables|Default|GetMaxDistance) (Math|Vector|Distance(Vector) (Variables|Default|GetStartLocation) (.location (Transformation|GetActorTransform))))
    (Actor|DestroyActor)
    (else
      (Transformation|SetRelativeTransform (Variables|Default|GetDefaultSceneRoot) (Math|Transform|MakeTransform (+ (* (Math|Vector|Normalize (Variables|Default|GetDirection)) (Math|Vector|MakeVector _speed _speed 0.0)) (.location _returnvalue_2)) (.rotation _returnvalue_2) (.scale _returnvalue_2)) false false)
      ;[1 1 1] Check Reflection
      (bind _outhit (Collision|LineTraceByChannel (.location _returnvalue) (+ (.location _returnvalue) (* (Math|Vector|GetForwardVector (.rotation _returnvalue)) 5e+01)) "TraceTypeQuery1" false 0 "None"))
      (Utilities|Casting|CastToBP_Mirror (.hitactor _outhit))
      ;[1 1 1] Apply Reflect
      (Variables|Default|SetDirection (- (Variables|Default|GetDirection) (* 2.0 (Math|Vector|DotProduct (Variables|Default|GetDirection) (.normal _outhit)) (.normal _outhit))))
      (Variables|Default|SetStartLocation (.location (Transformation|GetActorTransform))))))

(event Collision|EventActorBeginOverlap
  (params (OtherActor :type Actor%20Object%20Reference))
  ;[1 1 1] Cross Projectile Destruction
  (bind _asbp_projectile_pawn (Utilities|Casting|CastToBP_ProjectilePawn OtherActor))
  (Actor|DestroyActor _asbp_projectile_pawn)
  (Actor|DestroyActor))

(event EventSetEnable
  (params (Enable :type Boolean))
  (CallFunction|SetEnabled Enable))

(fn ConstructionScript)

(fn SetEnabled
  (params (Enable :type Boolean))
  (Actor|Tick|SetActorTickEnabled Enable))