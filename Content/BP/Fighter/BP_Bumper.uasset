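; BP_Bumper is a bumper actor that alters the velocity of a BP_FighterPawn when the two collide.
; On Hit, it multiplies the pawn's FloatingPawnMovement velocity by BumpForce, without using the hit normal, which is only debug-printed along with the component name.
; A TimeCancel countdown in Tick gates hits and resets to CooldownCancel after each successful bump.
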(event EventTick
  (params (DeltaSeconds :type Float%20%28single-precision%29))
  (if (not (< (Variables|Default|GetTimeCancel) 0.0))
    (Variables|Default|SetTimeCancel (- (Variables|Default|GetTimeCancel) DeltaSeconds))))

(event Collision|EventHit
  (params (MyComp :type Primitive%20Component%20Object%20Reference) (Other :type Actor%20Object%20Reference) (OtherComp :type Primitive%20Component%20Object%20Reference) (bSelfMoved :type Boolean) (HitLocation :type Vector :default "0, 0, 0") (HitNormal :type Vector :default "0, 0, 0") (NormalImpulse :type Vector :default "0, 0, 0") (Hit :type Hit%20Result%20Structure%20%28by%20ref%29))
  (if (< (Variables|Default|GetTimeCancel) 0.0)
    (Development|PrintString (Utilities|GetDisplayName OtherComp))
    (Development|PrintString (Utilities|String|Append "imp : " (Utilities|String|ToString(Vector) HitNormal)))
    (bind _asbp_fighter_pawn (Utilities|Casting|CastToBP_FighterPawn Other))
    (Variables|/Script/Engine.MovementComponent|SetVelocity (Variables|/Game/BP/Fighter/BP_FighterPawn.BP_FighterPawn_C|GetFloatingPawnMovement _asbp_fighter_pawn) (* (Variables|/Script/Engine.MovementComponent|GetVelocity (Variables|/Game/BP/Fighter/BP_FighterPawn.BP_FighterPawn_C|GetFloatingPawnMovement _asbp_fighter_pawn)) (Variables|Default|GetBumpForce)))
    (Variables|Default|SetTimeCancel (Variables|Default|GetCooldownCancel))))

(fn ConstructionScript)