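; Experimental fighter pawn, colored blue or red by player index, that moves and aims through Enhanced Input.
; BeginPlay adds the mapping context, sets the frame material and points that player's view at a shared or assigned camera.
; Input builds per-axis speeds, capped only in the positive direction, and turns stick direction into yaw.
; Tick applies both to the root transform and decays speed without delta-time scaling; attack only prints.
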(event Input|EnhancedActionEvents|EnhancedInputActionIA_Attack
  (params (ActionValue :type Boolean) (ElapsedSeconds :type Float%20%28double-precision%29) (TriggeredSeconds :type Float%20%28double-precision%29) (InputAction :type Input%20Action%20Object%20Reference :default "/Game/Inputs/IA_Attack.IA_Attack"))
  (:Triggered
    ;[1 1 1] Attack
    (Development|PrintString "Attack" :!label _label))
  (:Ongoing
    (goto _label)))

(event Input|EnhancedActionEvents|EnhancedInputActionIA_MoveForwardBackward
  (params (ActionValue :type Float%20%28double-precision%29) (ElapsedSeconds :type Float%20%28double-precision%29) (TriggeredSeconds :type Float%20%28double-precision%29) (InputAction :type Input%20Action%20Object%20Reference :default "/Game/Inputs/IA_MoveForwardBackward.IA_MoveForwardBackward"))
  (bind _maxspeed (Variables|Default|GetMaxSpeed))
  (:Triggered
    ;[1 1 1] Movement
    (bind _output_get (Variables|Default|SetSpeedX (+ (Variables|Default|GetSpeedX) (* ActionValue (Variables|Default|GetAcceleration))) :!label _label))
    (if (> _output_get _maxspeed)
      (Variables|Default|SetSpeedX _maxspeed)))
  (:Ongoing
    (goto _label)))

(event Input|EnhancedActionEvents|EnhancedInputActionIA_Move
  (params (ActionValue :type Vector%202D%20Structure) (ElapsedSeconds :type Float%20%28double-precision%29) (TriggeredSeconds :type Float%20%28double-precision%29) (InputAction :type Input%20Action%20Object%20Reference :default "/Game/Inputs/IA_Move.IA_Move")))

(event Input|EnhancedActionEvents|EnhancedInputActionIA_MoveRightLeft
  (params (ActionValue :type Float%20%28double-precision%29) (ElapsedSeconds :type Float%20%28double-precision%29) (TriggeredSeconds :type Float%20%28double-precision%29) (InputAction :type Input%20Action%20Object%20Reference :default "/Game/Inputs/IA_MoveRightLeft.IA_MoveRightLeft"))
  (bind _maxspeed (Variables|Default|GetMaxSpeed))
  (:Triggered
    ;[1 1 1] Movement
    (bind _output_get (Variables|Default|SetSpeedY (+ (Variables|Default|GetSpeedY) (* (Variables|Default|GetAcceleration) ActionValue)) :!label _label))
    (if (> _output_get _maxspeed)
      (Variables|Default|SetSpeedY _maxspeed)))
  (:Ongoing
    (goto _label)))

(event Input|EnhancedActionEvents|EnhancedInputActionIA_Orientation
  (params (ActionValue :type Vector%202D%20Structure) (ElapsedSeconds :type Float%20%28double-precision%29) (TriggeredSeconds :type Float%20%28double-precision%29) (InputAction :type Input%20Action%20Object%20Reference :default "/Game/Inputs/IA_Orientation.IA_Orientation"))
  (:Triggered
    (Variables|Default|SetStickRotation (Math|Rotator|MakeRotator 0.0 0.0 (Class|KismetMathLibrary|DegAtan2 (.y ActionValue) (.x ActionValue))) :!label _label))
  (:Ongoing
    (goto _label)))

(event EventBeginPlay
  ;[1 1 1] Link Input Format
  (bind _asplayer_controller (Utilities|Casting|CastToPlayerController (Pawn|GetController)))
  (Input|AddMappingContext (PlayerController|LocalPlayerSubsystems|GetEnhancedInputLocalPlayerSubsystem _asplayer_controller) (Variables|Default|GetinputContext) 0 "(bIgnoreAllPressedKeysUntilRelease=True,bForceImmediately=False)")
  (Rendering|Material|SetMaterial (Variables|Default|GetFrame) 0 (Utilities|Select :Index (Variables|Default|GetIndex) :Option%200 "/Game/Mat/BluePlayer.BluePlayer" :Option%201 "/Game/Mat/RedPlayer.RedPlayer"))
  ;[1 1 1] Set Camera
  (Game|Player|SetViewTargetwithBlend (Game|GetPlayerController (Variables|Default|GetIndex)) (Variables|Default|GetCam) 0.0 "VTBlend_Linear" 0.0 false))

(event EventTick
  (params (DeltaSeconds :type Float%20%28single-precision%29))
  (bind _defaultsceneroot (Variables|Default|GetDefaultSceneRoot))
  (bind _returnvalue (Transformation|GetRelativeTransform _defaultsceneroot))
  ;[1 1 1] Movement
  (bind _output_get (Variables|Default|SetMovement (Math|Vector|MakeVector (Variables|Default|GetSpeedX) (Variables|Default|GetSpeedY) 0.0)))
  (Transformation|SetRelativeTransform (Variables|Default|GetDefaultSceneRoot) (Math|Transform|MakeTransform (+ _output_get (.location _returnvalue)) (Variables|Default|GetStickRotation) (.scale _returnvalue)) false false)
  (Variables|Default|SetSpeedX (* (Variables|Default|GetSpeedX) (Variables|Default|GetSpeedDecrease)))
  (Variables|Default|SetSpeedY (* (Variables|Default|GetSpeedY) (Variables|Default|GetSpeedDecrease))))

(fn ConstructionScript)