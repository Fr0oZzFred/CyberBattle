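; Player pawn for a fighter with blue and red players, with twin-stick movement, dash, projectile shots and a runtime key remapping menu.
; Enhanced Input feeds speed and aim, which Tick applies directly to the Frame component's transform with damping, while counting down dash and reload timers.
; Overlapping another player's projectile resets Frame to the start transform.
; Skill and bonus inputs only print debug text.
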(event Custom|CreateMappingMenu
  ;[1 1 1] Create Mapping Widget and passes the Mappable Inputs
  (bind _returnvalue (UserInterface|CreateWidget "/Game/BP/Widget_MappingList.Widget_MappingList_C" 0 (Variables|Default|GetIndex)))
  (bind _output_get (Variables|Mapping|SetMappingSelectionWB _returnvalue))
  (UserInterface|Viewport|AddtoViewport _output_get 0)
  (Variables|/Script/Engine.PlayerController|SetbShowMouseCursor (Game|GetPlayerController 0) true)
  (Input|SetInputModeGameandUI (Game|GetPlayerController (Variables|Default|GetIndex)) _output_get "DoNotLock" true false)
  (Default|RefreshMappings (Variables|Mapping|GetMappingSelectionWB) (Variables|Mapping|GetMapping)))

(event Custom|RemoveCreateMappingMenu
  ;[1 1 1] Remove Widget
  (bind _mappingselectionwb (Variables|Mapping|GetMappingSelectionWB)
    (:then
      (Widget|RemovefromParent _mappingselectionwb)
      (Variables|/Script/Engine.PlayerController|SetbShowMouseCursor (Game|GetPlayerController (Variables|Default|GetIndex)) false))
    (:else)))

(event Custom|UpdateMapping
  (params (DisplayName :type Text) (NewKey :type Key%20Structure :default "None"))
  ;[1 1 1] Apply New Key
  (Class|EnhancedInputSubsystemInterface|AddPlayerMappedKey (PlayerController|LocalPlayerSubsystems|GetEnhancedInputLocalPlayerSubsystem (Game|GetPlayerController (Variables|Default|GetIndex))) (Utilities|String|StringToName (Utilities|String|ToString(Text) DisplayName)) NewKey "(bIgnoreAllPressedKeysUntilRelease=True,bForceImmediately=False)"))

(event Input|EnhancedActionEvents|EnhancedInputActionIA_Dash
  (params (ActionValue :type Boolean) (ElapsedSeconds :type Float%20%28double-precision%29) (TriggeredSeconds :type Float%20%28double-precision%29) (InputAction :type Input%20Action%20Object%20Reference :default "/Game/Inputs/IA_Dash.IA_Dash"))
  (bind _dashspeed (Variables|Dash|GetDashSpeed))
  (:Triggered
    ;[1 0.9691 0.4343] Check Dash Cooldown
    (if (<= (Variables|Dash|GetDashTimer) 0.0)
      ;[1 0.9551 0.2425] Set Dash State & Timer
      (Variables|Dash|SetIsDashing true)
      (Variables|Dash|SetDashTimer (Variables|Dash|GetDashCoolDownTime))
      (Variables|Dash|SetDashRemainingTime (Variables|Dash|GetDashDurationTime))
      ;[1 0.9371 0.4887] Set Dash Direction
      (bind _output_get (Variables|Dash|SetDashDir (Math|Vector|MakeVector (Variables|Movement|GetSpeedX) (Variables|Movement|GetSpeedY) 0.0)))
      (Variables|Dash|SetDashDir (Math|Vector|MakeVector (* (.x (Math|Vector|Normalize _output_get)) _dashspeed) (* (.y (Math|Vector|Normalize _output_get)) _dashspeed) 0.0)))))

(event Input|EnhancedActionEvents|EnhancedInputActionIA_Bonus
  (params (ActionValue :type Boolean) (ElapsedSeconds :type Float%20%28double-precision%29) (TriggeredSeconds :type Float%20%28double-precision%29) (InputAction :type Input%20Action%20Object%20Reference :default "/Game/Inputs/IA_Bonus.IA_Bonus"))
  (:Triggered
    (Development|PrintString "Bonus" true true "(R=0.104956,G=1.000000,B=0.000000,A=1.000000)" 1.0 :!label _label))
  (:Ongoing
    (goto _label)))

(event Input|EnhancedActionEvents|EnhancedInputActionIA_Attack
  (params (ActionValue :type Boolean) (ElapsedSeconds :type Float%20%28double-precision%29) (TriggeredSeconds :type Float%20%28double-precision%29) (InputAction :type Input%20Action%20Object%20Reference :default "/Game/Inputs/IA_Attack.IA_Attack"))
  (:Triggered
    ;[1 0.6128 0.3355] Check Reload Cooldown
    (if (<= (Variables|Attack|GetReloadTimer) 0.0) :!label _label
      ;[1 0.4986 0.1305] Attack
      (CallFunction|Shot)
      ;[1 0.6335 0.3727] Set Reload Cooldown
      (Variables|Attack|SetReloadTimer (Variables|Attack|GetReloadCooldownTime))))
  (:Ongoing
    (goto _label)))

(event Input|EnhancedActionEvents|EnhancedInputActionIA_Skill1
  (params (ActionValue :type Boolean) (ElapsedSeconds :type Float%20%28double-precision%29) (TriggeredSeconds :type Float%20%28double-precision%29) (InputAction :type Input%20Action%20Object%20Reference :default "/Game/Inputs/IA_Skill1.IA_Skill1"))
  (:Triggered
    (Development|PrintString "Skill 1" true true "(R=1.000000,G=0.000000,B=0.997849,A=1.000000)" 1.0 :!label _label))
  (:Ongoing
    (goto _label)))

(event Input|EnhancedActionEvents|EnhancedInputActionIA_Skill2
  (params (ActionValue :type Boolean) (ElapsedSeconds :type Float%20%28double-precision%29) (TriggeredSeconds :type Float%20%28double-precision%29) (InputAction :type Input%20Action%20Object%20Reference :default "/Game/Inputs/IA_Skill2.IA_Skill2"))
  (:Triggered
    (Development|PrintString "Skil 2" true true "(R=1.000000,G=0.000000,B=0.595663,A=1.000000)" 1.0 :!label _label))
  (:Ongoing
    (goto _label)))

(event Input|EnhancedActionEvents|EnhancedInputActionIA_MoveForwardBackward
  (params (ActionValue :type Float%20%28double-precision%29) (ElapsedSeconds :type Float%20%28double-precision%29) (TriggeredSeconds :type Float%20%28double-precision%29) (InputAction :type Input%20Action%20Object%20Reference :default "/Game/Inputs/IA_MoveForwardBackward.IA_MoveForwardBackward"))
  (bind _maxspeed (Variables|Movement|GetMaxSpeed))
  (:Triggered
    ;[0.5557 0.5846 1] Movement
    ;;[0.1717 0.1525 1] Set Speed X
    (bind _output_get (Variables|Movement|SetSpeedX (+ (Variables|Movement|GetSpeedX) (* ActionValue (Variables|Movement|GetAcceleration))) :!label _label))
    (bind (_is_superior _isinferior) (CallFunction|ForkChecker _output_get _maxspeed))
    (if _is_superior
      (Variables|Movement|SetSpeedX _maxspeed))
    (if _isinferior
      (Variables|Movement|SetSpeedX (* -1.0 _maxspeed))))
  (:Ongoing
    (goto _label)))

(event Input|EnhancedActionEvents|EnhancedInputActionIA_Move
  (params (ActionValue :type Vector%202D%20Structure) (ElapsedSeconds :type Float%20%28double-precision%29) (TriggeredSeconds :type Float%20%28double-precision%29) (InputAction :type Input%20Action%20Object%20Reference :default "/Game/Inputs/IA_Move.IA_Move")))

(event Input|EnhancedActionEvents|EnhancedInputActionIA_MoveRightLeft
  (params (ActionValue :type Float%20%28double-precision%29) (ElapsedSeconds :type Float%20%28double-precision%29) (TriggeredSeconds :type Float%20%28double-precision%29) (InputAction :type Input%20Action%20Object%20Reference :default "/Game/Inputs/IA_MoveRightLeft.IA_MoveRightLeft"))
  (bind _maxspeed (Variables|Movement|GetMaxSpeed))
  (:Triggered
    ;[0.5557 0.5846 1] Movement
    ;;[0.1717 0.1525 1] Set Speed Y
    (bind _output_get (Variables|Movement|SetSpeedY (+ (Variables|Movement|GetSpeedY) (* (Variables|Movement|GetAcceleration) ActionValue)) :!label _label))
    (bind (_is_superior _isinferior) (CallFunction|ForkChecker _output_get _maxspeed))
    (if _is_superior
      (Variables|Movement|SetSpeedY _maxspeed))
    (if _isinferior
      (Variables|Movement|SetSpeedY (* -1.0 _maxspeed))))
  (:Ongoing
    (goto _label)))

(event Input|EnhancedActionEvents|EnhancedInputActionIA_Orientation
  (params (ActionValue :type Vector%202D%20Structure) (ElapsedSeconds :type Float%20%28double-precision%29) (TriggeredSeconds :type Float%20%28double-precision%29) (InputAction :type Input%20Action%20Object%20Reference :default "/Game/Inputs/IA_Orientation.IA_Orientation"))
  (:Triggered
    ;[0.2466 0.8619 1] Get Stick Rotation
    (Variables|Movement|SetStickRotation (Math|Rotator|MakeRotator 0.0 0.0 (Class|KismetMathLibrary|DegAtan2 (.y ActionValue) (.x ActionValue))) :!label _label))
  (:Ongoing
    (goto _label)))

(event EventBeginPlay
  ;[1 1 1] Set Material
  (Rendering|Material|SetMaterial (Variables|Default|GetFrame) 0 (Utilities|Select :Index (Variables|Default|GetIndex) :Option%200 "/Game/Mat/BluePlayer.BluePlayer" :Option%201 "/Game/Mat/RedPlayer.RedPlayer"))
  ;[1 1 1] Set & Store Initialize Pos & Rot
  (bind _output_get (Variables|Respawn|SetStartPos (Transformation|GetActorTransform)))
  (Variables|Movement|SetStickRotation (.rotation _output_get))
  ;[1 1 1] Check Mappable Input
  (if (Math|Conversions|ToBoolean(Integer) (Utilities|Array|Length (Class|EnhancedInputSubsystemInterface|GetAllPlayerMappableActionKeyMappings (PlayerController|LocalPlayerSubsystems|GetEnhancedInputLocalPlayerSubsystem (Game|GetPlayerController (Variables|Default|GetIndex)))))) :!label _label
    (Variables|Mapping|SetMapping (Class|EnhancedInputSubsystemInterface|GetAllPlayerMappableActionKeyMappings (PlayerController|LocalPlayerSubsystems|GetEnhancedInputLocalPlayerSubsystem (Game|GetPlayerController (Variables|Default|GetIndex)))))
    (bind _mappingselectionwb (Variables|Mapping|GetMappingSelectionWB)
      (:then
        (Default|RefreshMappings _mappingselectionwb (Variables|Mapping|GetMapping)))
      (:else))
    (else
      (Utilities|FlowControl|DelayUntilNextTick)
      (goto _label))))

(event EventTick
  (params (DeltaSeconds :type Float%20%28single-precision%29))
  (bind _frame (Variables|Default|GetFrame))
  (bind _frame_2 (Variables|Default|GetFrame))
  (bind _returnvalue (Transformation|GetRelativeTransform _frame))
  (bind _returnvalue_2 (Transformation|GetRelativeTransform _frame_2))
  ;[1 1 1] Tmer Check
  (bind _checkedtimer (CallFunction|TimerCheck (Variables|Attack|GetReloadTimer) DeltaSeconds))
  (Variables|Attack|SetReloadTimer _checkedtimer)
  (bind _checkedtimer_2 (CallFunction|TimerCheck (Variables|Dash|GetDashTimer) DeltaSeconds))
  (Variables|Dash|SetDashTimer _checkedtimer_2)
  (bind (_checkedtimer_3 _checkresult) (CallFunction|TimerCheck (Variables|Dash|GetDashRemainingTime) DeltaSeconds))
  (Variables|Dash|SetDashRemainingTime _checkedtimer_3)
  ;[1 1 1] State Check
  (if _checkresult
    (Variables|Dash|SetIsDashing false)
    (else
      (Variables|Dash|SetIsDashing true)))
  (if (Variables|Dash|GetIsDashing)
    ;[1 1 1] Dash Movement
    (Transformation|SetRelativeTransform (Variables|Default|GetFrame) (Math|Transform|MakeTransform (+ (Variables|Dash|GetDashDir) (.location _returnvalue)) (.rotation _returnvalue) (.scale _returnvalue)) false false)
    (Development|PrintString "IsDashing" true true "(R=1.000000,G=0.848792,B=0.000000,A=1.000000)" 0.0)
    (else
      ;[1 1 1] Movement
      ;;[1 1 1] Apply Movement & Rotation
      (Variables|Movement|SetMovement (Math|Vector|MakeVector (Variables|Movement|GetSpeedX) (Variables|Movement|GetSpeedY) 0.0))
      (Transformation|SetRelativeTransform (Variables|Default|GetFrame) (Math|Transform|MakeTransform (+ (Variables|Movement|GetMovement) (.location _returnvalue_2)) (Math|Rotator|Lerp(Rotator) (Variables|Movement|GetStickRotation) (.rotation _returnvalue_2) 0.9 true) (.scale _returnvalue_2)) false false)
      ;;[1 1 1] Decrease Speed
      (Variables|Movement|SetSpeedX (* (Variables|Movement|GetSpeedX) (Variables|Movement|GetSpeedDecrease)))
      (Variables|Movement|SetSpeedY (* (Variables|Movement|GetSpeedY) (Variables|Movement|GetSpeedDecrease)))
      (Development|PrintString (Utilities|String|Append "Move : " (Utilities|String|ToString(Vector) (Variables|Movement|GetMovement))) true true "(R=0.000000,G=0.006318,B=1.000000,A=1.000000)" 0.0)
      ;[1 1 1] Timer Debug
      (Development|PrintString (Utilities|String|Append "Reload : " (Utilities|String|ToString(Float) (Variables|Attack|GetReloadTimer))) true true "(R=1.000000,G=0.423462,B=0.000000,A=1.000000)" 0.0)
      (Development|PrintString (Utilities|String|Append "Dash : " (Utilities|String|ToString(Float) (Variables|Dash|GetDashTimer))) true true "(R=1.000000,G=0.882513,B=0.000000,A=1.000000)" 0.0))))

(event Collision|EventActorBeginOverlap
  (params (OtherActor :type Actor%20Object%20Reference))
  ;[1 0.3318 0.2701] Hit Check
  (bind _asbp_projectile_pawn (Utilities|Casting|CastToBP_ProjectilePawn OtherActor))
  (if (!= (Variables|Default|GetIndex) (Variables|/Game/BP/BP_ProjectilePawn.BP_ProjectilePawn_C|GetIndex _asbp_projectile_pawn))
    (Transformation|SetRelativeTransform (Variables|Default|GetFrame) (Variables|Respawn|GetStartPos) false false)
    (Development|PrintString "Hit" true true "(R=1.000000,G=0.014146,B=0.000000,A=1.000000)" 2.5)))

(event Input|GamepadEvents|GamepadSpecialRight
  (params (Key :type Key%20Structure :default "None"))
  (:Pressed
    ;[1 1 1] Open Mapping Menu
    (Utilities|FlowControl|FlipFlop
      (:A
        (CallFunction|CreateMappingMenu))
      (:B
        (CallFunction|RemoveCreateMappingMenu)))))

(fn ConstructionScript)

(fn Shot
  (Game|SpawnActorfromClass "/Game/BP/BP_ProjectilePawn.BP_ProjectilePawn_C" (Math|Transform|MakeTransform (Transformation|GetWorldLocation (Variables|Default|GetProjSpawnPoint)) (.rotation (Transformation|GetActorTransform)) "1.000000,1.000000,1.000000") "Undefined" 0 (Variables|Default|GetIndex) (Math|Vector|GetUnitDirection(Vector) (Transformation|GetWorldLocation (Variables|Default|GetProjSpawnPoint)) (Transformation|GetWorldLocation (Variables|Default|GetProjDir))) 0))

(fn TimerCheck
  (params (ToCheckTimer :type Float%20%28single-precision%29) (DeltaSeconds :type Float%20%28double-precision%29))
  (bind _returnvalue (<= ToCheckTimer 0.0))
  (if _returnvalue
    (return ToCheckTimer _returnvalue)
    (else
      (return (- ToCheckTimer DeltaSeconds) _returnvalue))))

(fn ForkChecker
  (params (ToCheck :type Float%20%28double-precision%29) (Border :type Float%20%28double-precision%29))
  (bind _returnvalue (> ToCheck Border))
  (bind _returnvalue_2 (* Border -1.0))
  (bind _returnvalue_3 (< ToCheck _returnvalue_2))
  (if _returnvalue
    _
    (else
      _))
  (if _returnvalue_3
    _
    (else
      _))
  (return _returnvalue _returnvalue_3))