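; BP_PlayerSelection is an input relay for a player selection menu, broadcasting move, confirm and cancel actions through event dispatchers.
; On BeginPlay it waits a tick so the player index is valid, then adds MenuSelectionContext to the Enhanced Input subsystem.
; Move forwards its action value in every bound phase, while Confirm and Cancel send a phase enum.
; Cancel's end phase is bound to Canceled, whereas Confirm's uses Completed.
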(event Input|EnhancedActionEvents|EnhancedInputActionIA_Move
  (params (ActionValue :type Vector%202D%20Structure) (ElapsedSeconds :type Float%20%28double-precision%29) (TriggeredSeconds :type Float%20%28double-precision%29) (InputAction :type Input%20Action%20Object%20Reference :default "/Game/Inputs/IA_Move.IA_Move"))
  (:Triggered
    (Default|CallOnMove ActionValue :!label _label))
  (:Started
    (goto _label))
  (:Completed
    (goto _label)))

(event Input|EnhancedActionEvents|EnhancedInputActionIA_Confirm
  (params (ActionValue :type Boolean) (ElapsedSeconds :type Float%20%28double-precision%29) (TriggeredSeconds :type Float%20%28double-precision%29) (InputAction :type Input%20Action%20Object%20Reference :default "/Game/Inputs/IA_Confirm.IA_Confirm"))
  (:Triggered
    (Default|CallOnConfirm "NewEnumerator1"))
  (:Started
    (Default|CallOnConfirm "NewEnumerator0"))
  (:Completed
    (Default|CallOnConfirm "NewEnumerator2")))

(event Input|EnhancedActionEvents|EnhancedInputActionIA_Cancel
  (params (ActionValue :type Boolean) (ElapsedSeconds :type Float%20%28double-precision%29) (TriggeredSeconds :type Float%20%28double-precision%29) (InputAction :type Input%20Action%20Object%20Reference :default "/Game/Inputs/IA_Cancel.IA_Cancel"))
  (:Triggered
    (Default|CallOnCancel "NewEnumerator1"))
  (:Started
    (Default|CallOnCancel "NewEnumerator0"))
  (:Canceled
    (Default|CallOnCancel "NewEnumerator2")))

(event EventBeginPlay
  (Utilities|FlowControl|DelayUntilNextTick) ; Have to delay otherwise Index is not set correctly
  (Input|AddMappingContext (PlayerController|LocalPlayerSubsystems|GetEnhancedInputLocalPlayerSubsystem self) "/Game/Inputs/MenuSelectionContext.MenuSelectionContext" 0 "(bIgnoreAllPressedKeysUntilRelease=True,bForceImmediately=False)"))

(fn ConstructionScript)