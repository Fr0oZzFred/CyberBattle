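; BP_FighterQuentin is a player fighter with twin-stick-style controls, using Index to pick its P1 or P2 frame material.
; Enhanced Input builds X/Y speed, capped only in the positive direction, which Tick applies per frame with damping while smoothing rotation toward the stick angle.
; Attack spawns BP_ProjectilePawn, passing Index and the spawn-point-to-ProjDir direction.
; Tick prints debug location; the mapping-context setup is disconnected.
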(event Input|EnhancedActionEvents|EnhancedInputActionIA_Attack
  (params (ActionValue :type Boolean) (ElapsedSeconds :type Float%20%28double-precision%29) (TriggeredSeconds :type Float%20%28double-precision%29) (InputAction :type Input%20Action%20Object%20Reference :default "/Game/Inputs/IA_Attack.IA_Attack"))
  (:Triggered
    ;[1 1 1] Attack
    (CallFunction|Shot :!label _label))
  (:Ongoing
    (goto _label)))

(event Input|EnhancedActionEvents|EnhancedInputActionIA_MoveForwardBackward
  (params (ActionValue :type Float%20%28double-precision%29) (ElapsedSeconds :type Float%20%28double-precision%29) (TriggeredSeconds :type Float%20%28double-precision%29) (InputAction :type Input%20Action%20Object%20Reference :default "/Game/Inputs/IA_MoveForwardBackward.IA_MoveForwardBackward"))
  (bind _maxspeed (Variables|Default|GetMaxSpeed))
  (:Triggered
    ;[1 1 1] Movement
    (bind _output_get (Variables|Default|SetSpeedX (+ (Variables|Default|GetSpeedX) (* ActionValue (Variables|Default|GetAcceleration))) :!label _label))
    (if (> _output_get _maxspeed)
      (Variables|Default|SetSpeedX _maxspeed)))
  (:Ongoing
    (goto _label)))

(event Input|EnhancedActionEvents|EnhancedInputActionIA_Move
  (params (ActionValue :type Vector%202D%20Structure) (ElapsedSeconds :type Float%20%28double-precision%29) (TriggeredSeconds :type Float%20%28double-precision%29) (InputAction :type Input%20Action%20Object%20Reference :default "/Game/Inputs/IA_Move.IA_Move")))

(event Input|EnhancedActionEvents|EnhancedInputActionIA_MoveRightLeft
  (params (ActionValue :type Float%20%28double-precision%29) (ElapsedSeconds :type Float%20%28double-precision%29) (TriggeredSeconds :type Float%20%28double-precision%29) (InputAction :type Input%20Action%20Object%20Reference :default "/Game/Inputs/IA_MoveRightLeft.IA_MoveRightLeft"))
  (bind _maxspeed (Variables|Default|GetMaxSpeed))
  (:Triggered
    ;[1 1 1] Movement
    (bind _output_get (Variables|Default|SetSpeedY (+ (Variables|Default|GetSpeedY) (* (Variables|Default|GetAcceleration) ActionValue)) :!label _label))
    (if (> _output_get _maxspeed)
      (Variables|Default|SetSpeedY _maxspeed)))
  (:Ongoing
    (goto _label)))

(event Input|EnhancedActionEvents|EnhancedInputActionIA_Orientation
  (params (ActionValue :type Vector%202D%20Structure) (ElapsedSeconds :type Float%20%28double-precision%29) (TriggeredSeconds :type Float%20%28double-precision%29) (InputAction :type Input%20Action%20Object%20Reference :default "/Game/Inputs/IA_Orientation.IA_Orientation"))
  (:Triggered
    (Variables|Default|SetStickRotation (Math|Rotator|MakeRotator 0.0 0.0 (Class|KismetMathLibrary|DegAtan2 (.y ActionValue) (.x ActionValue))) :!label _label))
  (:Ongoing
    (goto _label)))

(event EventBeginPlay
  (Rendering|Material|SetMaterial (Variables|Default|GetFrame) 0 (Utilities|Select :Index (Variables|Default|GetIndex) :Option%200 "/Game/Materials/MI_P1.MI_P1" :Option%201 "/Game/Materials/MI_P2.MI_P2")))

(event EventTick
  (params (DeltaSeconds :type Float%20%28single-precision%29))
  (bind _defaultsceneroot (Variables|Default|GetDefaultSceneRoot))
  (bind _returnvalue (Transformation|GetRelativeTransform _defaultsceneroot))
  ;[1 1 1] Movement
  (bind _output_get (Variables|Default|SetMovement (Math|Vector|MakeVector (Variables|Default|GetSpeedX) (Variables|Default|GetSpeedY) 0.0)))
  (Transformation|SetRelativeTransform (Variables|Default|GetDefaultSceneRoot) (Math|Transform|MakeTransform (+ _output_get (.location _returnvalue)) (Math|Rotator|Lerp(Rotator) (Variables|Default|GetStickRotation) (.rotation _returnvalue) 0.9 true) (.scale _returnvalue)) false false)
  (Variables|Default|SetSpeedX (* (Variables|Default|GetSpeedX) (Variables|Default|GetSpeedDecrease)))
  (Variables|Default|SetSpeedY (* (Variables|Default|GetSpeedY) (Variables|Default|GetSpeedDecrease)))
  (Development|PrintString (Utilities|String|ToString(Vector) (.location _returnvalue)) true true "(R=1.000000,G=0.752513,B=0.010051,A=1.000000)" 0.0)
  (Development|PrintString "Ta Position Grid" true true "(R=0.106598,G=0.000000,B=1.000000,A=1.000000)" 0.0))

(fn ConstructionScript)

(fn Shot
  (Game|SpawnActorfromClass "/Game/BP/Fighter/BP_ProjectilePawn.BP_ProjectilePawn_C" (Math|Transform|MakeTransform (Transformation|GetWorldLocation (Variables|Default|GetProjSpawnPoint)) (.rotation (Transformation|GetActorTransform)) "1.000000,1.000000,1.000000") "Undefined" 0 (Variables|Default|GetIndex) (Math|Vector|GetUnitDirection(Vector) (Transformation|GetWorldLocation (Variables|Default|GetProjSpawnPoint)) (Transformation|GetWorldLocation (Variables|Default|GetProjDir))) 27.0 1.0 0 0))