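; Pooled player projectile pawn with normal, bouncy, ghost and super-shot types, skinned through Niagara VFX.
; Tick moves it along Direction until max range, where it is disabled or, for super shots, bursts into pooled shrapnel.
; Three forward line traces drive vector reflection off opposing mirrors and limited bounces off blocks and borders.
; Overlaps handle block damage and enemy-projectile collisions, while game-state changes pause it and Destroy hides it for reuse.
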(event Custom|OnGameStateChanged
  (params (New%20State :type E_GameState%20Enum :default "NewEnumerator0"))
  (bind _used (Variables|Default|GetUsed))
  (bind _returnvalue (not _used))
  (switch Utilities|FlowControl|Switch|SwitchonE_GameState New%20State
    (:NewEnumerator3
      (CallFunction|SetEnable _used _returnvalue))
    (:NewEnumerator5
      (CallFunction|SetEnable false _returnvalue :!label _label))
    (:NewEnumerator4
      (goto _label))))

(event EventBeginPlay
  (Utilities|InitSkin)
  (Variables|ProjectileSettings|SetStartLocation (.location (Transformation|GetActorTransform)))
  (bind _asbp_gi (Utilities|Casting|CastToBP_GI (Game|GetGameInstance)))
  (EventDispatchers|BindEventtoOnGameStateChanged _asbp_gi (delegate Custom|OnGameStateChanged)))

(event EventTick
  (params (DeltaSeconds :type Float%20%28single-precision%29))
  (bind _returnvalue (Transformation|GetActorTransform))
  (bind _maxdistance (Variables|ProjectileSettings|GetMaxDistance))
  (bind _speed (Variables|ProjectileSettings|GetSpeed))
  (bind _returnvalue_2 (* DeltaSeconds _speed))
  ;[1 1 1] Move Forward in direction
  (bind _output_get (Variables|ProjectileSettings|SetCurrentDistance (Math|Vector|Distance(Vector) (Variables|ProjectileSettings|GetStartLocation) (.location (Transformation|GetActorTransform)))))
  (Effects|Components|ParticleSystem|SetFloatParameter (Variables|Default|GetVFX_Projectile) "LifetimeOverDistance" (/ _output_get _maxdistance))
  (bind _output_get_2 (Variables|ProjectileSettings|SetOutOfRange (< _maxdistance _output_get)))
  (if _output_get_2
    (if (Utilities|Enum|Equal(Enum) (Variables|ProjectileSettings|GetProjectileType) "NewEnumerator1")
      (if (not (Variables|Default|GetExploded))
        (Variables|Default|SetExploded true)
        (CallFunction|Shrapnel))
      (else
        (CallFunction|Destroy)))
    (else
      (Transformation|SetRelativeTransform (Variables|Default|GetDefaultSceneRoot) (Math|Transform|MakeTransform (+ (* (Math|Vector|MakeVector _returnvalue_2 _returnvalue_2 0.0) (Math|Vector|Normalize (Variables|ProjectileSettings|GetDirection))) (.location _returnvalue)) (.rotation _returnvalue) (.scale _returnvalue)) false false)
      ;[1 1 1] Reflection
      (bind (_outhitnormal _out_hit_hit_actor) (Utilities|CheckReflection)
        (:Hit
          (Variables|Default|SetNormal%20Reflection _outhitnormal)
          (bind _output_get_3 (Variables|Default|SetHit%20Actor%20Reflection _out_hit_hit_actor))
          (bind _asbp_mirror (Utilities|Casting|CastToBP_Mirror _output_get_3)
            (:then
              (if (!= (Variables|/Game/BP/Players/Fighter/BP_FighterPawn.BP_FighterPawn_C|GetIndex (Variables|/Game/BP/Skills/BP_SkillParent.BP_SkillParent_C|GetFighterUser _asbp_mirror)) (Variables|ProjectileSettings|GetIndex))
                (Utilities|Reflect (Variables|Default|GetNormal%20Reflection) :!label _label)))
            (:CastFailed
              (if (Utilities|Enum|Equal(Enum) (Variables|ProjectileSettings|GetProjectileType) "NewEnumerator2") :!label _label_2
                (bind _asbp_bloc (Utilities|Casting|CastToBP_Bloc (Variables|Default|GetHit%20Actor%20Reflection))
                  (:then
                    (Default|Damage _asbp_bloc 1))
                  (:CastFailed
                    (Utilities|Casting|CastToBP_Border (Variables|Default|GetHit%20Actor%20Reflection))))
                (if (> (Variables|Bonus|GetBouncyCount) 0)
                  (Math|Integer|DecrementInt (Variables|Bonus|GetBouncyCount)
                    (:%20%20
                      (goto _label)))
                  (else
                    (CallFunction|Destroy)))))))
        (:No%20Hit
          (bind (_out_hit_normal _out_hit_hit_actor_2) (Utilities|CheckLeftReflection)
            (:Hit
              (Variables|Default|SetNormal%20Reflection _out_hit_normal)
              (Variables|Default|SetHit%20Actor%20Reflection _out_hit_hit_actor_2)
              (goto _label_2))
            (:No%20Hit
              (bind (_out_hit_normal_2 _out_hit_hit_actor_3) (Utilities|CheckRightReflection)
                (:Hit
                  (Variables|Default|SetNormal%20Reflection _out_hit_normal_2)
                  (Variables|Default|SetHit%20Actor%20Reflection _out_hit_hit_actor_3)
                  (goto _label_2))))))))))

(event EventDestroy
  (if (Variables|ProjectileSettings|GetOutOfRange)
    (Actor|Tick|SetActorTickEnabled false)
    (Collision|SetActorEnableCollision false)
    (Utilities|FlowControl|Delay 0.35)
    (else
      (Utilities|SpawnonDestroyVFX)))
  (CallFunction|SetEnable false true))

(event Collision|EventActorBeginOverlap
  (params (OtherActor :type Actor%20Object%20Reference))
  (switch Utilities|FlowControl|Switch|SwitchonE_ProjectileType (Variables|ProjectileSettings|GetProjectileType)
    (:NewEnumerator0
      _)
    (:NewEnumerator2
      _)
    (:NewEnumerator1
      _))
  (bind _asbp_projectile_pawn (Utilities|Casting|CastToBP_ProjectilePawn OtherActor)
    (:then
      (switch Utilities|FlowControl|Switch|SwitchonE_ProjectileType (Variables|ProjectileSettings|GetProjectileType)
        (:NewEnumerator0
          _)
        (:NewEnumerator2
          _))
      (if (not (== (Variables|BP_ProjectilePawn_C|GetIndex _asbp_projectile_pawn) (Variables|ProjectileSettings|GetIndex)))
        (CallFunction|Destroy)))
    (:CastFailed
      (bind _asbp_bloc (Utilities|Casting|CastToBP_Bloc OtherActor))
      (if (Utilities|Enum|Equal(Enum) (Variables|/Game/BP/Blocs/BP_Bloc.BP_Bloc_C|GetBlocState _asbp_bloc) "NewEnumerator2")
        (switch Utilities|FlowControl|Switch|SwitchonE_ProjectileType (Variables|ProjectileSettings|GetProjectileType)
          (:NewEnumerator0
            (Default|Damage _asbp_bloc 1)
            (CallFunction|Destroy))
          (:NewEnumerator1
            (Default|Annihilate _asbp_bloc false)))
        (elif (not (Utilities|Enum|Equal(Enum) (Variables|ProjectileSettings|GetProjectileType) "NewEnumerator1"))
          (CallFunction|Destroy))))))

(fn ConstructionScript)

(fn Init
  (params (Transform :type Transform) (Index :type Integer) (Direction :type Vector) (Speed :type Float%20%28double-precision%29) (DamageToStation :type Float%20%28double-precision%29) (DamageToFighter :type Float%20%28double-precision%29) (MaxDistance :type Float%20%28double-precision%29) (Skin :type S%20Projectile%20Skin%20Structure) (Type :type E_ProjectileType%20Enum :default "NewEnumerator0"))
  (Utilities|FlowControl|Sequence
    (:then_0
      (Transformation|SetActorTransform Transform)
      (Variables|ProjectileSettings|SetStartLocation (.Location (Math|Transform|BreakTransform Transform))))
    (:then_1
      (Variables|ProjectileSettings|SetIndex Index)
      (Variables|ProjectileSettings|SetDirection Direction))
    (:then_2
      (Variables|ProjectileSettings|SetSpeed Speed)
      (Variables|ProjectileSettings|SetDamageToStation DamageToStation))
    (:then_3
      (Variables|ProjectileSettings|SetDamageToFighter DamageToFighter))
    (:then_4
      (Variables|ProjectileSettings|SetMaxDistance MaxDistance)
      (Variables|Skin|SetSkin Skin))
    (:then_5
      (Variables|ProjectileSettings|SetProjectileType Type)
      (Utilities|InitSkin))
    (:then_6
      (Variables|Bonus|SetBouncyCount (Variables|Bonus|GetMaxBouncyCount)))
    (:then_7
      (return))))

(fn Shrapnel
  (bind _returnvalue (Transformation|GetActorTransform))
  (bind _returnvalue_2 (Transformation|GetActorTransform))
  (bind _returnvalue_3 (Math|Random|RandomFloatinRange -5.0 5.0))
  (bind _returnvalue_4 (Math|Random|RandomFloatinRange -5.0 5.0))
  (bind _returnvalue_5 (Math|Vector|MakeVector _returnvalue_4 _returnvalue_3 (.z (.location _returnvalue_2))))
  (bind _returnvalue_6 (Math|Vector|Normalize _returnvalue_5))
  (bind _asbp_fighter_pawn (Utilities|Casting|CastToBP_FighterPawn (Pawn|GetControlledPawn (Game|GetPlayerController (Variables|ProjectileSettings|GetIndex)))))
  (bind _asbp_gi (Utilities|Casting|CastToBP_GI (Game|GetGameInstance)))
  (for _index (range 0 (+ (Math|Random|RandomInteger 7) 16))
    (Default|SpawnProjectile (Variables|/Game/BP/BP_GI.BP_GI_C|GetPoolManager _asbp_gi) (Math|Transform|MakeTransform (.location _returnvalue) (Math|Rotator|MakeRotator 0.0 0.0 (.yaw (Math|Rotator|FindLookatRotation (.location _returnvalue) (+ (.location _returnvalue) (* _returnvalue_6 5e+02))))) "0.700000,0.700000,0.700000") (Variables|ProjectileSettings|GetIndex) (* _returnvalue_6 2e+01) 1e+04 0.5 1.0 4e+02 (.Projectile (Utilities|Struct|BreakS_PlayerSkin (Variables|/Game/BP/Players/Fighter/BP_FighterPawn.BP_FighterPawn_C|GetPlayerSkin _asbp_fighter_pawn))) "NewEnumerator0"))
  (Development|PrintString "destroyed")
  (Variables|Default|SetExploded false)
  (CallFunction|Destroy))

(fn SetEnable
  (params (Enable :type Boolean) (Hide :type Boolean))
  (bind _returnvalue (not Hide))
  (Actor|Tick|SetActorTickEnabled Enable)
  (Rendering|SetVisibility (Variables|Default|GetDefaultSceneRoot) _returnvalue true)
  (Collision|SetActorEnableCollision _returnvalue)
  (Variables|Default|SetUsed _returnvalue))