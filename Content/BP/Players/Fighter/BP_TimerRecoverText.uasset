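; Floating text actor for a fighter, apparently for timer recovery, tinted with the player skin's outline color and destroyed when its lifespan runs out.
; A Movement timeline animates an offset added to the fighter's location, so the text follows the fighter.
; Game instance state changes drive SetEnable, which toggles timeline, tick countdown and visibility: pause freezes it, while the battle intro cutscene and game over also hide it.
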(event Custom|ResumeMovement
  (bind _vector (Timeline|Movement Play)
    (:Update
      (Transformation|SetActorLocation (+ _vector (.location (Transformation|GetActorTransform (Variables|Default|GetFighterUser)))) false false))))

(event Custom|StopMovement
  (bind _vector (Timeline|Movement Stop)
    (:Update
      (Transformation|SetActorLocation (+ _vector (.location (Transformation|GetActorTransform (Variables|Default|GetFighterUser)))) false false))))

(event Custom|OnGameStateChanged
  (params (New%20State :type E_GameState%20Enum :default "NewEnumerator0"))
  (switch Utilities|FlowControl|Switch|SwitchonE_GameState New%20State
    (:NewEnumerator7
      (CallFunction|SetEnable false true :!label _label))
    (:NewEnumerator3
      (CallFunction|SetEnable true false))
    (:NewEnumerator5
      (CallFunction|SetEnable false false))
    (:NewEnumerator4
      (goto _label))))

(event EventBeginPlay
  (bind _asbp_gi (Utilities|Casting|CastToBP_GI (Game|GetGameInstance)))
  (EventDispatchers|BindEventtoOnGameStateChanged _asbp_gi (delegate Custom|OnGameStateChanged))
  (Variables|Default|SetPlayerSkin (Variables|/Game/BP/Players/Fighter/BP_FighterPawn.BP_FighterPawn_C|GetPlayerSkin (Variables|Default|GetFighterUser)))
  (Transformation|SetActorRotation "20.000000,270.000000,0.000000")
  (Variables|Default|SetLifespawnTimer (Variables|Default|GetLifespawn))
  (Rendering|Components|TextRender|SetTextRenderColor (Variables|Default|GetTextRender) (Math|Conversions|ToColor(LinearColor) (.OutlineColor (Utilities|Struct|BreakS_UI_Skin (.UI (Utilities|Struct|BreakS_NewPlayerSkin (Variables|Default|GetPlayerSkin)))))))
  (bind _vector (Timeline|Movement PlayFromStart)
    (:Update
      (Transformation|SetActorLocation (+ _vector (.location (Transformation|GetActorTransform (Variables|Default|GetFighterUser)))) false false))))

(event EventTick
  (params (DeltaSeconds :type Float%20%28single-precision%29))
  (bind _output_get (Variables|Default|SetLifespawnTimer (- (Variables|Default|GetLifespawnTimer) DeltaSeconds)))
  (if (< _output_get 0.0)
    (Actor|DestroyActor)))

(fn ConstructionScript)

(fn SetEnable
  (params (Enable :type Boolean) (Hide :type Boolean))
  (if Enable
    (CallFunction|ResumeMovement)
    (else
      (CallFunction|StopMovement)))
  (Rendering|SetVisibility (Variables|Default|GetDefaultSceneRoot) (not Hide) true)
  (Actor|Tick|SetActorTickEnabled Enable)
  (return false))