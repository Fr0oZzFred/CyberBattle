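; Player 1's fighter pawn Blueprint, mostly empty event stubs plus input-remapping hooks and an enable toggle.
; A debug Y key flip-flops between creating the mapping widget, never added to the viewport, and an empty remove event; UpdateMapping applies new keys through Enhanced Input.
; SetEnable toggles tick, movement and VFX pause, showing the frame or spawn VFX by respawn state.
; Disconnected nodes hold debug prints and unused menu display logic.
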(event Custom|CreateMappingMenu
  ;[1 1 1] Create Mapping Widget and passes the Mappable Inputs
  (bind _returnvalue (UserInterface|CreateWidget "/Game/BP/UMG_MappingList.UMG_MappingList_C" (Game|GetPlayerController 0))))

(event Custom|RemoveCreateMappingMenu)

(event Custom|UpdateMapping
  (params (DisplayName :type Text) (NewKey :type Key%20Structure :default "None"))
  ;[1 1 1] Apply New Key
  (Class|EnhancedInputSubsystemInterface|AddPlayerMappedKey (PlayerController|LocalPlayerSubsystems|GetEnhancedInputLocalPlayerSubsystem (Game|GetPlayerController 0)) (Utilities|String|StringToName (Utilities|String|ToString(Text) DisplayName)) NewKey "(bIgnoreAllPressedKeysUntilRelease=True,bForceImmediately=False)"))

(event Custom|OnGameStateChanged
  (params (New%20State :type E_GameState%20Enum :default "NewEnumerator0")))

(event Input|EnhancedActionEvents|EnhancedInputActionIA_Dash
  (params (ActionValue :type Boolean) (ElapsedSeconds :type Float%20%28double-precision%29) (TriggeredSeconds :type Float%20%28double-precision%29) (InputAction :type Input%20Action%20Object%20Reference :default "/Game/Inputs/IA_Dash.IA_Dash"))
  ;[1 1 1 1 100] Inputs
  ;;[1 1 1 1 50] Dash
)

(event Input|EnhancedActionEvents|EnhancedInputActionIA_Bonus
  (params (ActionValue :type Boolean) (ElapsedSeconds :type Float%20%28double-precision%29) (TriggeredSeconds :type Float%20%28double-precision%29) (InputAction :type Input%20Action%20Object%20Reference :default "/Game/Inputs/IA_Bonus.IA_Bonus"))
  ;[1 1 1 1 100] Inputs
  ;;[1 1 1 1 50] Skills, Bonus, Ultime
)

(event Input|EnhancedActionEvents|EnhancedInputActionIA_Attack
  (params (ActionValue :type Boolean) (ElapsedSeconds :type Float%20%28double-precision%29) (TriggeredSeconds :type Float%20%28double-precision%29) (InputAction :type Input%20Action%20Object%20Reference :default "/Game/Inputs/IA_Attack.IA_Attack"))
  ;[1 1 1 1 100] Inputs
  ;;[1 1 1 1 50] Shot
)

(event Input|EnhancedActionEvents|EnhancedInputActionIA_EndAttack
  (params (ActionValue :type Boolean) (ElapsedSeconds :type Float%20%28double-precision%29) (TriggeredSeconds :type Float%20%28double-precision%29) (InputAction :type Input%20Action%20Object%20Reference :default "/Game/Inputs/IA_EndAttack.IA_EndAttack")))

(event Input|EnhancedActionEvents|EnhancedInputActionIA_Skill1
  (params (ActionValue :type Boolean) (ElapsedSeconds :type Float%20%28double-precision%29) (TriggeredSeconds :type Float%20%28double-precision%29) (InputAction :type Input%20Action%20Object%20Reference :default "/Game/Inputs/IA_Skill1.IA_Skill1"))
  ;[1 1 1 1 100] Inputs
  ;;[1 1 1 1 50] Skills, Bonus, Ultime
)

(event Input|EnhancedActionEvents|EnhancedInputActionIA_Skill2
  (params (ActionValue :type Boolean) (ElapsedSeconds :type Float%20%28double-precision%29) (TriggeredSeconds :type Float%20%28double-precision%29) (InputAction :type Input%20Action%20Object%20Reference :default "/Game/Inputs/IA_Skill2.IA_Skill2"))
  ;[1 1 1 1 100] Inputs
  ;;[1 1 1 1 50] Skills, Bonus, Ultime
)

(event Input|EnhancedActionEvents|EnhancedInputActionIA_Ultimate
  (params (ActionValue :type Boolean) (ElapsedSeconds :type Float%20%28double-precision%29) (TriggeredSeconds :type Float%20%28double-precision%29) (InputAction :type Input%20Action%20Object%20Reference :default "/Game/Inputs/IA_Ultimate.IA_Ultimate"))
  ;[1 1 1 1 100] Inputs
  ;;[1 1 1 1 50] Skills, Bonus, Ultime
)

(event Input|EnhancedActionEvents|EnhancedInputActionIA_StartBoost
  (params (ActionValue :type Boolean) (ElapsedSeconds :type Float%20%28double-precision%29) (TriggeredSeconds :type Float%20%28double-precision%29) (InputAction :type Input%20Action%20Object%20Reference :default "/Game/Inputs/IA_StartBoost.IA_StartBoost"))
  ;[1 1 1 1 100] Inputs
  ;;[1 1 1 1 25] Boost
)

(event Input|EnhancedActionEvents|EnhancedInputActionIA_MoveForwardBackward
  (params (ActionValue :type Float%20%28double-precision%29) (ElapsedSeconds :type Float%20%28double-precision%29) (TriggeredSeconds :type Float%20%28double-precision%29) (InputAction :type Input%20Action%20Object%20Reference :default "/Game/Inputs/IA_MoveForwardBackward.IA_MoveForwardBackward"))
  ;[1 1 1 1 100] Inputs
  ;;[1 1 1 1 50] Movement
)

(event Input|EnhancedActionEvents|EnhancedInputActionIA_EndBoost
  (params (ActionValue :type Boolean) (ElapsedSeconds :type Float%20%28double-precision%29) (TriggeredSeconds :type Float%20%28double-precision%29) (InputAction :type Input%20Action%20Object%20Reference :default "/Game/Inputs/IA_EndBoost.IA_EndBoost"))
  ;[1 1 1 1 100] Inputs
  ;;[1 1 1 1 25] Boost
)

(event Input|EnhancedActionEvents|EnhancedInputActionIA_MoveRightLeft
  (params (ActionValue :type Float%20%28double-precision%29) (ElapsedSeconds :type Float%20%28double-precision%29) (TriggeredSeconds :type Float%20%28double-precision%29) (InputAction :type Input%20Action%20Object%20Reference :default "/Game/Inputs/IA_MoveRightLeft.IA_MoveRightLeft"))
  ;[1 1 1 1 100] Inputs
  ;;[1 1 1 1 50] Movement
)

(event Input|EnhancedActionEvents|EnhancedInputActionIA_Orientation
  (params (ActionValue :type Vector%202D%20Structure) (ElapsedSeconds :type Float%20%28double-precision%29) (TriggeredSeconds :type Float%20%28double-precision%29) (InputAction :type Input%20Action%20Object%20Reference :default "/Game/Inputs/IA_Orientation.IA_Orientation"))
  ;[1 1 1 1 100] Inputs
  ;;[1 1 1 1 50] Movement
)

(event EventBeginPlay)

(event EventTick
  (params (DeltaSeconds :type Float%20%28single-precision%29)))

(event Collision|EventActorBeginOverlap
  (params (OtherActor :type Actor%20Object%20Reference)))

(event Input|KeyboardEvents|DebugKeyY
  (params (Key :type Key%20Structure :default "None") (ActionValue :type Input%20Action%20Value%20Structure))
  (:Pressed
    ;[1 1 1] Open Mapping Menu
    (Utilities|FlowControl|FlipFlop
      (:A
        (CallFunction|CreateMappingMenu))
      (:B
        (CallFunction|RemoveCreateMappingMenu)))))

(event Input|GamepadEvents|GamepadSpecialRight
  (params (Key :type Key%20Structure :default "None"))
  ;[1 1 1] Handle Pause
)

(event Input|GamepadEvents|GamepadSpecialRight
  (params (Key :type Key%20Structure :default "None")))

(fn ConstructionScript)

(fn SetEnable
  (params (Enable :type Boolean) (Hide :type Boolean))
  (Actor|Tick|SetActorTickEnabled Enable)
  (Components|Tick|SetComponentTickEnabled (Variables|Default|GetFloatingPawnMovement1) Enable)
  (CallFunction|PauseVFXMacro Enable)
  (bind _return (CallFunction|IsRespawning))
  (Rendering|SetVisibility (Variables|Default|GetFrame_0) (and (not _return) (not Hide)) true)
  (Rendering|SetVisibility (Variables|Default|GetVFX_Spawn_0) (and _return (not Hide)) false)
  (Utilities|IsValid 0
    (:Is%20Valid
      (Rendering|SetActorHiddenInGame Hide))
    (:Is%20Not%20Valid
      _))
  (Utilities|IsValid 0
    (:Is%20Valid
      (Rendering|SetActorHiddenInGame Hide))
    (:Is%20Not%20Valid
      _))
  (return false))

(fn Destruct
  (params (LooseUpperHand :type Boolean)))