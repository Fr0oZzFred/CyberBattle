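; BP_Bumper is an actor that knocks a fighter pawn away when it begins to overlap it.
; One tick later, it sets the pawn's InputTimer and overwrites its FloatingPawnMovement velocity with a fixed-speed push away from the bumper's center, with Z zeroed after normalization.
; A debug "Hello" print follows, and an alternative AddMovementInput push is left unconnected.
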(event EventTick
  (params (DeltaSeconds :type Float%20%28single-precision%29)))

(event Collision|EventActorBeginOverlap
  (params (OtherActor :type Actor%20Object%20Reference))
  (bind _asbp_fighter_pawn (Utilities|Casting|CastToBP_FighterPawn OtherActor))
  (Utilities|FlowControl|DelayUntilNextTick)
  (Utilities|IsValid _asbp_fighter_pawn
    (:Is%20Valid
      (Variables|/Game/BP/Players/Fighter/BP_FighterPawn.BP_FighterPawn_C|SetInputTimer _asbp_fighter_pawn 0.5)
      (Variables|/Script/Engine.MovementComponent|SetVelocity (Variables|/Game/BP/Players/Fighter/BP_FighterPawn.BP_FighterPawn_C|GetFloatingPawnMovement _asbp_fighter_pawn) (Math|Vector|MakeVector (.x (+ "" (Math|Vector|MakeVector (.x (* (Math|Vector|Normalize (Math|Vector|GetUnitDirection(Vector) (Transformation|GetActorLocation self) (Transformation|GetActorLocation _asbp_fighter_pawn))) 1.5e+03)) (.y (* (Math|Vector|Normalize (Math|Vector|GetUnitDirection(Vector) (Transformation|GetActorLocation self) (Transformation|GetActorLocation _asbp_fighter_pawn))) 1.5e+03)) (.z (* (Math|Vector|Normalize (Math|Vector|GetUnitDirection(Vector) (Transformation|GetActorLocation self) (Transformation|GetActorLocation _asbp_fighter_pawn))) 1.5e+03))))) (.y (+ "" (Math|Vector|MakeVector (.x (* (Math|Vector|Normalize (Math|Vector|GetUnitDirection(Vector) (Transformation|GetActorLocation self) (Transformation|GetActorLocation _asbp_fighter_pawn))) 1.5e+03)) (.y (* (Math|Vector|Normalize (Math|Vector|GetUnitDirection(Vector) (Transformation|GetActorLocation self) (Transformation|GetActorLocation _asbp_fighter_pawn))) 1.5e+03)) (.z (* (Math|Vector|Normalize (Math|Vector|GetUnitDirection(Vector) (Transformation|GetActorLocation self) (Transformation|GetActorLocation _asbp_fighter_pawn))) 1.5e+03))))) 0.0))
      (Development|PrintString "Hello"))))

(fn ConstructionScript)