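; BP_FakeStation is a non-colliding visual copy of a player's station.
; On BeginPlay it polls each tick until the BattleManager's P1 or P2 (chosen by IsP1) is valid, then copies that station's life, spin speeds, shield visibility and skin.
; The skin sets part materials and shield-break VFX color, caches the damage color and blacks out the rotary part's emissive.
; Tick spins three parts, scaling rotary speed by the copied life ratio.
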(event EventBeginPlay
  (Collision|SetActorEnableCollision false)
  (bind _asbp_gi (Utilities|Casting|CastToBP_GI (Game|GetGameInstance)))
  (if (Variables|Default|GetIsP1)
    (bind _p1 (Variables|/Game/BP/BP_BattleManager.BP_BattleManager_C|GetP1 (Variables|/Game/BP/BP_GI.BP_GI_C|GetBattleManager _asbp_gi) :!label _label)
      (:then
        _)
      (:else
        (Utilities|FlowControl|DelayUntilNextTick)
        (goto _label)))
    (else
      (bind _p2 (Variables|/Game/BP/BP_BattleManager.BP_BattleManager_C|GetP2 (Variables|/Game/BP/BP_GI.BP_GI_C|GetBattleManager _asbp_gi) :!label _label_2)
        (:then
          _)
        (:else
          (Utilities|FlowControl|DelayUntilNextTick)
          (goto _label_2)))))
  (Utilities|FlowControl|DelayUntilNextTick)
  (CallFunction|Init (select (Variables|Default|GetIsP1) _p1 _p2)))

(event EventTick
  (params (DeltaSeconds :type Float%20%28single-precision%29))
  (Transformation|AddLocalRotation (Variables|Default|GetRotaryPart) (Math|Rotator|MakeRotator 0.0 0.0 (* (Math|Float|Lerp (Variables|RotatingAnimation|GetRotaryPartMaxSpeed) (Variables|RotatingAnimation|GetRotaryPartMinSpeed) (/ (Variables|Default|GetLifeStation) (Variables|Default|GetMax%20Life))) DeltaSeconds)) false false)
  (Transformation|AddLocalRotation (Variables|Default|GetEnergeticConduct) (Math|Rotator|MakeRotator 0.0 0.0 (* (Variables|RotatingAnimation|GetEnergeticCunductSpeed) DeltaSeconds)) false false)
  (Transformation|AddLocalRotation (Variables|Default|GetSideSupportDown) (Math|Rotator|MakeRotator 0.0 0.0 (* (Variables|RotatingAnimation|GetSideSupportDownSpeed) DeltaSeconds)) false false))

(fn ConstructionScript)

(fn InitSkin
  (params (StationSkin :type S%20Station%20Skin%20Structure))
  (Variables|Default|SetStationSkin StationSkin)
  (Utilities|InitSkin))

(fn Init
  (params (Player :type BP%20Fighter%20Pawn%20Object%20Reference))
  (|InitVariables Player)
  (CallFunction|InitSkin (Variables|/Game/BP/Players/Station/BP_Station.BP_Station_C|GetStationSkin (Variables|/Game/BP/Players/Fighter/BP_FighterPawn.BP_FighterPawn_C|GetStation Player)))
  (return))