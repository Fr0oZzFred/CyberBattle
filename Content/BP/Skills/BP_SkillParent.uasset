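; Base actor for fighter skills, loading cooldown, duration and range from a data table row by skill name during construction.
; UseSkill starts the cooldown and enters Use; Tick counts down and turns Reload into Usable, with state changes broadcast alongside the fighter index.
; GI game-state events toggle ticking, VFX pause and visibility.
; InitVFX is an empty stub; helpers resolve skin-settings row names and print lookup errors.
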(event Custom|OnGameStateChanged
  (params (New%20State :type E_GameState%20Enum :default "NewEnumerator0"))
  (switch Utilities|FlowControl|Switch|SwitchonE_GameState New%20State
    (:NewEnumerator7
      (CallFunction|SetEnable false true :!label _label))
    (:NewEnumerator3
      (CallFunction|SetEnable true false))
    (:NewEnumerator5
      (CallFunction|SetEnable false false))
    (:NewEnumerator4
      (goto _label))))

(event EventBeginPlay
  (CallFunction|InitVFX)
  (bind _asbp_gi (Utilities|Casting|CastToBP_GI (Game|GetGameInstance)))
  (bind _output_get (Variables|Default|SetGI _asbp_gi))
  (EventDispatchers|BindEventtoOnGameStateChanged _output_get (delegate Custom|OnGameStateChanged)))

(event EventTick
  (params (DeltaSeconds :type Float%20%28single-precision%29))
  (if (> (Variables|Default|GetSkillCooldownTimer) 0.0)
    (Variables|Default|SetSkillCooldownTimer (- (Variables|Default|GetSkillCooldownTimer) DeltaSeconds))
    (else
      (switch Utilities|FlowControl|Switch|SwitchonEnum_SkillState (Variables|Default|GetSkillState)
        (:NewEnumerator2
          (CallFunction|ChangeState "NewEnumerator0")
          (Variables|Default|SetSkillCooldownTimer 0.0))))))

(fn ConstructionScript
  (bind _returnvalue (Utilities|GetDataTableRow (Variables|Default|GetDataArray) (Variables|Default|GetName))
    (:then
      (bind _output_get (Variables|Default|SetSkillData _returnvalue))
      (bind _output_get_2 (Variables|Default|SetSkillCooldown (.Cooldown (Utilities|Struct|BreakStruct_Skill _output_get))))
      (Variables|Default|SetSkillCooldownInUse _output_get_2)
      (Variables|Default|SetSkillDuration (.Duration (Utilities|Struct|BreakStruct_Skill _output_get)))
      (Variables|Default|SetRange (.Range (Utilities|Struct|BreakStruct_Skill _output_get))))
    (:RowNotFound
      (Development|PrintString "Skill Name not found in data table" true true "(R=1.000000,G=0.000000,B=0.006452,A=1.000000)" 3e+01))))

(fn UseSkill
  (Variables|Default|SetSkillUseTimer 0.0)
  (Variables|Default|SetSkillCooldownTimer (Variables|Default|GetSkillCooldownInUse))
  (CallFunction|ChangeState "NewEnumerator1"))

(fn ChangeState
  (params (NewState :type Enum_SkillState%20Enum :default "NewEnumerator0"))
  (if (Utilities|Enum|NotEqual(Enum) (stale _output_get) NewState)
    (bind _output_get (Variables|Default|SetSkillState NewState))
    (Default|CallOnSkillStateChange _output_get (Variables|/Game/BP/Players/Fighter/BP_FighterPawn.BP_FighterPawn_C|GetIndex (Variables|Default|GetFighterUser)))))

(fn InitVFX)

(fn GetSkinSettingsRowName
  (return (select (Variables|Skin|GetSkinBaseSettings) "Base" (Utilities|String|StringToName (Utilities|String|ToString(Text) (.Name (Utilities|Struct|BreakS_NewPlayerSkin (Variables|/Game/BP/Players/Fighter/BP_FighterPawn.BP_FighterPawn_C|GetPlayerSkin (Variables|Default|GetFighterUser)))))))))

(fn CallSkinSettingsException
  (params (Error :type String))
  (switch string Error
    (:Default
      (Development|PrintString (Utilities|String|Append (Utilities|String|ToString(Name) (Variables|Default|GetName)) "Skin Settings called exception with no argument") true true "(R=1.000000,G=0.000000,B=0.000000,A=1.000000)" 2e+01))
    (:NOTFOUND
      (Development|PrintString (Utilities|String|Append (Utilities|String|ToString(Name) (Variables|Default|GetName)) " Skin Settings : Row Not Found") true true "(R=1.000000,G=0.000000,B=0.000000,A=1.000000)" 2e+01))
    (:NULL
      (Development|PrintString (Utilities|String|Append (Utilities|String|ToString(Name) (Variables|Default|GetName)) " Skin Settings is null") true true "(R=1.000000,G=0.000000,B=0.000000,A=1.000000)" 2e+01))))

(fn PauseVFX
  (params (Enable :type Boolean))
  (for _array_element (Variables|Skin|GetVFXs)
    (Class|NiagaraComponent|SetPaused _array_element (not Enable)))
  (return))

(fn SetEnable
  (params (Enable :type Boolean) (Hide :type Boolean))
  (Actor|Tick|SetActorTickEnabled Enable)
  (CallFunction|PauseVFX Enable)
  (Rendering|SetVisibility (Variables|Default|GetDefaultSceneRoot) (not Hide) true)
  (return false))