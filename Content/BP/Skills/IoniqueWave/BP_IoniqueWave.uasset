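; Fighter skill actor that, after a telegraph following its user, releases an expanding shockwave with sound and camera shake.
; Tick timers drive the phases, growing a collision sphere to Range along a curve, then shutting it off after a snapshot delay.
; Overlaps send destruct messages to other fighters, annihilate blocs and destroy projectiles.
; The wave VFX receives the timings and range, plus color and material from a skin data table.
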(event EventTick
  (params (DeltaSeconds :type Float%20%28single-precision%29))
  (bind _fighteruser (Variables|Default|GetFighterUser))
  (bind _returnvalue (Transformation|GetActorTransform _fighteruser))
  (|CallParentFunction DeltaSeconds)
  (bind _output_get (Variables|Default|SetDelayTimer (- (stale _output_get) DeltaSeconds)))
  (if (Utilities|Enum|Equal(Enum) (Variables|Default|GetSkillState) "NewEnumerator1")
    (bind _output_get_2 (Variables|Default|SetTelegraphTimer (+ (stale _output_get_2) DeltaSeconds)))
    (if (> (Variables|Default|GetTelegraphTimer) (Variables|Default|GetTelegraphDuration))
      (if (Variables|Default|GetWaveSpawned)
        _
        (else
          (Variables|Default|SetWaveSpawned true)
          (|SpawnWave)))
      (bind _output_get_3 (Variables|Default|SetSkillUseTimer (+ (stale _output_get_3) DeltaSeconds)))
      (if (>= (Variables|Default|GetSkillUseTimer) (Variables|Default|GetSkillDuration))
        (CallFunction|ChangeState "NewEnumerator2")
        (Utilities|DelaywithTimer (Variables|Default|GetSnapshotDuration))
        (Variables|Default|SetSkillUseTimer (Variables|Default|GetSkillDuration))
        (Collision|SetCollisionEnabled (Variables|Default|GetCollisionSphere) "NoCollision")
        (Components|Sphere|SetSphereRadius (Variables|Default|GetCollisionSphere) 0.0 false)
        (Variables|Default|SetWaveSpawned false)
        (else
          (Components|Sphere|SetSphereRadius (Variables|Default|GetCollisionSphere) (Math|Float|Lerp 0.0 (Variables|Default|GetRange) (Math|Curves|GetFloatValue (Variables|Default|GetRangeCurve) (/ (Variables|Default|GetSkillUseTimer) (Variables|Default|GetSkillDuration)))) true)))
      (else
        (Transformation|SetActorTransform (Math|Transform|MakeTransform (.location _returnvalue) (.rotation _returnvalue) (.scale _returnvalue)))))))

(event EventBeginPlay
  (|CallParentFunction)
  (Collision|SetCollisionEnabled (Variables|Default|GetCollisionSphere) "NoCollision"))

(event Collision|EventActorBeginOverlap
  (params (OtherActor :type Actor%20Object%20Reference))
  (Utilities|FlowControl|Sequence
    (:then_0
      (bind _asbp_fighter_pawn (Utilities|Casting|CastToBP_FighterPawn OtherActor))
      (if (!= _asbp_fighter_pawn (Variables|Default|GetFighterUser))
        (Class|BPIFighter|Destruct(Message) _asbp_fighter_pawn true)))
    (:then_1
      (bind _asbp_bloc (Utilities|Casting|CastToBP_Bloc OtherActor))
      (Default|Annihilate _asbp_bloc))
    (:then_2
      (bind _asbp_projectile_pawn (Utilities|Casting|CastToBP_ProjectilePawn OtherActor))
      (Default|Destroy _asbp_projectile_pawn))))

(fn ConstructionScript
  (|CallParentFunction))

(fn UseSkill
  (|CallParentFunction)
  (Variables|Default|SetTelegraphTimer 0.0)
  (Components|Activation|Activate (Variables|Default|GetVFX_IoniqueWave) true)
  (Components|Sphere|SetSphereRadius (Variables|Default|GetCollisionSphere) 0.0 true))

(fn InitVFX
  (Effects|Components|ParticleSystem|SetFloatParameter (Variables|Default|GetVFX_IoniqueWave) "Duration" (Variables|Default|GetSkillDuration))
  (Effects|Components|ParticleSystem|SetFloatParameter (Variables|Default|GetVFX_IoniqueWave) "TelegraphDuration" (Variables|Default|GetTelegraphDuration))
  (Effects|Components|ParticleSystem|SetFloatParameter (Variables|Default|GetVFX_IoniqueWave) "Range" (Variables|Default|GetRange))
  (Effects|Components|ParticleSystem|SetFloatParameter (Variables|Default|GetVFX_IoniqueWave) "SnapshotDuration" (Variables|Default|GetSnapshotDuration))
  (bind _returnvalue (CallFunction|GetSkinSettingsRowName))
  (bind _skinsettings (Variables|Default|GetSkinSettings)
    (:then
      (bind _returnvalue_2 (Utilities|GetDataTableRow _skinsettings _returnvalue)
        (:then
          (Effects|Components|ParticleSystem|SetColorParameter (Variables|Default|GetVFX_IoniqueWave) "Color" (.Color (Utilities|Struct|BreakS_IoniqueWaveSkin _returnvalue_2)))
          (Class|NiagaraComponent|SetVariableMaterial (Variables|Default|GetVFX_IoniqueWave) "Material" (.Material (Utilities|Struct|BreakS_IoniqueWaveSkin _returnvalue_2))))
        (:RowNotFound
          (CallFunction|CallSkinSettingsException "NOTFOUND"))))
    (:else
      (CallFunction|CallSkinSettingsException "NULL"))))

(fn PauseVFX
  (params (Enable :type Boolean))
  (Variables|Default|SetVFXs (Utilities|Array|MakeArray (Variables|Default|GetVFX_IoniqueWave)))
  (|CallParentFunction Enable))