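; BP_Mirror is a timed shield skill that follows its fighter and displays feedback when a projectile reflects off it.
; UseSkill enables collision, VFX and sound; Tick tracks the fighter until the duration expires or the fighter dies.
; A skin data table tints the VFX and dynamic material, while OnReflect drives a timeline ripple in the projectile owner's color.
; The old rebound math is disconnected, so this graph only handles reflection visuals.
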(event Custom|OnPlayerKilled
  (params (KilledPlayer :type Integer))
  (Variables|Default|SetSkillUseTimer (Variables|Default|GetSkillDuration))
  (Collision|SetCollisionEnabled (Variables|Default|GetCollision) "NoCollision")
  (CallFunction|ChangeState "NewEnumerator2"))

(event Custom|OnReflect
  (params (Projectile :type BP%20Projectile%20Pawn%20Object%20Reference))
  (bind _gi (Variables|Default|GetGI))
  (bind _battlemanager (Variables|/Game/BP/BP_GI.BP_GI_C|GetBattleManager _gi))
  (Rendering|Material|SetVectorParameterValue (Variables|Default|GetMDI_Mirror) "ProjLocation" (Math|Conversions|ToLinearColor(Vector) (Transformation|GetActorLocation Projectile)) :!class /Script/Engine.MaterialInstanceDynamic)
  (Variables|Default|SetProjColor (.Color (Utilities|Struct|BreakS_ProjectileSkin (.Projectile (Utilities|Struct|BreakS_NewPlayerSkin (Variables|/Game/BP/Players/Fighter/BP_FighterPawn.BP_FighterPawn_C|GetPlayerSkin (Utilities|Select :Index (Variables|/Game/BP/Players/Projectile/BP_ProjectilePawn.BP_ProjectilePawn_C|GetIndex Projectile) :Option%200 (Variables|/Game/BP/BP_BattleManager.BP_BattleManager_C|GetP1 _battlemanager) :Option%201 (Variables|/Game/BP/BP_BattleManager.BP_BattleManager_C|GetP2 _battlemanager))))))))
  (bind _radiusanim (Timeline|OnReflectAnim PlayFromStart)
    (:Update
      (Rendering|Material|SetScalarParameterValue (Variables|Default|GetMDI_Mirror) "Radius" (* _radiusanim 1.5e+02) :!class /Script/Engine.MaterialInstanceDynamic)
      (Rendering|Material|SetVectorParameterValue (Variables|Default|GetMDI_Mirror) "RadiusColor" (Utilities|Struct|MakeLinearColor (.r (Variables|Default|GetProjColor)) (.g (Variables|Default|GetProjColor)) (.b (Variables|Default|GetProjColor)) (- 1.0 _radiusanim)) :!class /Script/Engine.MaterialInstanceDynamic))))

(event Custom|ResumeAnim
  (bind _projcolor (Variables|Default|GetProjColor))
  (bind _radiusanim (Timeline|OnReflectAnim Play)
    (:Update
      (Rendering|Material|SetScalarParameterValue (Variables|Default|GetMDI_Mirror) "Radius" (* _radiusanim 1.5e+02) :!class /Script/Engine.MaterialInstanceDynamic)
      (Rendering|Material|SetVectorParameterValue (Variables|Default|GetMDI_Mirror) "RadiusColor" (Utilities|Struct|MakeLinearColor (.r _projcolor) (.g _projcolor) (.b _projcolor) (- 1.0 _radiusanim)) :!class /Script/Engine.MaterialInstanceDynamic))))

(event Custom|StopAnim
  (bind _projcolor (Variables|Default|GetProjColor))
  (bind _radiusanim (Timeline|OnReflectAnim Stop)
    (:Update
      (Rendering|Material|SetScalarParameterValue (Variables|Default|GetMDI_Mirror) "Radius" (* _radiusanim 1.5e+02) :!class /Script/Engine.MaterialInstanceDynamic)
      (Rendering|Material|SetVectorParameterValue (Variables|Default|GetMDI_Mirror) "RadiusColor" (Utilities|Struct|MakeLinearColor (.r _projcolor) (.g _projcolor) (.b _projcolor) (- 1.0 _radiusanim)) :!class /Script/Engine.MaterialInstanceDynamic))))

(event EventBeginPlay
  (|CallParentFunction)
  (Collision|SetCollisionEnabled (Variables|Default|GetCollision) "NoCollision")
  (EventDispatchers|AssignOnKilled (Variables|Default|GetFighterUser) (delegate Custom|OnPlayerKilled)))

(event EventTick
  (params (DeltaSeconds :type Float%20%28single-precision%29))
  (bind _fighteruser (Variables|Default|GetFighterUser))
  (bind _returnvalue (Transformation|GetActorTransform _fighteruser))
  (|CallParentFunction DeltaSeconds)
  (if (< (Variables|Default|GetSkillUseTimer) (Variables|Default|GetSkillDuration))
    (Variables|Default|SetSkillUseTimer (+ (Variables|Default|GetSkillUseTimer) DeltaSeconds))
    (Transformation|SetActorTransform (Math|Transform|MakeTransform (.location _returnvalue) (.rotation _returnvalue) "1.000000,1.000000,1.000000"))
    (elif (not (== (Variables|Default|GetSkillUseTimer) (Variables|Default|GetSkillDuration)))
      (Variables|Default|SetSkillUseTimer (Variables|Default|GetSkillDuration))
      (Audio|PlaySound2D "/Game/Sounds/SoundEffect/ShieldDown.ShieldDown" 1.0 1.0 0.0 0 0)
      (Collision|SetCollisionEnabled (Variables|Default|GetCollision) "NoCollision")
      (CallFunction|ChangeState "NewEnumerator2"))))

(event Collision|EventActorBeginOverlap
  (params (OtherActor :type Actor%20Object%20Reference)))

(fn ConstructionScript
  (|CallParentFunction))

(fn UseSkill
  (bind _returnvalue (Transformation|GetActorTransform))
  (|CallParentFunction)
  (Transformation|SetActorTransform (Math|Transform|MakeTransform (.location (Transformation|GetActorTransform (Variables|Default|GetFighterUser))) (.rotation _returnvalue) (.scale _returnvalue)) false true)
  (Components|Activation|Activate (Variables|Default|GetVFX_Mirror) true)
  (Collision|SetCollisionEnabled (Variables|Default|GetCollision) "QueryAndPhysics")
  (Audio|PlaySound2D "/Game/Sounds/SoundEffect/ShieldUp.ShieldUp" 1.0 1.0 0.0 0 0))

(fn InitVFX
  (Effects|Components|ParticleSystem|SetFloatParameter (Variables|Default|GetVFX_Mirror) "Duration" (Variables|Default|GetSkillDuration))
  (bind _returnvalue (Rendering|Material|CreateDynamicMaterialInstance (Variables|Default|GetMirrorMaterial) "None" "None" :!class /Script/Engine.KismetMaterialLibrary))
  (Variables|Default|SetMDI_Mirror _returnvalue)
  (bind _returnvalue_2 (CallFunction|GetSkinSettingsRowName))
  (bind _skinsettings (Variables|Default|GetSkinSettings)
    (:then
      (bind _returnvalue_3 (Utilities|GetDataTableRow _skinsettings _returnvalue_2)
        (:then
          (Effects|Components|ParticleSystem|SetColorParameter (Variables|Default|GetVFX_Mirror) "Color" (.Color (Utilities|Struct|BreakS_MirrorSkin _returnvalue_3)))
          (Rendering|Material|SetVectorParameterValue (Variables|Default|GetMDI_Mirror) "Color" (.ShieldColor (Utilities|Struct|BreakS_MirrorSkin _returnvalue_3)) :!class /Script/Engine.MaterialInstanceDynamic)
          (Class|NiagaraComponent|SetVariableMaterial (Variables|Default|GetVFX_Mirror) "Material" (Variables|Default|GetMDI_Mirror)))
        (:RowNotFound
          (CallFunction|CallSkinSettingsException "NOTFOUND"))))
    (:else
      (CallFunction|CallSkinSettingsException "NULL"))))

(fn SetEnable
  (params (Enable :type Boolean) (Hide :type Boolean))
  (|CallParentFunction Enable Hide)
  (if Enable
    (if (Audio|Components|Audio|IsPlaying (Variables|Default|GetOnReflectAnim))
      (CallFunction|ResumeAnim))
    (else
      (CallFunction|StopAnim)))
  (return false))