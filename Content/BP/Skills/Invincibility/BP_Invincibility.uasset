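; BP_Invincibility is a fighter skill that makes its user invulnerable for the skill duration.
; On use, it sets the user's invulnerability time, activates the shield VFX and plays a sound.
; Tick moves the actor with the user until the duration ends, then changes the skill state.
; VFX setup passes in the duration and pulls color and shield scale from a data table row, reporting missing data.
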(event EventTick
  (params (DeltaSeconds :type Float%20%28single-precision%29))
  (bind _fighteruser (Variables|Default|GetFighterUser))
  (bind _returnvalue (Transformation|GetActorTransform _fighteruser))
  (|CallParentFunction DeltaSeconds)
  (if (< (Variables|Default|GetSkillUseTimer) (Variables|Default|GetSkillDuration))
    (Variables|Default|SetSkillUseTimer (+ (Variables|Default|GetSkillUseTimer) DeltaSeconds))
    (Transformation|SetActorTransform (Math|Transform|MakeTransform (.location _returnvalue) (.rotation _returnvalue) "1.000000,1.000000,1.000000"))
    (elif (not (== (Variables|Default|GetSkillUseTimer) (Variables|Default|GetSkillDuration)))
      (Variables|Default|SetSkillUseTimer (Variables|Default|GetSkillDuration))
      (CallFunction|ChangeState "NewEnumerator2"))))

(fn ConstructionScript
  (|CallParentFunction))

(fn UseSkill
  (|CallParentFunction)
  (Default|SetInvulnerabilityTime (Variables|Default|GetFighterUser) (Variables|Default|GetSkillDuration) false)
  (Components|Activation|Activate (Variables|Default|GetVFX_Invincibility) true)
  (Audio|PlaySound2D "/Game/Sounds/SoundEffect/ShieldUp.ShieldUp" 1.0 1.0 0.0 0 0))

(fn InitVFX
  (bind _vfx_invincibility (Variables|Default|GetVFX_Invincibility))
  (Effects|Components|ParticleSystem|SetFloatParameter (Variables|Default|GetVFX_Invincibility) "Duration" (Variables|Default|GetSkillDuration))
  (bind _returnvalue (CallFunction|GetVFXSettingsRowName))
  (bind _vfxsettings (Variables|Default|GetVFXSettings)
    (:then
      (bind _returnvalue_2 (Utilities|GetDataTableRow _vfxsettings _returnvalue)
        (:then
          (Effects|Components|ParticleSystem|SetColorParameter _vfx_invincibility "Color" (.Color (Utilities|Struct|BreakS_InvincibilitySkin _returnvalue_2)))
          (Effects|Components|ParticleSystem|SetVectorParameter _vfx_invincibility "ShieldScale" (.ShieldScale (Utilities|Struct|BreakS_InvincibilitySkin _returnvalue_2))))
        (:RowNotFound
          (CallFunction|CallVFXSettingsException "NOTFOUND"))))
    (:else
      (CallFunction|CallVFXSettingsException "NULL"))))

(fn PauseVFX
  (params (Enable :type Boolean))
  (Variables|Default|SetVFXs (Utilities|Array|MakeArray (Variables|Default|GetVFX_Invincibility)))
  (|CallParentFunction Enable))