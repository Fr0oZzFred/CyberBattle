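; Skill mine that detonates when its target fighter overlaps it or its lifetime expires.
; Detonation swaps the sensor for a collision sphere that Tick grows into a shockwave, destructing the target and annihilating blocs, with skin-colored Niagara VFX, before the mine destroys itself.
; Projectiles sharing the target's index wear down its HP and can destroy it without detonation.
; Game state changes toggle its tick, collision and visibility.
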(event OnComponentBeginOverlap(CollisionSphere)
  (params (OverlappedComponent :type Primitive%20Component%20Object%20Reference) (OtherActor :type Actor%20Object%20Reference) (OtherComp :type Primitive%20Component%20Object%20Reference) (OtherBodyIndex :type Integer) (bFromSweep :type Boolean) (SweepResult :type Hit%20Result%20Structure%20%28by%20ref%29))
  (Utilities|FlowControl|Sequence
    (:then_0
      (bind _asbp_fighter_pawn (Utilities|Casting|CastToBP_FighterPawn OtherActor))
      (if (== _asbp_fighter_pawn (Variables|Default|GetTargetFighter))
        (Default|Destruct _asbp_fighter_pawn true)))
    (:then_1
      (bind _asbp_bloc (Utilities|Casting|CastToBP_Bloc OtherActor))
      (Default|Annihilate _asbp_bloc))))

(event EventBeginPlay
  (bind _asbp_gi (Utilities|Casting|CastToBP_GI (Game|GetGameInstance)))
  (EventDispatchers|BindEventtoOnGameStateChanged _asbp_gi (|OnGameState_Changed))
  (Collision|SetCollisionEnabled (Variables|Default|GetCollisionSphere) "NoCollision")
  (Components|Sphere|SetSphereRadius (Variables|Default|GetSensor) (Variables|Default|GetSensorRange) true)
  (Effects|Components|ParticleSystem|SetFloatParameter (Variables|Default|GetVFX_Mine) "Range" (Variables|Default|GetSensorRange))
  (Effects|Components|ParticleSystem|SetColorParameter (Variables|Default|GetVFX_Mine) "MineColor" (.MineColor (Utilities|Struct|BreakS_MineSkin (Variables|Default|GetMineSkin))))
  (Variables|Default|SetWaveTimer (Variables|Default|GetWaveDuration)))

(event Collision|EventActorBeginOverlap
  (params (OtherActor :type Actor%20Object%20Reference))
  (Utilities|FlowControl|Sequence
    (:then_0
      (bind _asbp_fighter_pawn (Utilities|Casting|CastToBP_FighterPawn OtherActor))
      (if (== _asbp_fighter_pawn (Variables|Default|GetTargetFighter))
        (CallFunction|Detonate)))
    (:then_1
      (bind _asbp_projectile_pawn (Utilities|Casting|CastToBP_ProjectilePawn OtherActor))
      (if (== (Variables|/Game/BP/Players/Projectile/BP_ProjectilePawn.BP_ProjectilePawn_C|GetIndex _asbp_projectile_pawn) (Variables|/Game/BP/Players/Fighter/BP_FighterPawn.BP_FighterPawn_C|GetIndex (Variables|Default|GetTargetFighter)))
        (bind _result (Math|Float|DecrementFloat (Variables|Default|GetHP))
          (:%20%20
            (if (<= _result 0.0)
              (Actor|DestroyActor))
            (Default|Destroy _asbp_projectile_pawn)))))))

(event EventTick
  (params (DeltaSeconds :type Float%20%28single-precision%29))
  (bind _waveduration (Variables|Default|GetWaveDuration))
  (|DebugCollisionSphere)
  (if (< (Variables|Default|GetLifetimeTimer) (Variables|Default|GetLifetime))
    (Variables|Default|SetLifetimeTimer (+ (Variables|Default|GetLifetimeTimer) DeltaSeconds))
    (else
      (CallFunction|Detonate)
      (Variables|Default|SetLifetimeTimer 5e+02)))
  (if (< (Variables|Default|GetWaveTimer) (Variables|Default|GetWaveDuration))
    (bind _output_get (Variables|Default|SetWaveTimer (+ (Variables|Default|GetWaveTimer) DeltaSeconds)))
    (Components|Sphere|SetSphereRadius (Variables|Default|GetCollisionSphere) (Math|Float|Lerp 0.0 (Variables|Default|GetRange) (/ _output_get _waveduration)) true)
    (elif (not (== (Variables|Default|GetWaveTimer) (Variables|Default|GetWaveDuration)))
      (Variables|Default|SetWaveTimer _waveduration)
      (Actor|DestroyActor))))

(fn ConstructionScript)

(fn Detonate
  (if (== (Variables|Default|GetWaveDuration) (Variables|Default|GetWaveTimer))
    (Variables|Default|SetWaveTimer 0.0)
    (Camera|PlayWorldCameraShake "/Game/BP/BP_CameraShake2.BP_CameraShake2_C" (Transformation|GetActorLocation) 0.0 2e+03)
    (Collision|SetCollisionEnabled (Variables|Default|GetSensor) "NoCollision")
    (Collision|SetCollisionEnabled (Variables|Default|GetCollisionSphere) "QueryAndPhysics")
    (|SpawnAndInitExplosionVFX)
    (Audio|PlaySound2D "/Game/Sounds/SoundEffect/Explosion.Explosion" 1.0 1.0 0.0 0 0)
    (Variables|Default|SetDetonated true)))

(event Custom|OnGameStateChanged
  (params (New%20State :type E_GameState%20Enum :default "NewEnumerator0"))
  (switch Utilities|FlowControl|Switch|SwitchonE_GameState New%20State
    (:NewEnumerator7
      (CallFunction|SetEnable false true :!label _label))
    (:NewEnumerator3
      (CallFunction|SetEnable true false))
    (:NewEnumerator5
      (CallFunction|SetEnable false false))
    (:NewEnumerator4
      (goto _label))))

(fn SetEnable
  (params (Enable :type Boolean) (Hide :type Boolean))
  (Actor|Tick|SetActorTickEnabled Enable)
  (Rendering|SetVisibility (Variables|Default|GetDefaultSceneRoot) (not Hide) true)
  (Collision|SetActorEnableCollision Enable)
  (return false))