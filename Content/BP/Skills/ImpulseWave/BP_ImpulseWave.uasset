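; Impulse Wave skill actor: a telegraphed radial shockwave that knocks the opposing fighter away.
; UseSkill moves it from off-map parking to the user; Tick shrinks the telegraph while following them, then expands the wave in place and parks it again.
; ApplyImpulseWave fires effects and resolves the opponent through the BattleManager.
; Scaling the actor drives the overlap, which spins the enemy, sets its input timer and overrides its velocity outward.
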(event EventBeginPlay
  (Transformation|SetActorTransform (Math|Transform|MakeTransform "-2000.000000,-2000.000000,0.000000" "0, 0, 0" "1.000000,1.000000,1.000000") false true))

(event Collision|EventActorBeginOverlap
  (params (OtherActor :type Actor%20Object%20Reference))
  (bind _returnvalue (Transformation|GetActorLocation))
  (bind _fighter_enemy (Variables|Default|GetFighter%20Enemy))
  (bind _fighter_enemy_2 (Variables|Default|GetFighter%20Enemy))
  (bind _returnvalue_2 (Transformation|GetActorLocation _fighter_enemy))
  (bind _returnvalue_3 (Math|Vector|GetUnitDirection(Vector) _returnvalue _returnvalue_2))
  (bind _returnvalue_4 (Math|Vector|Normalize _returnvalue_3))
  (bind _returnvalue_5 (* _returnvalue_4 2e+03))
  (bind _returnvalue_6 (+ "" _returnvalue_5))
  (if (== OtherActor _fighter_enemy_2)
    (Utilities|FlowControl|DelayUntilNextTick)
    (Default|SetSpinning _fighter_enemy_2 1.5 3e+01)
    (Variables|/Game/BP/Players/Fighter/BP_FighterPawn.BP_FighterPawn_C|SetInputTimer _fighter_enemy_2 1.5)
    (Variables|/Script/Engine.MovementComponent|SetVelocity (Variables|/Game/BP/Players/Fighter/BP_FighterPawn.BP_FighterPawn_C|GetFloatingPawnMovement _fighter_enemy_2) (Math|Vector|MakeVector (.x _returnvalue_6) (.y _returnvalue_6) 0.0))))

(event EventTick
  (params (DeltaSeconds :type Float%20%28single-precision%29))
  (bind _returnvalue (Transformation|GetActorTransform))
  (bind _fighteruser (Variables|Default|GetFighterUser))
  (bind _skillduration (Variables|Default|GetSkillDuration))
  (bind _returnvalue_2 (Transformation|GetActorTransform _fighteruser))
  (|CallParentFunction DeltaSeconds)
  (if (< (Variables|Default|GetTelegraphTimer) (Variables|Default|GetTelegraphDuration))
    (bind _output_get (Variables|Default|SetTelegraphTimer (+ (Variables|Default|GetTelegraphTimer) DeltaSeconds)))
    (Transformation|SetActorTransform (Math|Transform|MakeTransform (.location _returnvalue_2) (.rotation _returnvalue_2) (Math|Vector|MakeVector (* (Math|Float|Lerp -6.0 -1.0 (/ _output_get (Variables|Default|GetTelegraphDuration))) -1.0) (* (Math|Float|Lerp -6.0 -1.0 (/ _output_get (Variables|Default|GetTelegraphDuration))) -1.0) 1.0)))
    (elif (Variables|/Script/Engine.SceneComponent|GetbVisible (Variables|Default|GetPH_Telegraph))
      (Rendering|SetVisibility (Variables|Default|GetPH_Telegraph) false false)
      (|ApplyImpulseWave)
      (elif (< (Variables|Default|GetSkillUseTimer) (Variables|Default|GetSkillDuration))
        (bind _output_get_2 (Variables|Default|SetSkillUseTimer (+ (Variables|Default|GetSkillUseTimer) DeltaSeconds)))
        (Transformation|SetActorTransform (Math|Transform|MakeTransform (.location _returnvalue) (.rotation _returnvalue) (Math|Vector|MakeVector (Math|Float|Lerp 1.0 6.0 (/ _output_get_2 (- _skillduration (Variables|Default|GetLeftoverTime)))) (Math|Float|Lerp 1.0 6.0 (/ _output_get_2 (- _skillduration (Variables|Default|GetLeftoverTime)))) 1.0)))
        (elif (not (== (Variables|Default|GetSkillUseTimer) (Variables|Default|GetSkillDuration)))
          (Variables|Default|SetSkillUseTimer _skillduration)
          (Transformation|SetActorTransform (Math|Transform|MakeTransform "-2000.000000,-2000.000000,0.000000" "0, 0, 0" "1.000000,1.000000,1.000000") false true)
          (CallFunction|ChangeState "NewEnumerator2"))))))

(fn ConstructionScript
  (|CallParentFunction))

(fn UseSkill
  (bind _returnvalue (Transformation|GetActorTransform))
  (|CallParentFunction)
  (Transformation|SetActorTransform (Math|Transform|MakeTransform (.location (Transformation|GetActorTransform (Variables|Default|GetFighterUser))) (.rotation _returnvalue) (.scale _returnvalue)) false true)
  (Variables|Default|SetTelegraphTimer 0.0)
  (Rendering|SetVisibility (Variables|Default|GetPH_Telegraph) true false)
  (Development|PrintString "use impulse")
  (Components|Activation|Activate (Variables|Default|GetVFX_ImpulseWave) true))