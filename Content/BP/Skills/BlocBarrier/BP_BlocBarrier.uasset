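; Barrier skill that spawns a temporary wall of three blocs on the battle grid, in the row directly ahead of the fighter using it.
; UseSkill converts the forward and two forward-diagonal world offsets to grid cells, then passes them to the grid's MultiBlocInGrid with telegraph, appear and lifespan timings.
; It also triggers the VFX and spawn sound and changes the skill state.
; InitVFX themes the effect using the player's arena bloc material and skin-table color.
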(event EventBeginPlay
  (|CallParentFunction))

(event EventTick
  (params (DeltaSeconds :type Float%20%28single-precision%29))
  (|CallParentFunction DeltaSeconds))

(fn ConstructionScript
  (|CallParentFunction))

(fn UseSkill
  (bind _fighteruser (Variables|Default|GetFighterUser))
  (bind _returnvalue (Transformation|GetActorTransform _fighteruser))
  (bind _returnvalue_2 (Math|Vector|GetRightVector (.rotation _returnvalue)))
  (|CallParentFunction)
  (bind _asbp_gi (Utilities|Casting|CastToBP_GI (Game|GetGameInstance)))
  (Variables|Default|SetGrid%20Offset (Variables|/Game/BP/BP_BattleManager.BP_BattleManager_C|GetOffset (Variables|/Game/BP/BP_GI.BP_GI_C|GetBattleManager _asbp_gi)))
  (bind (_xgridpos _ygridpos) (Default|WorldPostoGridPos (Variables|/Game/BP/BP_BattleManager.BP_BattleManager_C|GetGrid (Variables|/Game/BP/BP_GI.BP_GI_C|GetBattleManager _asbp_gi)) (+ (* (Math|Vector|GetForwardVector (.rotation _returnvalue)) (Variables|Default|GetGrid%20Offset)) (+ (/ (Variables|Default|GetGrid%20Offset) 2) (.location _returnvalue)))))
  (bind (_xgridpos_2 _ygridpos_2) (Default|WorldPostoGridPos (Variables|/Game/BP/BP_BattleManager.BP_BattleManager_C|GetGrid (Variables|/Game/BP/BP_GI.BP_GI_C|GetBattleManager _asbp_gi)) (+ (+ (/ (Variables|Default|GetGrid%20Offset) 2) (.location _returnvalue)) (* _returnvalue_2 (Variables|Default|GetGrid%20Offset)) (* (Math|Vector|GetForwardVector (.rotation _returnvalue)) (Variables|Default|GetGrid%20Offset)))))
  (bind (_xgridpos_3 _ygridpos_3) (Default|WorldPostoGridPos (Variables|/Game/BP/BP_BattleManager.BP_BattleManager_C|GetGrid (Variables|/Game/BP/BP_GI.BP_GI_C|GetBattleManager _asbp_gi)) (+ (+ (/ (Variables|Default|GetGrid%20Offset) 2) (.location _returnvalue)) (* _returnvalue_2 (Variables|Default|GetGrid%20Offset) -1) (* (Math|Vector|GetForwardVector (.rotation _returnvalue)) (Variables|Default|GetGrid%20Offset)))))
  (bind _output_get (Variables|Default|SetBlocPos (Utilities|Array|MakeArray (Math|Vector|MakeVector (Math|Conversions|ToFloat(Integer) _xgridpos) (Math|Conversions|ToFloat(Integer) _ygridpos) 0.0) (Math|Vector|MakeVector (Math|Conversions|ToFloat(Integer) _xgridpos_2) (Math|Conversions|ToFloat(Integer) _ygridpos_2) 0.0) (Math|Vector|MakeVector (Math|Conversions|ToFloat(Integer) _xgridpos_3) (Math|Conversions|ToFloat(Integer) _ygridpos_3) 0.0))))
  (Default|MultiBlocinGrid (Variables|/Game/BP/BP_BattleManager.BP_BattleManager_C|GetGrid (Variables|/Game/BP/BP_GI.BP_GI_C|GetBattleManager _asbp_gi)) _output_get 4.0 0.5 0.5 1.0 (Variables|Default|GetFighterUser))
  (Components|Activation|Activate (Variables|Default|GetVFX_BlocBarrier) true)
  (Audio|PlaySound2D "/Game/Sounds/SoundEffect/BlocSpawn.BlocSpawn" 1.0 1.0 0.0 0 0)
  (CallFunction|ChangeState "NewEnumerator2"))

(fn PauseVFX
  (params (Enable :type Boolean))
  (Variables|Default|SetVFXs (Utilities|Array|MakeArray (Variables|Default|GetVFX_BlocBarrier)))
  (|CallParentFunction Enable))

(fn InitVFX
  (|CallParentFunction)
  (Class|NiagaraComponent|SetVariableMaterial (Variables|Default|GetVFX_BlocBarrier) "BlocsMaterial" (.Bloc (Utilities|Struct|BreakS_ArenaSkin (.Arena (Utilities|Struct|BreakS_NewPlayerSkin (Variables|/Game/BP/Players/Fighter/BP_FighterPawn.BP_FighterPawn_C|GetPlayerSkin (Variables|Default|GetFighterUser)))))))
  (bind _returnvalue (CallFunction|GetSkinSettingsRowName))
  (bind _skinsettings (Variables|Default|GetSkinSettings)
    (:then
      (bind _returnvalue_2 (Utilities|GetDataTableRow _skinsettings _returnvalue)
        (:then
          (Effects|Components|ParticleSystem|SetColorParameter (Variables|Default|GetVFX_BlocBarrier) "Color" (Utilities|Struct|BreakS_BlocBarrierSkin _returnvalue_2)))
        (:RowNotFound
          (CallFunction|CallSkinSettingsException "NOTFOUND"))))
    (:else
      (CallFunction|CallSkinSettingsException "NULL"))))