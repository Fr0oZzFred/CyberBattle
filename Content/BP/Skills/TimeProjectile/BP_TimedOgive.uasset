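; Skill projectile that flies along its direction and explodes after a random distance or on overlapping a block, border or other projectile.
; Explode starts a timer in Tick that grows the collision sphere to Range, alongside Niagara VFX, camera shake and sound.
; Actor overlaps destruct the target fighter and annihilate blocks.
; A tick-counted delay precedes self-destruction, and game-state changes from BP_GI drive visibility.
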(event OnComponentBeginOverlap(ExplosionCollide)
  (params (OverlappedComponent :type Primitive%20Component%20Object%20Reference) (OtherActor :type Actor%20Object%20Reference) (OtherComp :type Primitive%20Component%20Object%20Reference) (OtherBodyIndex :type Integer) (bFromSweep :type Boolean) (SweepResult :type Hit%20Result%20Structure%20%28by%20ref%29)))

(event OnComponentBeginOverlap(Box)
  (params (OverlappedComponent :type Primitive%20Component%20Object%20Reference) (OtherActor :type Actor%20Object%20Reference) (OtherComp :type Primitive%20Component%20Object%20Reference) (OtherBodyIndex :type Integer) (bFromSweep :type Boolean) (SweepResult :type Hit%20Result%20Structure%20%28by%20ref%29))
  (bind _asbp_projectile_pawn (Utilities|Casting|CastToBP_ProjectilePawn OtherActor))
  (CallFunction|Explode)
  (Default|Destroy _asbp_projectile_pawn))

(event EventBeginPlay
  (bind _asbp_gi (Utilities|Casting|CastToBP_GI (Game|GetGameInstance)))
  (EventDispatchers|BindEventtoOnGameStateChanged _asbp_gi (|OnGameState_Changed))
  (Variables|Default|SetStartLocation (.location (Transformation|GetActorTransform)))
  (Variables|Default|SetDistance (Math|Random|RandomFloatinRange 4e+02 8e+02))
  (Variables|Default|SetWaveTimer (Variables|Default|GetWaveDuration)))

(event Collision|EventActorBeginOverlap
  (params (OtherActor :type Actor%20Object%20Reference))
  (Utilities|FlowControl|Sequence
    (:then_0
      (bind _asbp_fighter_pawn (Utilities|Casting|CastToBP_FighterPawn OtherActor))
      (if (== _asbp_fighter_pawn (Variables|Default|GetTargetFighter))
        (Default|Destruct _asbp_fighter_pawn true)))
    (:then_1
      (bind _asbp_bloc (Utilities|Casting|CastToBP_Bloc OtherActor))
      (Default|Annihilate _asbp_bloc)
      (CallFunction|Explode))
    (:then_2
      (Utilities|Casting|CastToBP_Border OtherActor)
      (CallFunction|Explode))))

(event EventTick
  (params (DeltaSeconds :type Float%20%28single-precision%29))
  (bind _speed (Variables|Default|Getspeed))
  (bind _output_get (Variables|Default|SetDelayTimer (- (stale _output_get) DeltaSeconds)))
  (|DebugCollisionSphere)
  (Variables|Default|SetCurrentDistance (Math|Vector|Distance(Vector) (Variables|Default|GetStartLocation) (.location (Transformation|GetActorTransform))))
  (if (!= (/ (Variables|Default|GetCurrentDistance) (Variables|Default|GetDistance)) 0.0)
    (Effects|Components|ParticleSystem|SetFloatParameter (Variables|Default|GetVFX_TimedProjectile) "LifetimeOverDistance" (/ (Variables|Default|GetCurrentDistance) (Variables|Default|GetDistance))))
  (if (< (Variables|Default|GetDistance) (Variables|Default|GetCurrentDistance))
    (CallFunction|Explode)
    (else
      (Transformation|AddActorWorldOffset (* (Math|Vector|Normalize (Variables|Default|GetDirection)) (Math|Vector|MakeVector _speed _speed 0.0)))))
  (if (< (Variables|Default|GetWaveTimer) (Variables|Default|GetWaveDuration))
    (bind _output_get_2 (Variables|Default|SetWaveTimer (+ (Variables|Default|GetWaveTimer) DeltaSeconds)))
    (Components|Sphere|SetSphereRadius (Variables|Default|GetExplosionCollide) (Math|Float|Lerp 0.0 (Variables|Default|GetRange) (/ _output_get_2 (Variables|Default|GetWaveDuration))) true)
    (elif (not (== (Variables|Default|GetWaveTimer) (Variables|Default|GetWaveDuration)))
      (if (< (Variables|Default|GetDelayTimer) -1e+01) ; DelayTimer already set at -10
        (Utilities|DelaywithTimer (Variables|Default|GetSnapshotDuration)
          (:Completed
            (Variables|Default|SetWaveTimer (Variables|Default|GetWaveDuration))
            (Actor|DestroyActor)))))))

(fn ConstructionScript)

(fn Explode
  (bind _returnvalue (Transformation|GetActorTransform))
  (if (== (Variables|Default|GetWaveDuration) (Variables|Default|GetWaveTimer))
    (Variables|Default|SetWaveTimer 0.0)
    (Camera|PlayWorldCameraShake "/Game/BP/BP_CameraShake2.BP_CameraShake2_C" (Transformation|GetActorLocation) 0.0 2e+03)
    (Variables|Default|SetDistance 0.0)
    (Effects|Components|ParticleSystem|SetFloatParameter (Variables|Default|GetVFX_TimedProjectile) "LifetimeOverDistance" 1.0)
    (Components|Activation|Deactivate (Variables|Default|GetVFX_TimedProjectile))
    (bind _returnvalue_2 (Niagara|SpawnSystematLocation "/Game/BP/Skills/TimeProjectile/VFX_WaveExplosion.VFX_WaveExplosion" (.location _returnvalue) (.rotation _returnvalue) (.scale _returnvalue)))
    (Effects|Components|ParticleSystem|SetFloatParameter _returnvalue_2 "Range" (Variables|Default|GetRange))
    (Effects|Components|ParticleSystem|SetFloatParameter _returnvalue_2 "WaveDuration" (Variables|Default|GetWaveDuration))
    (Effects|Components|ParticleSystem|SetFloatParameter _returnvalue_2 "SnapshotDuration" (Variables|Default|GetSnapshotDuration))
    (Audio|PlaySound2D "/Game/Sounds/SoundEffect/Explosion.Explosion" 1.0 1.0 0.0 0 0)))

(event Custom|OnGameStateChanged
  (params (New%20State :type E_GameState%20Enum :default "NewEnumerator0"))
  (switch Utilities|FlowControl|Switch|SwitchonE_GameState New%20State
    (:NewEnumerator3
      (CallFunction|SetEnable true false))
    (:NewEnumerator5
      (CallFunction|SetEnable true false))
    (:NewEnumerator4
      (CallFunction|SetEnable true true))))

(fn SetEnable
  (params (Enable :type Boolean) (Hide :type Boolean))
  (Actor|Tick|SetActorTickEnabled Enable)
  (Rendering|SetVisibility (Variables|Default|GetDefaultSceneRoot) (not Hide) true)
  (Collision|SetActorEnableCollision Enable)
  (return false))