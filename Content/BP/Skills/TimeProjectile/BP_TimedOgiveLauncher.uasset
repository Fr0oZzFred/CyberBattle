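; BP_TimedOgiveLauncher is a fighter skill that launches a BP_TimedOgive projectile targeted at the opposing fighter.
; When used, it runs the parent skill logic, then picks P1 or P2 from the GameInstance's BattleManager as the enemy, based on the user's index.
; It spawns the projectile at the user's location and rotation, passes the forward vector and target, then changes the skill's state.
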(event EventBeginPlay
  (|CallParentFunction) ; This node is disabled and will not be called.\nDrag off pins to build functionality.
)

(event Collision|EventActorBeginOverlap
  (params (OtherActor :type Actor%20Object%20Reference)))

(event EventTick
  (params (DeltaSeconds :type Float%20%28single-precision%29))
  (|CallParentFunction DeltaSeconds) ; This node is disabled and will not be called.\nDrag off pins to build functionality.
)

(fn ConstructionScript
  (|CallParentFunction))

(fn UseSkill
  (bind _fighteruser (Variables|Default|GetFighterUser))
  (bind _returnvalue (Transformation|GetActorTransform _fighteruser))
  (|CallParentFunction)
  (bind _asbp_gi (Utilities|Casting|CastToBP_GI (Game|GetGameInstance)))
  (if (== (Variables|/Game/BP/Players/Fighter/BP_FighterPawn.BP_FighterPawn_C|GetIndex (Variables|Default|GetFighterUser)) 0)
    (Variables|Default|SetFighterEnemy (Variables|/Game/BP/BP_BattleManager.BP_BattleManager_C|GetP2 (Variables|/Game/BP/BP_GI.BP_GI_C|GetBattleManager _asbp_gi)))
    (else
      (Variables|Default|SetFighterEnemy (Variables|/Game/BP/BP_BattleManager.BP_BattleManager_C|GetP1 (Variables|/Game/BP/BP_GI.BP_GI_C|GetBattleManager _asbp_gi)))))
  (Game|SpawnActorfromClass "/Game/BP/Skills/TimeProjectile/BP_TimedOgive.BP_TimedOgive_C" (Math|Transform|MakeTransform (.location _returnvalue) (.rotation _returnvalue) "1.000000,1.000000,1.000000") "Undefined" 0 (Transformation|GetActorForwardVector _fighteruser) (Variables|Default|GetFighterEnemy) 0)
  (CallFunction|ChangeState "NewEnumerator2"))