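; BP_ProjectilePawn is a fighter projectile that moves horizontally along its Direction by a Speed step each tick, without delta-time scaling.
; Overlapping a fighter with a different Index calls RestoreShield on its stored Fighter reference, while overlapping another projectile destroys both.
; Its destruction spawns an impact Niagara effect facing against the travel direction.
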(event Custom|OnDestroyed_Event
  (params (DestroyedActor :type Actor%20Object%20Reference))
  (Niagara|SpawnSystematLocation "/Game/Placeholder/Fred/VFX_ShotImpact.VFX_ShotImpact" (Transformation|GetWorldLocation (Variables|Default|GetDefaultSceneRoot)) (Math|Rotator|MakeRotfromZ (* (Variables|Default|GetDirection) -1.0))))

(event EventBeginPlay
  ;[1 1 1] Set Material
  (Rendering|Material|SetMaterial (Variables|Default|GetCube) 0 (Utilities|Select :Index (Variables|Default|GetIndex) :Option%200 "/Game/Materials/MI_Projectile.MI_Projectile" :Option%201 "/Game/Materials/MI_Projectile.MI_Projectile"))
  (EventDispatchers|BindEventtoOnDestroyed (delegate Custom|OnDestroyed_Event)))

(event EventTick
  (params (DeltaSeconds :type Float%20%28single-precision%29))
  (bind _returnvalue (Transformation|GetActorTransform))
  (bind _speed (Variables|Default|Getspeed))
  ;[1 1 1] Move Forward in direction
  (Transformation|SetRelativeTransform (Variables|Default|GetDefaultSceneRoot) (Math|Transform|MakeTransform (+ (* (Math|Vector|Normalize (Variables|Default|GetDirection)) (Math|Vector|MakeVector _speed _speed 0.0)) (.location _returnvalue)) (.rotation _returnvalue) (.scale _returnvalue)) false false))

(event Collision|EventActorBeginOverlap
  (params (OtherActor :type Actor%20Object%20Reference))
  (bind _asbp_fighter_pawn (Utilities|Casting|CastToBP_FighterPawn OtherActor)
    (:then
      (if (!= (Variables|Default|GetIndex) (Variables|/Game/BP/BP_FighterPawn.BP_FighterPawn_C|GetIndex _asbp_fighter_pawn))
        (Default|RestoreShield (Variables|Default|GetFighter))))
    (:CastFailed
      (bind _asbp_projectile_pawn (Utilities|Casting|CastToBP_ProjectilePawn OtherActor))
      (Actor|DestroyActor _asbp_projectile_pawn)
      (Actor|DestroyActor))))

(fn ConstructionScript)