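; BP_TutoRotationTarget is a tutorial target for the rotation-shot step, advancing the tutorial when a projectile hits it.
; On BeginPlay it feeds Niagara material parameters with P1's attack key icon and a left or right joystick icon, depending on P1's inverted-control setting.
; Overlap by a BP_ProjectilePawn fires and unbinds the Step2TutoRotaShot dispatcher, then hides, disables collision and destroys the actor.
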(event EventBeginPlay
  (bind _returnvalue (Game|GetGameInstance))
  (bind _vfx_rotationtarget (Variables|Default|GetVFX_RotationTarget))
  (bind _asbp_gi (Utilities|Casting|CastToBP_GI _returnvalue))
  (bind (_found _out_row) (Default|FindKeyImage _asbp_gi (Variables|/Game/BP/BP_GI.BP_GI_C|GetP1_Actions _asbp_gi) "/Game/Inputs/IA_Attack.IA_Attack"))
  (if _found
    (Class|NiagaraComponent|SetVariableMaterial _vfx_rotationtarget "ShotKeyMaterial" (.KeyMaterial (Utilities|Struct|BreakS_KeyImage _out_row))))
  (Class|NiagaraComponent|SetVariableMaterial _vfx_rotationtarget "JoystickKeyMaterial" (select (Variables|/Game/BP/Players/Fighter/BP_FighterPawn.BP_FighterPawn_C|GetInvertedControl (Variables|/Game/BP/BP_BattleManager.BP_BattleManager_C|GetP1 (Variables|/Game/BP/BP_GI.BP_GI_C|GetBattleManager _asbp_gi))) "/Game/UI/Buttons/MI_R_Joystick.MI_R_Joystick" "/Game/UI/Buttons/MI_L_Joystick.MI_L_Joystick")))

(event Collision|EventActorBeginOverlap
  (params (OtherActor :type Actor%20Object%20Reference))
  (Utilities|Casting|CastToBP_ProjectilePawn OtherActor)
  (Default|CallStep2TutoRotaShot)
  (EventDispatchers|UnbindallEventsfromStep2TutoRotaShot)
  (Rendering|SetVisibility (Variables|Default|GetSphere) false false)
  (Collision|SetActorEnableCollision false)
  (Actor|DestroyActor))

(fn ConstructionScript)