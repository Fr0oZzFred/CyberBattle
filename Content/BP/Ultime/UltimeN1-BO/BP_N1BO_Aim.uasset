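; Aim actor for the N1-BO ultimate that tracks a Fighter while spinning at a fixed tilt.
; Each Tick it moves to the Fighter's location plus an offset and advances its roll by the spin speed, keeping pitch and yaw constant.
; When the Fighter is dead, it anchors to that Fighter's Station instead, with the base X offset mirrored by the Fighter's index.
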(event EventBeginPlay)

(event EventTick
  (params (DeltaSeconds :type Float%20%28single-precision%29))
  (bind _offsetbase (Variables|Default|GetOffsetBase))
  (if (Variables|/Game/BP/Players/Fighter/BP_FighterPawn.BP_FighterPawn_C|GetIsDead (Variables|Default|GetFighter))
    (Transformation|SetActorTransform (Math|Transform|MakeTransform (+ (.location (Transformation|GetActorTransform (Variables|/Game/BP/Players/Fighter/BP_FighterPawn.BP_FighterPawn_C|GetStation (Variables|Default|GetFighter)))) (Math|Vector|MakeVector (* (.x _offsetbase) (Utilities|Select :Index (Variables|/Game/BP/Players/Fighter/BP_FighterPawn.BP_FighterPawn_C|GetIndex (Variables|Default|GetFighter)) :Option%200 -1.0 :Option%201 1.0)) (.y _offsetbase) (.z _offsetbase))) (Math|Rotator|MakeRotator (+ (* (Variables|Default|GetSpinSspeed) DeltaSeconds) (.roll (Transformation|GetActorRotation))) 5e+01 2.7e+02) "1.000000,1.000000,1.000000"))
    (else
      (Transformation|SetActorTransform (Math|Transform|MakeTransform (+ (Variables|Default|GetOffsetFighter) (.location (Transformation|GetActorTransform (Variables|Default|GetFighter)))) (Math|Rotator|MakeRotator (+ (* (Variables|Default|GetSpinSspeed) DeltaSeconds) (.roll (Transformation|GetActorRotation))) 5e+01 2.7e+02) "1.000000,1.000000,1.000000")))))

(fn ConstructionScript)