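; Ultimate ability for the fighter N1-BO that grants its user auto-aim for a limited duration.
; On use, it enables auto-aim and spawns a BP_N1BO_Aim actor at the opposing player's pawn, living as long as the ultimate.
; Tick counts up the duration, then disables auto-aim and changes state.
; Game state changes from BP_GI toggle ticking, so the timer runs only in game; the Hide flag is unused.
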(event Custom|CustomEvent
  (params (New%20State :type E_GameState%20Enum :default "NewEnumerator0"))
  (switch Utilities|FlowControl|Switch|SwitchonE_GameState New%20State
    (:NewEnumerator7
      (CallFunction|SetEnable false true :!label _label))
    (:NewEnumerator3
      (CallFunction|SetEnable true false))
    (:NewEnumerator5
      (CallFunction|SetEnable false false))
    (:NewEnumerator4
      (goto _label))))

(event EventBeginPlay
  (|CallParentFunction)
  (bind _asbp_gi (Utilities|Casting|CastToBP_GI (Game|GetGameInstance)))
  (EventDispatchers|BindEventtoOnGameStateChanged _asbp_gi (delegate Custom|CustomEvent)))

(event Collision|EventActorBeginOverlap
  (params (OtherActor :type Actor%20Object%20Reference)))

(event EventTick
  (params (DeltaSeconds :type Float%20%28single-precision%29))
  (|CallParentFunction DeltaSeconds)
  (if (< (Variables|Default|GetUltimeDurationTimer) (Variables|Default|GetUltimeDuration))
    (Variables|Default|SetUltimeDurationTimer (+ (Variables|Default|GetUltimeDurationTimer) DeltaSeconds))
    (elif (not (== (Variables|Default|GetUltimeDurationTimer) (Variables|Default|GetUltimeDuration)))
      (Variables|Default|SetUltimeDurationTimer (Variables|Default|GetUltimeDuration))
      (Variables|/Game/BP/Players/Fighter/BP_FighterPawn.BP_FighterPawn_C|SetUseAutoAim (Variables|Default|GetFighterUser) false)
      (CallFunction|ChangeState "NewEnumerator2"))))

(fn ConstructionScript
  (|CallParentFunction))

(fn UseUltime
  (bind _fighteruser (Variables|Default|GetFighterUser))
  (|CallParentFunction)
  (Variables|/Game/BP/Players/Fighter/BP_FighterPawn.BP_FighterPawn_C|SetUseAutoAim _fighteruser true)
  (bind _asbp_fighter_pawn (Utilities|Casting|CastToBP_FighterPawn (Game|Player|GetPlayerPawn (Utilities|Select :Index (Variables|/Game/BP/Players/Fighter/BP_FighterPawn.BP_FighterPawn_C|GetIndex _fighteruser) :Option%200 1 :Option%201 0))))
  (Game|SpawnActorfromClass "/Game/BP/Ultime/UltimeN1-BO/BP_N1BO_Aim.BP_N1BO_Aim_C" (Transformation|GetActorTransform _asbp_fighter_pawn) "Undefined" 0 _asbp_fighter_pawn (Variables|Default|GetUltimeDuration) 0))

(fn SetEnable
  (params (Enable :type Boolean) (Hide :type Boolean))
  (Actor|Tick|SetActorTickEnabled Enable)
  (return false))