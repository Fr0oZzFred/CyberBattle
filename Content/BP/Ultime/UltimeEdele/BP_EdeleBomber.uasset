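; Bomber actor for Edele's ultimate that flies to the enemy fighter's spawn point and drops a bomb given that fighter's station.
; Tick drives forward flight and rotation, while a timed radar fires two line traces and shoots pooled projectiles at detected blocs.
; After the drop, it turns to a random side with a timeline-driven roll.
; Enemy projectiles drain its HP; it self-destructs at zero health or outside arena bounds.
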(event EventBeginPlay
  (bind _asbp_gi (Utilities|Casting|CastToBP_GI (Game|GetGameInstance)))
  (bind _output_get (Variables|Default|SetEnemyFighter (Utilities|Select :Index (Variables|Default|GetIndex) :Option%200 (Variables|/Game/BP/BP_BattleManager.BP_BattleManager_C|GetP2 (Variables|/Game/BP/BP_GI.BP_GI_C|GetBattleManager _asbp_gi)) :Option%201 (Variables|/Game/BP/BP_BattleManager.BP_BattleManager_C|GetP1 (Variables|/Game/BP/BP_GI.BP_GI_C|GetBattleManager _asbp_gi)))))
  (bind _output_get_2 (Variables|Default|SetObjective (Utilities|Array|Get(acopy) (Variables|/Game/BP/Players/Fighter/BP_FighterPawn.BP_FighterPawn_C|GetSpawnPos _output_get))))
  (Transformation|SetActorRotation (Math|Rotator|FindLookatRotation (Transformation|GetActorLocation) _output_get_2))
  (Variables|Default|SetDesireRotation (Transformation|GetActorRotation)))

(event Collision|EventActorBeginOverlap
  (params (OtherActor :type Actor%20Object%20Reference))
  (bind _asbp_projectile_pawn (Utilities|Casting|CastToBP_ProjectilePawn OtherActor))
  (if (!= (Variables|/Game/BP/Players/Projectile/BP_ProjectilePawn.BP_ProjectilePawn_C|GetIndex _asbp_projectile_pawn) (Variables|Default|GetIndex))
    (Default|Destroy _asbp_projectile_pawn)
    (bind _result (Math|Float|DecrementFloat (Variables|Default|GetHP))
      (:%20%20
        (if (< _result 0.0)
          (Actor|DestroyActor))))))

(event EventTick
  (params (DeltaSeconds :type Float%20%28single-precision%29))
  (bind _returnvalue (Transformation|GetActorRotation))
  (bind _returnvalue_2 (Transformation|GetActorLocation))
  (bind _output_get (Variables|Default|SetRadarTimer (- (Variables|Default|GetRadarTimer) DeltaSeconds)))
  (if (< _output_get 0.0)
    (CallFunction|CheckBloc))
  (Transformation|SetActorLocation (+ (Transformation|GetActorLocation) (* (Math|Vector|GetForwardVector (Transformation|GetWorldRotation (Variables|Default|GetBody))) (* DeltaSeconds (Variables|Default|GetSpeed)))) false false)
  (Transformation|SetActorRotation (Math|Rotator|Lerp(Rotator) (Transformation|GetActorRotation) (Variables|Default|GetDesireRotation) (* DeltaSeconds (Variables|Default|GetRotSpeed)) true))
  (if (and (not (Variables|Default|GetDropBomb)) (< (Math|Vector|Distance(Vector) (Transformation|GetActorLocation) (Variables|Default|GetObjective)) 3e+01))
    (bind _turnleft (CallFunction|Drop))
    (if _turnleft
      (bind _rotation (Timeline|BomberLeft Play)
        (:Update
          (Transformation|SetActorRotation (Math|Rotator|MakeRotator _rotation (.pitch _returnvalue) (.yaw _returnvalue)))))
      (else
        (bind _rotation_2 (Timeline|BomberRight Play)
          (:Update
            (Transformation|SetActorRotation (Math|Rotator|MakeRotator _rotation_2 (.pitch _returnvalue) (.yaw _returnvalue))))))))
  (if (or (< (.x _returnvalue_2) -5.5e+02) (> (.x _returnvalue_2) 2.9e+03))
    (Actor|DestroyActor :!label _label)
    (elif (or (< (.y _returnvalue_2) -5.5e+02) (> (.y _returnvalue_2) 2.9e+03))
      (goto _label))))

(fn ConstructionScript)

(fn CheckBloc
  (bind _returnvalue (Transformation|GetActorTransform))
  (Variables|Default|SetRadarTimer (Variables|Default|GetRadarCooldown))
  (for _index (range 0 1)
    (bind (_outhit _returnvalue_2) (Collision|LineTraceByChannel (+ (.location _returnvalue) (Math|Vector|MakeVector 0.0 (Utilities|Array|Get(acopy) (LocalVariables|GetOffset) _index) 0.0)) (+ (.location _returnvalue) (* (Math|Vector|GetForwardVector (.rotation _returnvalue)) 2e+02)) "TraceTypeQuery1" false 0 "None"))
    (if _returnvalue_2
      (Utilities|Casting|CastToBP_Bloc (.hitactor _outhit))
      (CallFunction|Shot)))
  (return))

(fn Shot
  (bind _fighteruser (Variables|Default|GetfighterUser))
  (bind _asbp_gi (Utilities|Casting|CastToBP_GI (Game|GetGameInstance)))
  (if (Utilities|Enum|Equal(Enum) (Variables|/Game/BP/BP_GI.BP_GI_C|GetCurrentState _asbp_gi) "NewEnumerator3")
    (Default|SpawnProjectile (Variables|/Game/BP/Players/Fighter/BP_FighterPawn.BP_FighterPawn_C|GetPoolManager _fighteruser) (Math|Transform|MakeTransform (Transformation|GetWorldLocation (Variables|Default|GetBody)) (.rotation (Transformation|GetActorTransform)) "1.000000,1.000000,1.000000") (Variables|Default|GetIndex) (Transformation|GetActorForwardVector) (Variables|/Game/BP/Players/Fighter/BP_FighterPawn.BP_FighterPawn_C|GetProjectileSpeed _fighteruser) 0.0 (Variables|/Game/BP/Players/Fighter/BP_FighterPawn.BP_FighterPawn_C|GetProjectileDamageToFighter _fighteruser) 1e+02 (.Projectile (Utilities|Struct|BreakS_NewPlayerSkin (Variables|/Game/BP/Players/Fighter/BP_FighterPawn.BP_FighterPawn_C|GetPlayerSkin _fighteruser))) "NewEnumerator5")
    (Audio|PlaySound2D (Utilities|Select :Index (Math|Random|RandomInteger 5) :Option%200 "/Game/Sounds/SoundEffect/Fighter/laserShoot1.laserShoot1" :Option%201 "/Game/Sounds/SoundEffect/Fighter/laserShoot2.laserShoot2" :Option%202 "/Game/Sounds/SoundEffect/Fighter/laserShoot3.laserShoot3" :Option%203 "/Game/Sounds/SoundEffect/Fighter/laserShoot4.laserShoot4" :Option%204 "/Game/Sounds/SoundEffect/Fighter/laserShoot5.laserShoot5" :Option%205 "/Game/Sounds/SoundEffect/Fighter/laserShoot6.laserShoot6") 1.0 1.0 0.0 0 0)))

(fn Drop
  (bind _returnvalue (Math|Random|RandomFloatinRange 8e+01 1e+02))
  (bind _returnvalue_2 (Transformation|GetActorRotation))
  (Variables|Default|SetDropBomb true)
  (Rendering|SetVisibility (Variables|Default|GetBomb) false false)
  (Game|SpawnActorfromClass "/Game/BP/Ultime/UltimeEdele/BP_DroppedBomb.BP_DroppedBomb_C" (Transformation|GetActorTransform) "Undefined" 0 (Variables|/Game/BP/Players/Fighter/BP_FighterPawn.BP_FighterPawn_C|GetStation (Variables|Default|GetEnemyFighter)) 0)
  (bind _output_get (LocalVariables|SetExitSide (Math|Random|RandomBool)))
  (if _output_get
    (Variables|Default|SetDesireRotation (Math|Rotator|MakeRotator (.roll _returnvalue_2) (.pitch _returnvalue_2) _returnvalue))
    (else
      (Variables|Default|SetDesireRotation (Math|Rotator|MakeRotator (.roll _returnvalue_2) (.pitch _returnvalue_2) (* _returnvalue -1.0)))))
  (return (LocalVariables|GetExitSide)))