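; Ultimate ability actor for Edele that sends waves of fighters and bombers into the arena for a limited duration.
; While the duration runs, Tick counts down two independent timers, each spawning its unit and re-rolling a random delay on expiry.
; Fighters appear beyond a random one of four edges with inward rotation, while bombers spawn around the arena half selected by the user's index.
; Each spawned unit receives the user and their index.
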(event EventBeginPlay
  (|CallParentFunction) ; This node is disabled and will not be called.\nDrag off pins to build functionality.
)

(event Collision|EventActorBeginOverlap
  (params (OtherActor :type Actor%20Object%20Reference)))

(event EventTick
  (params (DeltaSeconds :type Float%20%28single-precision%29))
  (|CallParentFunction DeltaSeconds)
  (if (< (Variables|Default|GetUltimeDurationTimer) (Variables|Default|GetUltimeDuration))
    (Variables|Default|SetUltimeDurationTimer (+ (Variables|Default|GetUltimeDurationTimer) DeltaSeconds))
    (bind (_newtimer _hasended) (CallFunction|DecreaseTimer (Variables|Default|GetFighterSpawnTimer) DeltaSeconds))
    (Variables|Default|SetFighterSpawnTimer _newtimer)
    (if _hasended
      (CallFunction|SpawnFighter))
    (bind (_newtimer_2 _hasended_2) (CallFunction|DecreaseTimer (Variables|Default|GetBomberSpawnTimer) DeltaSeconds))
    (Variables|Default|SetBomberSpawnTimer _newtimer_2)
    (if _hasended_2
      (CallFunction|SpawnBomber))
    (elif (not (== (Variables|Default|GetUltimeDurationTimer) (Variables|Default|GetUltimeDuration)))
      (Variables|Default|SetUltimeDurationTimer (Variables|Default|GetUltimeDuration)))))

(fn ConstructionScript
  (|CallParentFunction))

(fn UseUltime
  (|CallParentFunction))

(fn DecreaseTimer
  (params (TimerToSet :type Float%20%28double-precision%29) (DeltaTime :type Float%20%28double-precision%29))
  (bind _returnvalue (- TimerToSet DeltaTime))
  (return _returnvalue (<= _returnvalue 0.0)))

(fn SpawnFighter
  (bind _returnvalue (Math|Random|RandomFloatinRange 1e+02 2e+03))
  (bind _returnvalue_2 (Math|Random|RandomFloatinRange 5e+01 9.5e+02))
  (bind _fighteruser (Variables|Default|GetFighterUser))
  (switch int (Math|Random|RandomInteger 4)
    (:0
      (LocalVariables|SetSpawnPos (Math|Vector|MakeVector -5.2e+02 _returnvalue_2 7e+01))
      (LocalVariables|SetRotation "0, 0, 0"))
    (:1
      (LocalVariables|SetSpawnPos (Math|Vector|MakeVector 2.72e+03 _returnvalue_2 7e+01))
      (LocalVariables|SetRotation "0.000000,180.000000,0.000000"))
    (:2
      (LocalVariables|SetSpawnPos (Math|Vector|MakeVector _returnvalue -5e+02 7e+01))
      (LocalVariables|SetRotation "0.000000,90.000000,0.000000"))
    (:3
      (LocalVariables|SetSpawnPos (Math|Vector|MakeVector _returnvalue 1.5e+03 7e+01))
      (LocalVariables|SetRotation "0.000000,-90.000000,0.000000")))
  (Game|SpawnActorfromClass "/Game/BP/Ultime/UltimeEdele/BP_EdeleFighter.BP_EdeleFighter_C" (Math|Transform|MakeTransform (LocalVariables|GetSpawnPos) (LocalVariables|GetRotation) "1.000000,1.000000,1.000000") "Undefined" 0 (Variables|/Game/BP/Players/Fighter/BP_FighterPawn.BP_FighterPawn_C|GetIndex _fighteruser) 3.5e+02 _fighteruser 0)
  (Variables|Default|SetFighterSpawnTimer (Math|Random|RandomFloatinRange (Variables|Default|GetFighterDelayMin) (Variables|Default|GetFighterDelayMax)))
  (return))

(fn SpawnBomber
  (bind _fighteruser (Variables|Default|GetFighterUser))
  (bind _fighteruser_2 (Variables|Default|GetFighterUser))
  (bind _fighteruser_3 (Variables|Default|GetFighterUser))
  (bind _index (Variables|/Game/BP/Players/Fighter/BP_FighterPawn.BP_FighterPawn_C|GetIndex _fighteruser))
  (bind _index_2 (Variables|/Game/BP/Players/Fighter/BP_FighterPawn.BP_FighterPawn_C|GetIndex _fighteruser_2))
  (bind _returnvalue (Utilities|Select :Index _index :Option%200 2.22e+03 :Option%201 1.05e+03))
  (bind _returnvalue_2 (Utilities|Select :Index _index_2 :Option%200 1.05e+03 :Option%201 -1.2e+02))
  (bind _returnvalue_3 (Math|Random|RandomFloatinRange _returnvalue_2 _returnvalue))
  (switch int (Math|Random|RandomInteger 4)
    (:0
      (LocalVariables|SetSpawn%20Pos (Math|Vector|MakeVector (Utilities|Select :Index (Variables|/Game/BP/Players/Fighter/BP_FighterPawn.BP_FighterPawn_C|GetIndex (Variables|Default|GetFighterUser)) :Option%200 2.22e+03 :Option%201 -1.2e+02) (Math|Random|RandomFloatinRange -1e+02 1.1e+03) 1e+02) :!label _label))
    (:1
      (goto _label))
    (:2
      (LocalVariables|SetSpawn%20Pos (Math|Vector|MakeVector _returnvalue_3 -1e+02 1e+02)))
    (:3
      (LocalVariables|SetSpawn%20Pos (Math|Vector|MakeVector _returnvalue_3 1.1e+03 1e+02))))
  (Game|SpawnActorfromClass "/Game/BP/Ultime/UltimeEdele/BP_EdeleBomber.BP_EdeleBomber_C" (Math|Transform|MakeTransform (LocalVariables|GetSpawn%20Pos) "0, 0, 0" "1.000000,1.000000,1.000000") "Undefined" 0 (Variables|/Game/BP/Players/Fighter/BP_FighterPawn.BP_FighterPawn_C|GetIndex _fighteruser_3) _fighteruser_3 0)
  (Variables|Default|SetBomberSpawnTimer (Math|Random|RandomFloatinRange (Variables|Default|GetBomberDelayMin) (Variables|Default|GetBomberDelayMax)))
  (return))