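; Bomb actor, apparently part of Edele's ultimate, that falls along a timeline-driven arc from its spawn point and damages a target Station.
; The Dropped timeline offsets it along its starting forward vector and vertically, with a trail VFX.
; When finished, it hides the mesh, plays explosion VFX and camera shake, damages a valid, vulnerable Station, then self-destructs via a Tick countdown if Station is valid.
; BP_GI game-state changes pause, hide or resume timeline, tick and effects.
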(event Custom|TryToResumeAnim
  (bind _dropped (Variables|Default|GetDropped))
  (if (not (Utilities|IsTimeLineFinished _dropped))
    (Audio|Components|Audio|Play _dropped)))

(event Custom|StopAnim
  (Audio|Components|Audio|Stop (Variables|Default|GetDropped)))

(event Custom|OnGameStateChanged
  (params (New%20State :type E_GameState%20Enum :default "NewEnumerator0"))
  (switch Utilities|FlowControl|Switch|SwitchonE_GameState New%20State
    (:NewEnumerator7
      (CallFunction|SetEnable false true :!label _label))
    (:NewEnumerator3
      (CallFunction|SetEnable true false))
    (:NewEnumerator5
      (CallFunction|SetEnable false false))
    (:NewEnumerator4
      (goto _label))))

(event EventBeginPlay
  (bind _returnvalue (Transformation|GetActorRotation))
  (bind _station (Variables|Default|GetStation))
  (Utilities|FlowControl|Sequence
    (:then_0
      (Variables|Default|SetStartPos (Transformation|GetActorLocation))
      (Variables|Default|SetforwardVectorStart (Math|Vector|GetForwardVector _returnvalue))
      (Variables|Default|SetStartRot _returnvalue)
      (Variables|Default|SetNotExploded true))
    (:then_1
      (Utilities|InitTimeline)
      (bind _asbp_gi (Utilities|Casting|CastToBP_GI (Game|GetGameInstance)))
      (EventDispatchers|BindEventtoOnGameStateChanged _asbp_gi (delegate Custom|OnGameStateChanged)))
    (:then_2
      (Components|Activation|Activate (Variables|Default|GetVFX_Trail) false)
      (bind (_direction _xpos _zpos) (Timeline|Dropped PlayFromStart)
        (:Update
          (Transformation|SetActorTransform (Math|Transform|MakeTransform (+ (Variables|Default|GetStartPos) (Math|Vector|MakeVector (* (.x (Variables|Default|GetforwardVectorStart)) _xpos) (* (.y (Variables|Default|GetforwardVectorStart)) _xpos) _zpos)) (Math|Rotator|MakeRotator (.roll (Variables|Default|GetStartRot)) (+ 0.0 (.pitch (Variables|Default|GetStartRot))) (.yaw (Variables|Default|GetStartRot))) "1.000000,1.000000,1.000000")))
        (:Finished
          (if (Variables|Default|GetNotExploded)
            (Components|Activation|Deactivate (Variables|Default|GetVFX_Trail))
            (Components|Activation|Activate (Variables|Default|GetVFX_Expurosion) false)
            (Rendering|SetVisibility (Variables|Default|GetCube) false false)
            (Camera|PlayWorldCameraShake "/Game/BP/BP_CameraShake2.BP_CameraShake2_C" (Transformation|GetActorLocation) 0.0 2e+03)
            (Variables|Default|SetNotExploded false)
            (Utilities|IsValid _station
              (:Is%20Valid
                (if (Variables|/Game/BP/Players/Station/BP_Station.BP_Station_C|GetIsVulnerable _station)
                  (Default|ApplyDamage _station 8.0 true))
                (Variables|Default|SetDestroyTimer 1.0)))))))))

(event Collision|EventActorBeginOverlap
  (params (OtherActor :type Actor%20Object%20Reference)))

(event EventTick
  (params (DeltaSeconds :type Float%20%28single-precision%29))
  (if (> (Variables|Default|GetDestroyTimer) 0.0)
    (bind _output_get (Variables|Default|SetDestroyTimer (- (Variables|Default|GetDestroyTimer) DeltaSeconds)))
    (if (< _output_get 0.0)
      (Actor|DestroyActor))))

(fn ConstructionScript)

(fn SetEnable
  (params (Enable :type Boolean) (Hide :type Boolean))
  (bind _returnvalue (not Hide))
  (bind _returnvalue_2 (not Enable))
  (bind _vfx_expurosion (Variables|Default|GetVFX_Expurosion))
  (bind _vfx_trail (Variables|Default|GetVFX_Trail))
  (Actor|Tick|SetActorTickEnabled Enable)
  (Rendering|SetVisibility (Variables|Default|GetCube) (and (not Hide) (Variables|Default|GetNotExploded)) false)
  (Class|NiagaraComponent|SetPaused _vfx_expurosion _returnvalue_2)
  (Rendering|SetVisibility _vfx_expurosion _returnvalue false)
  (Class|NiagaraComponent|SetPaused _vfx_trail _returnvalue_2)
  (Rendering|SetVisibility _vfx_trail _returnvalue false)
  (if Enable
    (CallFunction|TrytoResumeAnim)
    (else
      (CallFunction|StopAnim)))
  (return false))