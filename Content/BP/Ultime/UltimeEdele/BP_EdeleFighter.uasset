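; BP_EdeleFighter is an autonomous fighter for Edele's ultimate that flies straight ahead, firing until shot down or out of bounds.
; Tick timers drive randomized-interval cannon shots and a forward line trace that fires a short-range projectile at any BP_Bloc.
; Both shots use FighterUser's PoolManager, skin and projectile stats.
; Overlapping projectiles with another Index cost HP, and GameInstance state changes toggle tick and visibility.
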(event Custom|OnGameStateChanged
  (params (New%20State :type E_GameState%20Enum :default "NewEnumerator0"))
  (switch Utilities|FlowControl|Switch|SwitchonE_GameState New%20State
    (:NewEnumerator7
      (CallFunction|SetEnable false true :!label _label))
    (:NewEnumerator3
      (CallFunction|SetEnable true false))
    (:NewEnumerator5
      (CallFunction|SetEnable false false))
    (:NewEnumerator4
      (goto _label))))

(event EventBeginPlay
  (bind _asbp_gi (Utilities|Casting|CastToBP_GI (Game|GetGameInstance)))
  (EventDispatchers|BindEventtoOnGameStateChanged _asbp_gi (delegate Custom|OnGameStateChanged)))

(event Collision|EventActorBeginOverlap
  (params (OtherActor :type Actor%20Object%20Reference))
  (bind _asbp_projectile_pawn (Utilities|Casting|CastToBP_ProjectilePawn OtherActor))
  (if (!= (Variables|/Game/BP/Players/Projectile/BP_ProjectilePawn.BP_ProjectilePawn_C|GetIndex _asbp_projectile_pawn) (Variables|Default|GetIndex))
    (Default|Destroy _asbp_projectile_pawn)
    (bind _result (Math|Float|DecrementFloat (Variables|Default|GetHP))
      (:%20%20
        (if (< _result 0.0)
          (Actor|DestroyActor))))))

(event EventTick
  (params (DeltaSeconds :type Float%20%28single-precision%29))
  (bind _returnvalue (Transformation|GetActorLocation))
  (bind _output_get (Variables|Default|SetRadarTimer (- (Variables|Default|GetRadarTimer) DeltaSeconds)))
  (if (< _output_get 0.0)
    (CallFunction|CheckBloc))
  (bind _output_get_2 (Variables|Default|SetReloadTimer (- (Variables|Default|GetReloadTimer) DeltaSeconds)))
  (if (< _output_get_2 0.0)
    (CallFunction|Shot)
    (Variables|Default|SetReloadTimer (+ (Variables|Default|GetReloadCooldown) (Math|Random|RandomFloatinRange -0.75 0.75))))
  (Transformation|SetActorLocation (+ (Transformation|GetActorLocation) (* (Math|Vector|GetForwardVector (Transformation|GetWorldRotation (Variables|Default|GetBody))) (* DeltaSeconds (Variables|Default|GetSpeed)))) false false)
  (if (or (< (.x _returnvalue) -5.5e+02) (> (.x _returnvalue) 2.9e+03))
    (Actor|DestroyActor :!label _label)
    (elif (or (< (.y _returnvalue) -5.5e+02) (> (.y _returnvalue) 2.9e+03))
      (goto _label))))

(fn ConstructionScript)

(fn Shot
  (bind _fighteruser (Variables|Default|GetfighterUser))
  (bind _asbp_gi (Utilities|Casting|CastToBP_GI (Game|GetGameInstance)))
  (if (Utilities|Enum|Equal(Enum) (Variables|/Game/BP/BP_GI.BP_GI_C|GetCurrentState _asbp_gi) "NewEnumerator3")
    (Default|SpawnProjectile (Variables|/Game/BP/Players/Fighter/BP_FighterPawn.BP_FighterPawn_C|GetPoolManager _fighteruser) (Math|Transform|MakeTransform (Transformation|GetWorldLocation (Variables|Default|GetCannon)) (.rotation (Transformation|GetActorTransform)) "1.000000,1.000000,1.000000") (Variables|Default|GetIndex) (Transformation|GetActorForwardVector) (Variables|/Game/BP/Players/Fighter/BP_FighterPawn.BP_FighterPawn_C|GetProjectileSpeed _fighteruser) 0.0 (Variables|/Game/BP/Players/Fighter/BP_FighterPawn.BP_FighterPawn_C|GetProjectileDamageToFighter _fighteruser) (Variables|/Game/BP/Players/Fighter/BP_FighterPawn.BP_FighterPawn_C|GetMaxProjDistance _fighteruser) (.Projectile (Utilities|Struct|BreakS_NewPlayerSkin (Variables|/Game/BP/Players/Fighter/BP_FighterPawn.BP_FighterPawn_C|GetPlayerSkin _fighteruser))) "NewEnumerator4" false)
    (Audio|PlaySound2D (Utilities|Select :Index (Math|Random|RandomInteger 5) :Option%200 "/Game/Sounds/SoundEffect/Fighter/laserShoot1.laserShoot1" :Option%201 "/Game/Sounds/SoundEffect/Fighter/laserShoot2.laserShoot2" :Option%202 "/Game/Sounds/SoundEffect/Fighter/laserShoot3.laserShoot3" :Option%203 "/Game/Sounds/SoundEffect/Fighter/laserShoot4.laserShoot4" :Option%204 "/Game/Sounds/SoundEffect/Fighter/laserShoot5.laserShoot5" :Option%205 "/Game/Sounds/SoundEffect/Fighter/laserShoot6.laserShoot6") 1.0 1.0 0.0 0 0)))

(fn CheckBloc
  (bind _returnvalue (Transformation|GetActorTransform))
  (Variables|Default|SetRadarTimer (Variables|Default|GetRadarCooldown))
  (bind (_outhit _returnvalue_2) (Collision|LineTraceByChannel (.location _returnvalue) (+ (.location _returnvalue) (* (Math|Vector|GetForwardVector (.rotation _returnvalue)) 2e+02)) "TraceTypeQuery1" false 0 "None"))
  (if _returnvalue_2
    (Utilities|Casting|CastToBP_Bloc (.hitactor _outhit))
    (CallFunction|ShotBloc))
  (return))

(fn ShotBloc
  (bind _fighteruser (Variables|Default|GetfighterUser))
  (bind _asbp_gi (Utilities|Casting|CastToBP_GI (Game|GetGameInstance)))
  (if (Utilities|Enum|Equal(Enum) (Variables|/Game/BP/BP_GI.BP_GI_C|GetCurrentState _asbp_gi) "NewEnumerator3")
    (Default|SpawnProjectile (Variables|/Game/BP/Players/Fighter/BP_FighterPawn.BP_FighterPawn_C|GetPoolManager _fighteruser) (Math|Transform|MakeTransform (Transformation|GetWorldLocation (Variables|Default|GetBody)) (.rotation (Transformation|GetActorTransform)) "1.000000,1.000000,1.000000") (Variables|Default|GetIndex) (Transformation|GetActorForwardVector) (Variables|/Game/BP/Players/Fighter/BP_FighterPawn.BP_FighterPawn_C|GetProjectileSpeed _fighteruser) 0.0 (Variables|/Game/BP/Players/Fighter/BP_FighterPawn.BP_FighterPawn_C|GetProjectileDamageToFighter _fighteruser) 1e+02 (.Projectile (Utilities|Struct|BreakS_NewPlayerSkin (Variables|/Game/BP/Players/Fighter/BP_FighterPawn.BP_FighterPawn_C|GetPlayerSkin _fighteruser))) "NewEnumerator5" false)
    (Audio|PlaySound2D (Utilities|Select :Index (Math|Random|RandomInteger 5) :Option%200 "/Game/Sounds/SoundEffect/Fighter/laserShoot1.laserShoot1" :Option%201 "/Game/Sounds/SoundEffect/Fighter/laserShoot2.laserShoot2" :Option%202 "/Game/Sounds/SoundEffect/Fighter/laserShoot3.laserShoot3" :Option%203 "/Game/Sounds/SoundEffect/Fighter/laserShoot4.laserShoot4" :Option%204 "/Game/Sounds/SoundEffect/Fighter/laserShoot5.laserShoot5" :Option%205 "/Game/Sounds/SoundEffect/Fighter/laserShoot6.laserShoot6") 1.0 1.0 0.0 0 0)))

(fn SetEnable
  (params (Enable :type Boolean) (Hide :type Boolean))
  (Actor|Tick|SetActorTickEnabled Enable)
  (Rendering|SetVisibility (Variables|Default|GetBody) (not Hide) true)
  (return false))