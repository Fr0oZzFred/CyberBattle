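; Satoshi's ultimate ability, a child of a base ultimate that drops a timed black hole at the user's position.
; The Attraction volume captures one opposing fighter, whom Tick pulls inward by adding distance-scaled, clamped velocity to its movement, while the Center volume stuns opponents on overlap.
; When the duration expires, collision and VFX switch off and the state changes.
; Game-state changes from BP_GI enable, disable or hide the ability.
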(event OnComponentBeginOverlap(Attraction)
  (params (OverlappedComponent :type Primitive%20Component%20Object%20Reference) (OtherActor :type Actor%20Object%20Reference) (OtherComp :type Primitive%20Component%20Object%20Reference) (OtherBodyIndex :type Integer) (bFromSweep :type Boolean) (SweepResult :type Hit%20Result%20Structure%20%28by%20ref%29))
  (bind _asbp_fighter_pawn (Utilities|Casting|CastToBP_FighterPawn OtherActor))
  (if (!= (Variables|/Game/BP/Players/Fighter/BP_FighterPawn.BP_FighterPawn_C|GetIndex _asbp_fighter_pawn) (Variables|/Game/BP/Players/Fighter/BP_FighterPawn.BP_FighterPawn_C|GetIndex (Variables|Default|GetFighterUser)))
    (Variables|Default|SetIsAttracting true)
    (Variables|Default|SetCaptedFighter _asbp_fighter_pawn)))

(event OnComponentBeginOverlap(Center)
  (params (OverlappedComponent :type Primitive%20Component%20Object%20Reference) (OtherActor :type Actor%20Object%20Reference) (OtherComp :type Primitive%20Component%20Object%20Reference) (OtherBodyIndex :type Integer) (bFromSweep :type Boolean) (SweepResult :type Hit%20Result%20Structure%20%28by%20ref%29))
  (bind _asbp_fighter_pawn (Utilities|Casting|CastToBP_FighterPawn OtherActor))
  (if (!= (Variables|/Game/BP/Players/Fighter/BP_FighterPawn.BP_FighterPawn_C|GetIndex _asbp_fighter_pawn) (Variables|/Game/BP/Players/Fighter/BP_FighterPawn.BP_FighterPawn_C|GetIndex (Variables|Default|GetFighterUser)))
    (Default|SetStun _asbp_fighter_pawn 1.5 3e+01)))

(event OnComponentEndOverlap(Attraction)
  (params (OverlappedComponent :type Primitive%20Component%20Object%20Reference) (OtherActor :type Actor%20Object%20Reference) (OtherComp :type Primitive%20Component%20Object%20Reference) (OtherBodyIndex :type Integer))
  (if (== OtherActor (Variables|Default|GetCaptedFighter))
    (Variables|Default|SetIsAttracting false)
    (Variables|Default|SetCaptedFighter 0)))

(event Custom|CustomEvent
  (params (New%20State :type E_GameState%20Enum :default "NewEnumerator0"))
  (switch Utilities|FlowControl|Switch|SwitchonE_GameState New%20State
    (:NewEnumerator7
      (CallFunction|SetEnable false true :!label _label))
    (:NewEnumerator3
      (CallFunction|SetEnable true false))
    (:NewEnumerator5
      (CallFunction|SetEnable false false))
    (:NewEnumerator4
      (goto _label))))

(event EventBeginPlay
  (|CallParentFunction)
  (bind _asbp_gi (Utilities|Casting|CastToBP_GI (Game|GetGameInstance)))
  (EventDispatchers|BindEventtoOnGameStateChanged _asbp_gi (delegate Custom|CustomEvent)))

(event EventTick
  (params (DeltaSeconds :type Float%20%28single-precision%29))
  (Utilities|FlowControl|Sequence
    (:then_0
      (|CallParentFunction DeltaSeconds)
      (if (< (Variables|Default|GetUltimeDurationTimer) (Variables|Default|GetUltimeDuration))
        (Variables|Default|SetUltimeDurationTimer (+ (Variables|Default|GetUltimeDurationTimer) DeltaSeconds))
        (elif (not (== (Variables|Default|GetUltimeDurationTimer) (Variables|Default|GetUltimeDuration)))
          (Variables|Default|SetUltimeDurationTimer (Variables|Default|GetUltimeDuration))
          (Collision|SetCollisionEnabled (Variables|Default|GetAttraction) "NoCollision")
          (Collision|SetCollisionEnabled (Variables|Default|GetCenter) "NoCollision")
          (Rendering|SetVisibility (Variables|Default|GetVFX_Satoshi) false false)
          (Variables|Default|SetIsAttracting false)
          (Variables|Default|SetCaptedFighter 0)
          (CallFunction|ChangeState "NewEnumerator2"))))
    (:then_1
      (CallFunction|Traction DeltaSeconds))))

(fn ConstructionScript
  (|CallParentFunction)
  (Collision|SetCollisionEnabled (Variables|Default|GetAttraction) "NoCollision")
  (Collision|SetCollisionEnabled (Variables|Default|GetCenter) "NoCollision"))

(fn UseUltime
  (|CallParentFunction)
  (Transformation|SetActorLocation (Transformation|GetActorLocation (Variables|Default|GetFighterUser)) false true)
  (Collision|SetCollisionEnabled (Variables|Default|GetAttraction) "NoCollision")
  (Collision|SetCollisionEnabled (Variables|Default|GetCenter) "NoCollision")
  (CallFunction|SpawnBlackHole))

(fn SpawnBlackHole
  (bind _vfx_satoshi (Variables|Default|GetVFX_Satoshi))
  (Collision|SetCollisionEnabled (Variables|Default|GetAttraction) "QueryOnly")
  (Collision|SetCollisionEnabled (Variables|Default|GetCenter) "QueryOnly")
  (Components|Activation|Activate _vfx_satoshi false)
  (Rendering|SetVisibility _vfx_satoshi true false))

(fn Traction
  (params (DeltaTime :type Float%20%28single-precision%29))
  (bind _returnvalue (Transformation|GetActorLocation))
  (bind _captedfighter (Variables|Default|GetCaptedFighter))
  (bind _returnvalue_2 (Transformation|GetActorLocation _captedfighter))
  (bind _floatingpawnmovement (Variables|/Game/BP/Players/Fighter/BP_FighterPawn.BP_FighterPawn_C|GetFloatingPawnMovement _captedfighter))
  (bind _returnvalue_3 (Math|Vector|Distance(Vector) _returnvalue_2 _returnvalue))
  (if (Variables|Default|GetIsAttracting)
    (Development|PrintString (Utilities|String|Append "dist : " (Utilities|String|ToString(Float) _returnvalue_3)) true true "(R=1.000000,G=0.423462,B=0.000000,A=1.000000)" 0.0)
    (bind _output_get (Variables|/Script/Engine.MovementComponent|SetVelocity _floatingpawnmovement (+ (Variables|/Script/Engine.MovementComponent|GetVelocity _floatingpawnmovement) (* (Math|Vector|GetForwardVector (Math|Rotator|FindLookatRotation _returnvalue_2 _returnvalue)) DeltaTime (Math|Float|Clamp(Float) (* (Variables|Default|GetTractionStrenght) (Math|Float|Lerp 3.0 0.25 (Math|Float|Clamp(Float) (/ (- _returnvalue_3 2e+02) 3.2e+02)))) 3e+03 1.5e+04)))))))

(fn SetEnable
  (params (Enable :type Boolean) (Hide :type Boolean))
  (Variables|Default|SetVFXs (Utilities|Array|MakeArray (Variables|Default|GetVFX_Satoshi)))
  (|CallParentFunction Enable Hide)
  (return false))