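; Maria's ultimate: spawns a black hole at the user's location for UltimeDuration.
; A DelayWithTimer per-tick loop resizes the Attraction and Center spheres along BlackHoleScaleCurve, then disables collision and VFX and changes state.
; Attraction captures one opposing fighter, and Tick adds velocity toward the hole, stronger at close range and clamped.
; Opponents entering Center are stunned and spun.
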(event OnComponentBeginOverlap(Attraction)
  (params (OverlappedComponent :type Primitive%20Component%20Object%20Reference) (OtherActor :type Actor%20Object%20Reference) (OtherComp :type Primitive%20Component%20Object%20Reference) (OtherBodyIndex :type Integer) (bFromSweep :type Boolean) (SweepResult :type Hit%20Result%20Structure%20%28by%20ref%29))
  (bind _asbp_fighter_pawn (Utilities|Casting|CastToBP_FighterPawn OtherActor))
  (if (!= (Variables|/Game/BP/Players/Fighter/BP_FighterPawn.BP_FighterPawn_C|GetIndex _asbp_fighter_pawn) (Variables|/Game/BP/Players/Fighter/BP_FighterPawn.BP_FighterPawn_C|GetIndex (Variables|Default|GetFighterUser)))
    (Variables|Default|SetIsAttracting true)
    (Variables|Default|SetCaptedFighter _asbp_fighter_pawn)))

(event OnComponentBeginOverlap(Center)
  (params (OverlappedComponent :type Primitive%20Component%20Object%20Reference) (OtherActor :type Actor%20Object%20Reference) (OtherComp :type Primitive%20Component%20Object%20Reference) (OtherBodyIndex :type Integer) (bFromSweep :type Boolean) (SweepResult :type Hit%20Result%20Structure%20%28by%20ref%29))
  (bind _asbp_fighter_pawn (Utilities|Casting|CastToBP_FighterPawn OtherActor))
  (if (!= (Variables|/Game/BP/Players/Fighter/BP_FighterPawn.BP_FighterPawn_C|GetIndex _asbp_fighter_pawn) (Variables|/Game/BP/Players/Fighter/BP_FighterPawn.BP_FighterPawn_C|GetIndex (Variables|Default|GetFighterUser)))
    (Default|SetStun _asbp_fighter_pawn 1.5 3e+01)))

(event OnComponentEndOverlap(Attraction)
  (params (OverlappedComponent :type Primitive%20Component%20Object%20Reference) (OtherActor :type Actor%20Object%20Reference) (OtherComp :type Primitive%20Component%20Object%20Reference) (OtherBodyIndex :type Integer))
  (if (== OtherActor (Variables|Default|GetCaptedFighter))
    (Variables|Default|SetIsAttracting false)
    (Variables|Default|SetCaptedFighter 0)))

(event EventBeginPlay
  (|CallParentFunction)
  (Variables|Default|SetCenterColliderBaseRadius (Components|Sphere|GetScaledSphereRadius (Variables|Default|GetCenter)))
  (Variables|Default|SetAttractionColliderBaseRadius (Components|Sphere|GetScaledSphereRadius (Variables|Default|GetAttraction))))

(event EventUseUltime
  (bind _ultimeduration (Variables|Default|GetUltimeDuration))
  (bind _blackholescalecurve (Variables|Default|GetBlackHoleScaleCurve))
  (bind _delaytimer (Variables|Default|GetDelayTimer))
  (bind _returnvalue (/ _delaytimer _ultimeduration))
  (bind _returnvalue_2 (- 1.0 _returnvalue))
  (bind _returnvalue_3 (Math|Curves|GetFloatValue _blackholescalecurve _returnvalue_2))
  (|CallParentFunction)
  (Transformation|SetActorLocation (Transformation|GetActorLocation (Variables|Default|GetFighterUser)) false true)
  (CallFunction|SpawnBlackHole)
  (Audio|PlaySound2D "/Game/BP/Ultime/UltimeSatoshi/CUE_UltSatoshi.CUE_UltSatoshi" 1.0 1.0 0.0 0 0)
  (Utilities|DelaywithTimer (Variables|Default|GetUltimeDuration)
    (:Completed
      (Variables|Default|SetUltimeDurationTimer (Variables|Default|GetUltimeDuration))
      (Collision|SetCollisionEnabled (Variables|Default|GetAttraction) "NoCollision")
      (Collision|SetCollisionEnabled (Variables|Default|GetCenter) "NoCollision")
      (Components|Activation|Deactivate (Variables|Default|GetVFX_Satoshi))
      (Variables|Default|SetIsAttracting false)
      (Variables|Default|SetCaptedFighter 0)
      (CallFunction|ChangeState "NewEnumerator2"))
    (:OnGoing
      (Components|Sphere|SetSphereRadius (Variables|Default|GetCenter) (* _returnvalue_3 (Variables|Default|GetCenterColliderBaseRadius)) true)
      (Components|Sphere|SetSphereRadius (Variables|Default|GetAttraction) (* _returnvalue_3 (Variables|Default|GetAttractionColliderBaseRadius)) true))))

(event EventTick
  (params (DeltaSeconds :type Float%20%28single-precision%29))
  (bind _output_get (Variables|Default|SetDelayTimer (- (stale _output_get) DeltaSeconds)))
  (|CallParentFunction DeltaSeconds)
  (|DebugCollision)
  (CallFunction|Traction DeltaSeconds))

(fn ConstructionScript
  (|CallParentFunction)
  (Collision|SetCollisionEnabled (Variables|Default|GetAttraction) "NoCollision")
  (Collision|SetCollisionEnabled (Variables|Default|GetCenter) "NoCollision"))

(fn SpawnBlackHole
  (bind _vfx_satoshi (Variables|Default|GetVFX_Satoshi))
  (Collision|SetCollisionEnabled (Variables|Default|GetAttraction) "QueryAndPhysics")
  (Collision|SetCollisionEnabled (Variables|Default|GetCenter) "QueryAndPhysics")
  (Components|Activation|Activate _vfx_satoshi false)
  (Rendering|SetVisibility _vfx_satoshi true false))

(fn Traction
  (params (DeltaTime :type Float%20%28single-precision%29))
  (bind _returnvalue (Transformation|GetActorLocation))
  (bind _captedfighter (Variables|Default|GetCaptedFighter))
  (bind _returnvalue_2 (Transformation|GetActorLocation _captedfighter))
  (bind _floatingpawnmovement (Variables|/Game/BP/Players/Fighter/BP_FighterPawn.BP_FighterPawn_C|GetFloatingPawnMovement _captedfighter))
  (if (Variables|Default|GetIsAttracting)
    (bind _output_get (Variables|/Script/Engine.MovementComponent|SetVelocity _floatingpawnmovement (+ (Variables|/Script/Engine.MovementComponent|GetVelocity _floatingpawnmovement) (* (Math|Vector|GetForwardVector (Math|Rotator|FindLookatRotation _returnvalue_2 _returnvalue)) DeltaTime (Math|Float|Clamp(Float) (* (Variables|Default|GetTractionForce) (Math|Float|Lerp 3.0 0.25 (Math|Float|Clamp(Float) (/ (- (Math|Vector|Distance(Vector) _returnvalue_2 _returnvalue) 2e+02) 3.2e+02)))) 3e+03 1.5e+04)))))))

(fn SetEnable
  (params (Enable :type Boolean) (Hide :type Boolean))
  (Variables|Default|SetVFXs (Utilities|Array|MakeArray (Variables|Default|GetVFX_Satoshi)))
  (|CallParentFunction Enable Hide)
  (return false))