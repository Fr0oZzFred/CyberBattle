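; Parent actor for fighter ultimates, handling cooldown, state changes and skin-tinted Niagara VFX attached to the owning fighter.
; Construction loads settings from a data table by name, and Tick counts the cooldown from half to turn Reload into Usable.
; UseUltime waits out any playing UI use animation, then enters Use and plays a level sequence flagged as cinematic.
; Game state toggles tick, VFX and visibility; fighter death and respawn toggle the ready effect.
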(event Custom|UseUltime
  (bind _gi (Variables|Default|GetGI))
  (bind _uimanager (Variables|/Game/BP/BP_GI.BP_GI_C|GetUIManager _gi))
  (bind _inbattle (Variables|/Game/UI/HUD_Manager.HUD_Manager_C|GetInBattle _uimanager))
  (Utilities|IsValid _inbattle
    (:Is%20Valid
      (if (Class|UserWidget|IsAnimationPlaying _inbattle (Variables|/Game/UI/UMG_InBattle.UMG_InBattle_C|GetOnUltUse _inbattle)) :!label _label
        (Utilities|FlowControl|DelayUntilNextTick)
        (goto _label)
        (else
          _)))
    (:Is%20Not%20Valid
      _))
  (CallFunction|ChangeState "NewEnumerator1")
  (Variables|/Game/BP/BP_GI.BP_GI_C|SetInCinematic (Variables|Default|GetGI) true)
  (Variables|Default|SetUltimeDurationTimer 0.0)
  (Variables|Default|SetUltimeCooldownTimer (Variables|Default|GetUltimeCooldown))
  (bind _returnvalue (Sequencer|Player|CreateLevelSequencePlayer "/Game/BP/Ultime/Ult_NoCam.Ult_NoCam"))
  (Sequencer|Player|Play _returnvalue :!class /Script/MovieScene.MovieSceneSequencePlayer)
  (EventDispatchers|AssignOnFinished _returnvalue (delegate Custom|OnFinished_Event)))

(event Custom|OnKilled_Event
  (params (KilledPlayer :type Integer))
  (bind _vfx_onultusable (Variables|Default|GetVFX_OnUltUsable))
  (Components|Activation|Deactivate _vfx_onultusable)
  (Rendering|SetVisibility _vfx_onultusable false false))

(event Custom|OnRespawn_Event
  (params (Index :type Integer))
  (bind _vfx_onultusable (Variables|Default|GetVFX_OnUltUsable))
  (if (Utilities|Enum|Equal(Enum) (Variables|Default|GetUltimeState) "NewEnumerator0")
    (Components|Activation|Activate _vfx_onultusable true)
    (Rendering|SetVisibility _vfx_onultusable true false)))

(event Custom|OnGameStateChanged
  (params (New%20State :type E_GameState%20Enum :default "NewEnumerator0"))
  (switch Utilities|FlowControl|Switch|SwitchonE_GameState New%20State
    (:NewEnumerator7
      (CallFunction|SetEnable false true :!label _label))
    (:NewEnumerator3
      (CallFunction|SetEnable true false))
    (:NewEnumerator5
      (CallFunction|SetEnable false false))
    (:NewEnumerator4
      (goto _label))))

(event Custom|OnFinished_Event
  (Variables|/Game/BP/BP_GI.BP_GI_C|SetInCinematic (Variables|Default|GetGI) false))

(event Custom|BindUltEvent
  (EventDispatchers|AssignOnKilled (Variables|Default|GetFighterUser) (delegate Custom|OnKilled_Event))
  (EventDispatchers|AssignOnRespawn (Variables|Default|GetFighterUser) (delegate Custom|OnRespawn_Event)))

(event EventBeginPlay
  (bind _output_get (Variables|Default|SetGI (.AsBP%20GI (Utilities|Casting|CastToBP_GI (Game|GetGameInstance)))))
  (EventDispatchers|BindEventtoOnGameStateChanged _output_get (delegate Custom|OnGameStateChanged))
  (CallFunction|InitVFX)
  (EventDispatchers|AssignOnKilled (Variables|Default|GetFighterUser) (delegate Custom|OnKilled_Event))
  (EventDispatchers|AssignOnRespawn (Variables|Default|GetFighterUser) (delegate Custom|OnRespawn_Event)))

(event EventTick
  (params (DeltaSeconds :type Float%20%28single-precision%29))
  (if (> (Variables|Default|GetUltimeCooldownTimer) 0.0)
    (Variables|Default|SetUltimeCooldownTimer (- (Variables|Default|GetUltimeCooldownTimer) DeltaSeconds))
    (else
      (switch Utilities|FlowControl|Switch|SwitchonEnum_SkillState (Variables|Default|GetUltimeState)
        (:NewEnumerator2
          (CallFunction|ChangeState "NewEnumerator0")
          (Variables|Default|SetUltimeCooldownTimer 0.0))))))

(fn ConstructionScript
  (bind _returnvalue (Utilities|GetDataTableRow (Variables|Default|GetUltimeData) (Variables|Default|GetName))
    (:then
      (bind _output_get (Variables|Default|SetUltimeDataArray _returnvalue))
      (Variables|Default|SetIcon (.Icon (Utilities|Struct|BreakStruct_Ultime _output_get)))
      (Variables|Default|SetDescription (.Description (Utilities|Struct|BreakStruct_Ultime _output_get)))
      (bind _output_get_2 (Variables|Default|SetUltimeCooldown (.Cooldown (Utilities|Struct|BreakStruct_Ultime _output_get))))
      (Variables|Default|SetUltimeCooldownTimer (/ _output_get_2 2.0))
      (bind _output_get_3 (Variables|Default|SetUltimeDuration (.Duration (Utilities|Struct|BreakStruct_Ultime _output_get))))
      (Variables|Default|SetUltimeDurationTimer _output_get_3)
      (Variables|Default|SetBehaviorTree (.BehaviorTree (Utilities|Struct|BreakStruct_Ultime _output_get))))
    (:RowNotFound
      (Development|PrintString "Ult Name not found in data table" true true "(R=1.000000,G=0.000000,B=0.006452,A=1.000000)" 3e+01))))

(fn ChangeState
  (params (NewState :type Enum_SkillState%20Enum :default "NewEnumerator0"))
  (bind _vfx_onultusable (Variables|Default|GetVFX_OnUltUsable))
  (if (Utilities|Enum|NotEqual(Enum) NewState (Variables|Default|GetUltimeState))
    (bind _output_get (Variables|Default|SetUltimeState NewState))
    (Default|CallOnUltimeChangeState _output_get (Variables|/Game/BP/Players/Fighter/BP_FighterPawn.BP_FighterPawn_C|GetIndex (Variables|Default|GetFighterUser)))
    (switch Utilities|FlowControl|Switch|SwitchonEnum_SkillState _output_get
      (:NewEnumerator0
        (Components|Activation|Activate _vfx_onultusable true)
        (Rendering|SetVisibility _vfx_onultusable true false))
      (:NewEnumerator1
        (Components|Activation|Deactivate _vfx_onultusable)
        (Rendering|SetVisibility _vfx_onultusable false false)
        (Components|Activation|Activate (Variables|Default|GetVFX_OnUltUse) true)))))

(fn PauseVFX
  (params (Enable :type Boolean))
  (Class|NiagaraComponent|SetPaused (Variables|Default|GetVFX_OnUltUsable) (not Enable))
  (for _array_element (Variables|Default|GetVFXs)
    (Class|NiagaraComponent|SetPaused _array_element (not Enable)))
  (return))

(fn InitVFX
  (bind _fighteruser (Variables|Default|GetFighterUser))
  (bind _fighteruser_2 (Variables|Default|GetFighterUser))
  (bind _returnvalue (Niagara|SpawnSystemAttached "/Game/BP/Ultime/VFX_OnUltUsable.VFX_OnUltUsable" (Variables|/Game/BP/Players/Fighter/BP_FighterPawn.BP_FighterPawn_C|GetFrame _fighteruser) "None" "0, 0, 0" "0, 0, 0" "KeepRelativeOffset" false false))
  (bind _output_get (Variables|Default|SetVFX_OnUltUsable _returnvalue))
  (Effects|Components|ParticleSystem|SetColorParameter _output_get "Color" (Utilities|Struct|BreakS_DashSkin (.Dash (Utilities|Struct|BreakS_FighterSkin (Variables|/Game/BP/Players/Fighter/BP_FighterPawn.BP_FighterPawn_C|GetFighterSkin _fighteruser)))))
  (bind _returnvalue_2 (Niagara|SpawnSystemAttached "/Game/BP/Ultime/VFX_OnUltUse.VFX_OnUltUse" (Variables|/Game/BP/Players/Fighter/BP_FighterPawn.BP_FighterPawn_C|GetFrame _fighteruser_2) "None" "0, 0, 0" "0, 0, 0" "KeepRelativeOffset" false false))
  (bind _output_get_2 (Variables|Default|SetVFX_OnUltUse _returnvalue_2))
  (Effects|Components|ParticleSystem|SetColorParameter _output_get_2 "Color" (Utilities|Struct|BreakS_DashSkin (.Dash (Utilities|Struct|BreakS_FighterSkin (Variables|/Game/BP/Players/Fighter/BP_FighterPawn.BP_FighterPawn_C|GetFighterSkin _fighteruser_2))))))

(fn SetEnable
  (params (Enable :type Boolean) (Hide :type Boolean))
  (Actor|Tick|SetActorTickEnabled Enable)
  (CallFunction|PauseVFX Enable)
  (Rendering|SetVisibility (Variables|Default|GetDefaultSceneRoot) (and (not Hide) (Utilities|Enum|Equal(Enum) (Variables|Default|GetUltimeState) "NewEnumerator1")) true)
  (return false))