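; BP_MariaFighterOld is a temporary fighter from Maria's ultimate that fires on its owner's behalf until its lifetime expires.
; Tick moves it toward randomized X targets, alternating bias via FlipFlop, on a Y line chosen by UltIndex.
; A jittered reload timer triggers Shot, which spawns pooled projectiles using FighterUser's stats and skin, with a random laser sound.
; BP_GI game-state changes toggle its tick and visibility.
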(event Custom|OnGameStateChanged
  (params (New%20State :type E_GameState%20Enum :default "NewEnumerator0"))
  (switch Utilities|FlowControl|Switch|SwitchonE_GameState New%20State
    (:NewEnumerator7
      (CallFunction|SetEnable false true :!label _label))
    (:NewEnumerator3
      (CallFunction|SetEnable true false))
    (:NewEnumerator5
      (CallFunction|SetEnable false false))
    (:NewEnumerator4
      (goto _label))))

(event EventBeginPlay
  (bind _returnvalue (Transformation|GetActorLocation))
  (bind _output_get (Variables|Default|SetOffsetXTarget (Math|Float|Clamp(Float) (Math|Random|RandomFloatinRange 0.0 425.0) -425.0 425.0)))
  (Variables|Default|SetTargetPos (Math|Vector|MakeVector (+ _output_get (.x _returnvalue)) (Utilities|Select :Index (Variables|Default|GetUltIndex) :Option%200 1.15e+03 :Option%201 1.15e+03 :Option%202 -1.5e+02 :Option%203 -1.5e+02) 7e+01))
  (Variables|Default|SetStartPos (Math|Vector|MakeVector (.x _returnvalue) (.y _returnvalue) (.z _returnvalue)))
  (bind _asbp_gi (Utilities|Casting|CastToBP_GI (Game|GetGameInstance)))
  (EventDispatchers|BindEventtoOnGameStateChanged _asbp_gi (delegate Custom|OnGameStateChanged)))

(event Collision|EventActorBeginOverlap
  (params (OtherActor :type Actor%20Object%20Reference)))

(event EventTick
  (params (DeltaSeconds :type Float%20%28single-precision%29))
  (bind _returnvalue (Transformation|GetActorLocation))
  (bind _output_get (Variables|Default|SetReloadTimer (- (Variables|Default|GetReloadTimer) DeltaSeconds)))
  (if (< _output_get 0.0)
    (CallFunction|Shot)
    (Variables|Default|SetReloadTimer (+ (Variables|Default|GetReloadCD) (Math|Random|RandomFloatinRange -0.75 0.75))))
  (if (Utilities|Operators|EqualEqual (Variables|Default|GetTargetPos) _returnvalue 2e+01)
    (Utilities|FlowControl|FlipFlop
      (:A
        (Variables|Default|SetOffsetXTarget (Math|Float|Clamp(Float) (Math|Random|RandomFloatinRange -2e+02 1e+02) -425.0 425.0)))
      (:B
        (Variables|Default|SetOffsetXTarget (Math|Float|Clamp(Float) (Math|Random|RandomFloatinRange -1e+02 2e+02) -425.0 425.0))))
    (Variables|Default|SetTargetPos (Math|Vector|MakeVector (+ (Variables|Default|GetOffsetXTarget) (.x (Variables|Default|GetStartPos))) (Utilities|Select :Index (Variables|Default|GetUltIndex) :Option%200 1.15e+03 :Option%201 1.15e+03 :Option%202 -1.5e+02 :Option%203 -1.5e+02) 7e+01))
    (else
      (Transformation|SetActorLocation (+ (Transformation|GetActorLocation) (* (Math|Vector|GetForwardVector (Math|Rotator|FindLookatRotation _returnvalue (Variables|Default|GetTargetPos))) (* DeltaSeconds (Variables|Default|GetSpeed)))) false false)))
  (Variables|Default|SetLifeTime (- (Variables|Default|GetLifeTime) DeltaSeconds))
  (if (< (Variables|Default|GetLifeTime) 0.0)
    (Actor|DestroyActor)))

(fn ConstructionScript)

(fn Shot
  (bind _fighteruser (Variables|Default|GetfighterUser))
  (bind _asbp_gi (Utilities|Casting|CastToBP_GI (Game|GetGameInstance)))
  (if (Utilities|Enum|Equal(Enum) (Variables|/Game/BP/BP_GI.BP_GI_C|GetCurrentState _asbp_gi) "NewEnumerator3")
    (Default|SpawnProjectile (Variables|/Game/BP/Players/Fighter/BP_FighterPawn.BP_FighterPawn_C|GetPoolManager _fighteruser) (Math|Transform|MakeTransform (Transformation|GetWorldLocation (Variables|Default|GetFrame)) (.rotation (Transformation|GetActorTransform)) "1.000000,1.000000,1.000000") (Variables|Default|GetIndex) (Transformation|GetActorForwardVector) (Variables|/Game/BP/Players/Fighter/BP_FighterPawn.BP_FighterPawn_C|GetProjectileSpeed _fighteruser) 0.0 (Variables|/Game/BP/Players/Fighter/BP_FighterPawn.BP_FighterPawn_C|GetProjectileDamageToFighter _fighteruser) (Variables|/Game/BP/Players/Fighter/BP_FighterPawn.BP_FighterPawn_C|GetMaxProjDistance _fighteruser) (.Projectile (Utilities|Struct|BreakS_NewPlayerSkin (Variables|/Game/BP/Players/Fighter/BP_FighterPawn.BP_FighterPawn_C|GetPlayerSkin _fighteruser))) "NewEnumerator4")
    (Audio|PlaySound2D (Utilities|Select :Index (Math|Random|RandomInteger 5) :Option%200 "/Game/Sounds/SoundEffect/Fighter/laserShoot1.laserShoot1" :Option%201 "/Game/Sounds/SoundEffect/Fighter/laserShoot2.laserShoot2" :Option%202 "/Game/Sounds/SoundEffect/Fighter/laserShoot3.laserShoot3" :Option%203 "/Game/Sounds/SoundEffect/Fighter/laserShoot4.laserShoot4" :Option%204 "/Game/Sounds/SoundEffect/Fighter/laserShoot5.laserShoot5" :Option%205 "/Game/Sounds/SoundEffect/Fighter/laserShoot6.laserShoot6") 1.0 1.0 0.0 0 0)))

(fn SetEnable
  (params (Enable :type Boolean) (Hide :type Boolean))
  (Actor|Tick|SetActorTickEnabled Enable)
  (Rendering|SetVisibility (Variables|Default|GetFrame) (not Hide) true)
  (return false))