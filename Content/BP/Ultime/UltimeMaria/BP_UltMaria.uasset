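; Maria's ultimate ability actor, which snaps onto the fighter using it and summons helper fighters.
; On use, it spawns two BP_MariaFighter actors, passing each the owner, its index, the opposing player from the BattleManager and the ultimate's duration.
; Tick counts up to that duration, then clamps the timer and changes state once.
; An older four-fighter spawn at fixed arena positions remains but never runs.
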(event EventBeginPlay
  (|CallParentFunction)
  (Transformation|AttachActorToActor (Variables|Default|GetFighterUser) "None" "SnapToTarget" "SnapToTarget" "SnapToTarget" true))

(event EventTick
  (params (DeltaSeconds :type Float%20%28single-precision%29))
  (|CallParentFunction DeltaSeconds)
  (if (< (Variables|Default|GetUltimeDurationTimer) (Variables|Default|GetUltimeDuration))
    (Variables|Default|SetUltimeDurationTimer (+ (Variables|Default|GetUltimeDurationTimer) DeltaSeconds))
    (elif (not (== (Variables|Default|GetUltimeDurationTimer) (Variables|Default|GetUltimeDuration)))
      (Variables|Default|SetUltimeDurationTimer (Variables|Default|GetUltimeDuration))
      (CallFunction|ChangeState "NewEnumerator2"))))

(event EventUseUltime
  (|CallParentFunction)
  (CallFunction|SpawnFighters))

(fn ConstructionScript
  (|CallParentFunction))

(fn OldSpawnFighters
  (bind _fighteruser (Variables|Default|GetFighterUser))
  (for _index (range 0 3)
    (Game|SpawnActorfromClass "/Game/BP/Ultime/UltimeMaria/BP_MariaFighterOld.BP_MariaFighterOld_C" (Math|Transform|MakeTransform (Utilities|Select :Index _index :Option%200 "625.000000,1150.000000,70.000000" :Option%201 "1475.000000,1150.000000,70.000000" :Option%202 "625.000000,-150.000000,70.000000" :Option%203 "1475.000000,-150.000000,70.000000") (Utilities|Select :Index _index :Option%200 "0.000000,-90.000000,0.000000" :Option%201 "0.000000,-90.000000,0.000000" :Option%202 "0.000000,90.000000,0.000000" :Option%203 "0.000000,90.000000,0.000000") "1.000000,1.000000,1.000000") "Undefined" 0 (Variables|/Game/BP/Players/Fighter/BP_FighterPawn.BP_FighterPawn_C|GetIndex _fighteruser) _index (Variables|Default|GetUltimeDuration) _fighteruser 0)))

(fn SpawnFighters
  (bind _fighteruser (Variables|Default|GetFighterUser))
  (bind _gi (Variables|Default|GetGI))
  (bind _index (Variables|/Game/BP/Players/Fighter/BP_FighterPawn.BP_FighterPawn_C|GetIndex _fighteruser))
  (bind _battlemanager (Variables|/Game/BP/BP_GI.BP_GI_C|GetBattleManager _gi))
  (for _index_2 (range 0 1)
    (Game|SpawnActorfromClass "/Game/BP/Ultime/UltimeMaria/BP_MariaFighter.BP_MariaFighter_C" (Math|Transform|MakeTransform "0, 0, 0" "0, 0, 0" "1.000000,1.000000,1.000000") "Undefined" 0 _index _index_2 _fighteruser (Utilities|Select :Index _index :Option%200 (Variables|/Game/BP/BP_BattleManager.BP_BattleManager_C|GetP2 _battlemanager) :Option%201 (Variables|/Game/BP/BP_BattleManager.BP_BattleManager_C|GetP1 _battlemanager)) (Variables|Default|GetUltimeDuration) 0)))