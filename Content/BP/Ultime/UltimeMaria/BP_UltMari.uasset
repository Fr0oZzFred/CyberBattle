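; Maria's ultimate ability, which summons four BP_MariaFighter actors when used.
; SpawnFighters places them at fixed world positions in two opposing pairs, passing each the user's index, its own slot, the user reference and the ultimate's duration as lifetime.
; Tick counts up to that duration, then clamps the timer and switches the inherited ultimate state once.
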(event EventBeginPlay
  (|CallParentFunction) ; This node is disabled and will not be called.\nDrag off pins to build functionality.
)

(event Collision|EventActorBeginOverlap
  (params (OtherActor :type Actor%20Object%20Reference)))

(event EventTick
  (params (DeltaSeconds :type Float%20%28single-precision%29))
  (|CallParentFunction DeltaSeconds)
  (if (< (Variables|Default|GetUltimeDurationTimer) (Variables|Default|GetUltimeDuration))
    (Variables|Default|SetUltimeDurationTimer (+ (Variables|Default|GetUltimeDurationTimer) DeltaSeconds))
    (elif (not (== (Variables|Default|GetUltimeDurationTimer) (Variables|Default|GetUltimeDuration)))
      (Variables|Default|SetUltimeDurationTimer (Variables|Default|GetUltimeDuration))
      (CallFunction|ChangeState "NewEnumerator2"))))

(event EventUseUltime
  (|CallParentFunction)
  (CallFunction|SpawnFighters))

(fn ConstructionScript
  (|CallParentFunction))

(fn SpawnFighters
  (bind _fighteruser (Variables|Default|GetFighterUser))
  (for _index (range 0 3)
    (Game|SpawnActorfromClass "/Game/BP/Ultime/UltimeMaria/BP_MariaFighter.BP_MariaFighter_C" (Math|Transform|MakeTransform (Utilities|Select :Index _index :Option%200 "625.000000,1150.000000,70.000000" :Option%201 "1475.000000,1150.000000,70.000000" :Option%202 "625.000000,-150.000000,70.000000" :Option%203 "1475.000000,-150.000000,70.000000") (Utilities|Select :Index _index :Option%200 "0.000000,-90.000000,0.000000" :Option%201 "0.000000,-90.000000,0.000000" :Option%202 "0.000000,90.000000,0.000000" :Option%203 "0.000000,90.000000,0.000000") "1.000000,1.000000,1.000000") "Undefined" 0 (Variables|/Game/BP/Players/Fighter/BP_FighterPawn.BP_FighterPawn_C|GetIndex _fighteruser) _index (Variables|Default|GetUltimeDuration) _fighteruser 0)))