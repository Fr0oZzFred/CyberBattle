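; BP_TestParticles is a placeholder test Blueprint that plays block appear and disappear effects on a key press.
; On BeginPlay it retries each tick until the first player controller is valid, then enables input.
; The "<" key prints a debug string, activates VFXBlocAppear, then two seconds later activates VFXBlocDisappear and hides the appear effect.
; The appear effect is never unhidden in this graph.
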(event EventBeginPlay
  (bind _returnvalue (Game|GetPlayerController 0))
  (Utilities|IsValid _returnvalue :!label _label
    (:Is%20Valid
      (Input|EnableInput _returnvalue))
    (:Is%20Not%20Valid
      (Utilities|FlowControl|DelayUntilNextTick)
      (goto _label))))

(event Input|KeyboardEvents|<
  (params (Key :type Key%20Structure :default "None"))
  (:Pressed
    (Development|PrintString "Hello")
    (Components|Activation|Activate (Variables|Default|GetVFX_BlocAppear) false)
    (Utilities|FlowControl|Delay 2.0)
    (Components|Activation|Activate (Variables|Default|GetVFX_BlocDisappear) false)
    (Development|SetHiddeninGame (Variables|Default|GetVFX_BlocAppear) true false)))

(fn ConstructionScript)